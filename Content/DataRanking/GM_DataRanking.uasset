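; Game mode for the ranking screen that alternates between local and online leaderboard widgets with fade transitions.
; BeginPlay creates the widgets and a timer actor, then a looping timer drives an enum state machine.
; Each board holds until the timer expires, then swaps once the fade widget reports completion.
; The online board is skipped, keeping the local one, when its success-state check fails.
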(event `self.ReceiveBeginPlay`
  (bind _returnvalue (`|SpawnActorFromClass` "/Game/Play/Common/GroundObject/BP_Timer.BP_Timer_C" (`KismetMathLibrary.MakeTransform` (0.0 0.0 0.0)) "Undefined" "OverrideRootScale" null null))
  (bind _output_get (set `self.mBP_CountTimer` _returnvalue))
  (`/Game/Play/Common/GroundObject/BP_Timer.fSetMaxTime` _output_get 3.0)
  ;[1 1 1] ウィジェットの作成
  (bind _returnvalue_2 (`|CreateWidget` "/Game/Play/Common/Fade/WBP_Fade.WBP_Fade_C"))
  (bind _output_get_2 (set `self.WBP_Fade` _returnvalue_2))
  (`UserWidget.AddToViewport` _output_get_2 100)
  (bind _returnvalue_3 (`|CreateWidget` "/Game/DataRanking/WBP_OnLineRanking.WBP_OnLineRanking_C"))
  (bind _output_get_3 (set `self.WBP_OnlineRanking` _returnvalue_3))
  (`UserWidget.AddToViewport` _output_get_3 0)
  (`Widget.RemoveFromParent` _output_get_3)
  (bind _returnvalue_4 (`|CreateWidget` "/Game/DataRanking/WBP_LocalRanking.WBP_LocalRanking_C"))
  (set `self.WBP_LocalRanking` _returnvalue_4)
  (`/Game/Play/Common/Fade/WBP_Fade.BlackOut` (`self.WBP_Fade`)) ; 画面暗転
  (`self.Init`)
  (`KismetSystemLibrary.K2_SetTimerDelegate` (delegate `Update`) (`self.DELTA_TIME`) true))

(event `Init`
  (`UserWidget.AddToViewport` (`self.WBP_LocalRanking`) 0) ; ローカルランキングの表示
  (`/Game/Play/Common/Fade/WBP_Fade.FadeInitialize` (`self.WBP_Fade`) "NewEnumerator1" 0.01))

(event `Update`
  (switch `/Game/DataRanking/EN_DataRankingState` (`self.mState`)
    (:`NewEnumerator0`
      (`self.InitFadeOut`))
    (:`NewEnumerator1`
      (`self.DrawLocalRanking`))
    (:`NewEnumerator2`
      (`self.LocalRankingFadeIn`))
    (:`NewEnumerator3`
      (`self.LocalRankingFadeOut`))
    (:`NewEnumerator4`
      (`self.DrawOnlineRanking`))
    (:`NewEnumerator5`
      (`self.OnlineRankingFadeIn`))
    (:`NewEnumerator6`
      (`self.OnlineRankingFadeOut`))
    (:`NewEnumerator8`
      (`self.EndFadeIn`))))

(event `InitFadeOut`
  (if (`/Game/Play/Common/Fade/WBP_Fade.mEnd` (`self.WBP_Fade`))
    (set `self.mState` "NewEnumerator1")))

(event `DrawLocalRanking`
  (bind _newparam (`/Game/Play/Common/GroundObject/BP_Timer.fCountUp` (`self.mBP_CountTimer`) (`self.DELTA_TIME`))) ; 時間が終わったら
  (if _newparam
    (`/Game/Play/Common/Fade/WBP_Fade.FadeInitialize` (`self.WBP_Fade`) "NewEnumerator0" 0.01)
    (set `self.mState` "NewEnumerator2")
    (`/Game/Play/Common/GroundObject/BP_Timer.fReset` (`self.mBP_CountTimer`))))

(event `LocalRankingFadeIn`
  (if (`/Game/Play/Common/Fade/WBP_Fade.mEnd` (`self.WBP_Fade`))
    (`/Game/Play/Common/Fade/WBP_Fade.FadeInitialize` (`self.WBP_Fade`) "NewEnumerator1" 0.01)
    (bind _newparam (`self.fChackOnline`))
    (if _newparam
      (`UserWidget.AddToViewport` (`self.WBP_OnlineRanking`) 0) ; オンラインランキングの表示
      (`Widget.RemoveFromParent` (`self.WBP_LocalRanking`)) ; ローカルランキングの非表示
      (set `self.mState` "NewEnumerator3")
      (else
        (set `self.mState` "NewEnumerator0")))))

(event `LocalRankingFadeOut`
  (if (`/Game/Play/Common/Fade/WBP_Fade.mEnd` (`self.WBP_Fade`))
    (set `self.mState` "NewEnumerator4")))

(event `DrawOnlineRanking`
  (bind _newparam (`/Game/Play/Common/GroundObject/BP_Timer.fCountUp` (`self.mBP_CountTimer`) (`self.DELTA_TIME`))) ; 時間が終わったら
  (if _newparam
    (`/Game/Play/Common/Fade/WBP_Fade.FadeInitialize` (`self.WBP_Fade`) "NewEnumerator0" 0.01)
    (set `self.mState` "NewEnumerator5")
    (`/Game/Play/Common/GroundObject/BP_Timer.fReset` (`self.mBP_CountTimer`))))

(event `OnlineRankingFadeIn`
  (if (`/Game/Play/Common/Fade/WBP_Fade.mEnd` (`self.WBP_Fade`))
    (`/Game/Play/Common/Fade/WBP_Fade.FadeInitialize` (`self.WBP_Fade`) "NewEnumerator1" 0.01)
    (`UserWidget.AddToViewport` (`self.WBP_LocalRanking`) 0) ; ローカルランキングの表示
    (`Widget.RemoveFromParent` (`self.WBP_OnlineRanking`)) ; オンラインランキングの非表示
    (set `self.mState` "NewEnumerator6")))

(event `OnlineRankingFadeOut`
  (if (`/Game/Play/Common/Fade/WBP_Fade.mEnd` (`self.WBP_Fade`))
    (set `self.mState` "NewEnumerator0")))

(event `EndFadeIn`)

(fn `fChackOnline`
  (returns (NewParam :type Boolean))
  (return (`|EnumInequality` (`/Game/DataRanking/WBP_OnLineRanking.mEN_SuccessState` (`self.WBP_OnlineRanking`)) "NewEnumerator1")))

(fn `UserConstructionScript`)