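; Debug game mode for the data ranking feature that switches between debug and ranking widgets.
; BeginPlay shows the online ranking debug widget, and DrawRanking2 replaces it with the online ranking widget.
; DrawRanking does the same swap for local ranking, but the code that creates the local debug widget is disconnected, so its DEBUG reference is never assigned here.
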(event `self.ReceiveBeginPlay`
  (bind _returnvalue (`|CreateWidget` "/Game/DataRanking/WBP_DEBUGOnLineRanking.WBP_DEBUGOnLineRanking_C"))
  (bind _output_get (set `self.DEBUG_2` _returnvalue))
  (`UserWidget.AddToViewport` _output_get 0))

(event `DrawRanking`
  (`Widget.RemoveFromParent` (`self.DEBUG`))
  (bind _returnvalue (`|CreateWidget` "/Game/DataRanking/WBP_LocalRanking.WBP_LocalRanking_C"))
  (`UserWidget.AddToViewport` _returnvalue 0))

(event `DrawRanking2`
  (`Widget.RemoveFromParent` (`self.DEBUG_2`))
  (bind _returnvalue (`|CreateWidget` "/Game/DataRanking/WBP_OnLineRanking.WBP_OnLineRanking_C"))
  (`UserWidget.AddToViewport` _returnvalue 0))

(fn `UserConstructionScript`)