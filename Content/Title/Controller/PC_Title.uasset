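; Title-screen player controller that handles mouse and gamepad input and drives the title camera.
; Input actions route to title, mode-select or pause-menu widgets by pause and widget state, while a spawned timer tracks the click interval for section selection.
; Key presses exit an active ranking display or restart the idle timer that flags the game mode.
; A looping timer makes the camera trail the target car, easing accumulated movement through lerp.
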(event `self.ReceiveBeginPlay`
  ;[1 1 1] タイマーの作成
  (bind _returnvalue (`|SpawnActorFromClass` "/Game/Play/Common/GroundObject/BP_Timer.BP_Timer_C" (`self.GetTransform`) "Undefined" "OverrideRootScale" null null))
  (bind _output_get (set `self.BP_ClickIntervalTimer` _returnvalue))
  (`/Game/Play/Common/GroundObject/BP_Timer.fSetMaxTime` _output_get (`self.CLICK_INTERVAL`))
  (`KismetSystemLibrary.K2_SetTimerDelegate` (delegate `ClickTimerUpdate`) (`/Game/Play/Common/GameMode/GM_DestructionCity.DELTA_TIME` (cast `/Game/Title/GameMode/GM_TitleCity` (`GameplayStatics.GetGameMode`) :!pure true)) true)
  (`self.ChackInput`))

(event `ClickTimerUpdate`
  (if (`self.mClickFlag`)
    (bind _newparam (`/Game/Play/Common/GroundObject/BP_Timer.fCountUp` (`self.BP_ClickIntervalTimer`) (`/Game/Play/Common/GameMode/GM_DestructionCity.DELTA_TIME` (cast `/Game/Title/GameMode/GM_TitleCity` (`GameplayStatics.GetGameMode`) :!pure true))))
    (if _newparam
      (set `self.mClickFlag` false))))

(event `InputAction|GameEnd`
  (params (Key :type "Key Structure"))
  ;[1 0 0] ゲーム終了処理
)

(event `PC_TitleCamera`
  (bind _mbp_camera (`/Game/Title/Controller/PC_Title.mBP_Camera` (cast `/Game/Title/Controller/PC_Title` (`GameplayStatics.GetPlayerController` 0) :!pure true)))
  (bind _returnvalue (+ (`self.K2_GetActorLocation` (`/Game/Title/GameMode/GM_TitleCity.mTargetCar` (cast `/Game/Title/GameMode/GM_TitleCity` (`GameplayStatics.GetGameMode`) :!pure true))) (`self.SHIFT_CAMERA_POS`)))
  ;[1 1 1] カメラ初期化処理(GMで呼び出し)
  (`self.K2_SetActorLocation` _mbp_camera _returnvalue false true) ; カメラを初期位置にセット
  (set `self.mTargetCameraVel` _returnvalue)
  (`self.K2_SetActorRotation` :`self` _mbp_camera)
  (`KismetSystemLibrary.K2_SetTimerDelegate` (delegate `CameraUpdate`) (`/Game/Play/Common/GameMode/GM_DestructionCity.DELTA_TIME` (cast `/Game/Title/GameMode/GM_TitleCity` (`GameplayStatics.GetGameMode`) :!pure true)) true) ; カメラ更新処理
)

(event `CameraUpdate`
  ;[1 1 1] カメラ初期化処理(GMで呼び出し)
  (if (`KismetSystemLibrary.IsValid` (`/Game/Title/Controller/PC_Title.mBP_Camera` (cast `/Game/Title/Controller/PC_Title` (`GameplayStatics.GetPlayerController` 0) :!pure true)))
    (`self.fTargetUpdate`)
    (`self.fCameraUpdate`)))

(event `InputAction|Building`
  (params (Key :type "Key Structure"))
  (:`Pressed`
    (if (not (and (`self.mClickFlag`) (`self.GetPause`)))
      (`/Game/Title/GameMode/BP_TitleManager.SelectSection` (`/Game/Title/GameMode/GM_TitleCity.fGetTitleManager` (cast `/Game/Title/GameMode/GM_TitleCity` (`GameplayStatics.GetGameMode`) :!pure true)))
      (set `self.mClickFlag` true)
      (if (`/Game/Play/Common/GameInstance/GMI_DestructionCIty.IsDEBUG` (cast `/Game/Play/Common/GameInstance/GMI_DestructionCIty` (`GameplayStatics.GetGameInstance`) :!pure true))
        (`KismetSystemLibrary.PrintString` "Click!" true false (struct :`R` 1.0 :`G` 0.145709 :`B` 0.017991 :`A` 1.0))))))

(event `ChackInput`
  (bind _asgm_title_city (cast `/Game/Title/GameMode/GM_TitleCity` (`GameplayStatics.GetGameMode`) :!pure true))
  (bind _mbp_titleranking (`/Game/Title/GameMode/GM_TitleCity.mBP_TitleRanking` (cast `/Game/Title/GameMode/GM_TitleCity` (`GameplayStatics.GetGameMode`) :!pure true)))
  (if (`/Game/Title/GameMode/BP_TitleDataRanking.mActiveFlag` _mbp_titleranking)
    (set `/Game/Title/GameMode/BP_TitleDataRanking.mTitleBackFlag` true _mbp_titleranking)
    (else
      (set `/Game/Title/GameMode/GM_TitleCity.mInputFlag` false _asgm_title_city)
      (`/Game/Play/Common/GroundObject/BP_Timer.fReset` (`/Game/Title/GameMode/GM_TitleCity.mBP_RankingTimer` _asgm_title_city)) ; タイマーリセット
      (bind _returnvalue (`KismetSystemLibrary.K2_SetTimerDelegate` (delegate `Update`) (`/Game/Play/Common/GameMode/GM_DestructionCity.DELTA_TIME` _asgm_title_city) true)))))

(event `Update`
  (bind _asgm_title_city (cast `/Game/Title/GameMode/GM_TitleCity` (`GameplayStatics.GetGameMode`) :!pure true))
  (if (`|EnumEquality` (`self.mEN_TitleWidgetState`) "NewEnumerator0")
    (bind _newparam (`/Game/Play/Common/GroundObject/BP_Timer.fCountUp` (`/Game/Title/GameMode/GM_TitleCity.mBP_RankingTimer` _asgm_title_city) (`/Game/Play/Common/GameMode/GM_DestructionCity.DELTA_TIME` _asgm_title_city)))
    (if _newparam
      (set `/Game/Title/GameMode/GM_TitleCity.mInputFlag` true _asgm_title_city)
      (`KismetSystemLibrary.K2_ClearAndInvalidateTimerHandle` (stale `ChackInput` _returnvalue)) ; タイマーを止める
    )))

(event `InputAction|GameStartButton`
  (params (Key :type "Key Structure"))
  (bind _asgm_title_city (cast `/Game/Title/GameMode/GM_TitleCity` (`GameplayStatics.GetGameMode`) :!pure true))
  (bind _mwbp_title (`/Game/Title/GameMode/GM_TitleCity.mWBP_Title` _asgm_title_city))
  ;[1 1 1] コントーラーのゲーム開始処理
  (:`Pressed`
    (if (`self.GetPause`)
      (switch `/Game/Title/EN_TitleWidgetState` (`self.mEN_TitleWidgetState`)
        (:`NewEnumerator0`
          (`/Engine/EditorBlueprintResources/StandardMacros.IsValid` _mwbp_title
            (:`Is Valid`
              (`/Game/Title/WBP_Title.GameStart` _mwbp_title))
            (:`Is Not Valid`
              (`/Game/Title/PackageTitle/WBP_PackageTitle.GameStart` (`/Game/Title/GameMode/GM_TitleCity.mWBP_PackageTitle` _asgm_title_city)))))
        (:`NewEnumerator2`
          (`/Game/Title/ModeSelect/WBP_ModeSelect.fGamePadStart` (`/Game/Title/GameMode/GM_TitleCity.mWBP_ModeSelect` _asgm_title_city)))))))

(event `Key|AnyKey`
  (params (Key :type "Key Structure"))
  ;[1 1 1] コントーラー入力処理
  (:`Pressed`
    (if (`self.GetPause`)
      (`self.ChackInput`)
      (if (and (`KismetInputLibrary.Key_IsGamepadKey` Key) (`|EnumEquality` (`self.mEN_TitleWidgetState`) "NewEnumerator2"))
        (`/Engine/EditorBlueprintResources/StandardMacros.DoOnce` false
          (:`Completed`
            (`/Game/Title/ModeSelect/WBP_ModeSelect.SelectBuildingDestroyMode` (`/Game/Title/GameMode/GM_TitleCity.mWBP_ModeSelect` (cast `/Game/Title/GameMode/GM_TitleCity` (`GameplayStatics.GetGameMode`) :!pure true))) ; 建築＆破壊モードを選択した状態に
          ))))))

(event `InputAction|Pause`
  (params (Key :type "Key Structure"))
  ;[1 1 1] ポーズを開く処理
  (:`Pressed`
    (`/Game/Pause/WBP_Pause.fChangeDraw` (`/Game/Play/Common/GameMode/GM_DestructionCity.mWBP_Pause` (cast `/Game/Play/Common/GameMode/GM_DestructionCity` (`GameplayStatics.GetGameMode`) :!pure true))) ; 表示切替処理
  ))

(event `InputAction|SelectUp`
  (params (Key :type "Key Structure"))
  ;[1 1 1] モード選択時のキー操作処理
  (:`Pressed`
    (if (and (`|EnumEquality` (`self.mEN_TitleWidgetState`) "NewEnumerator2") (`self.GetPause`))
      (`/Game/Title/ModeSelect/WBP_ModeSelect.fGamePadSelect` (`/Game/Title/GameMode/GM_TitleCity.mWBP_ModeSelect` (cast `/Game/Title/GameMode/GM_TitleCity` (`GameplayStatics.GetGameMode`) :!pure true)) -1))))

(event `InputAction|SelectDown`
  (params (Key :type "Key Structure"))
  ;[1 1 1] モード選択時のキー操作処理
  (:`Pressed`
    (if (and (`|EnumEquality` (`self.mEN_TitleWidgetState`) "NewEnumerator2") (`self.GetPause`))
      (`/Game/Title/ModeSelect/WBP_ModeSelect.fGamePadSelect` (`/Game/Title/GameMode/GM_TitleCity.mWBP_ModeSelect` (cast `/Game/Title/GameMode/GM_TitleCity` (`GameplayStatics.GetGameMode`) :!pure true)) 1))))

(event `InputAction|GameStartButton`
  (params (Key :type "Key Structure"))
  ;[1 1 1] ゲームパッドで何かしらの項目で決定ボタンを押した処理
  (:`Pressed`
    (if (`|EnumEquality` (`self.GetMPauseState`) "NewEnumerator0")
      (switch `/Game/Pause/EN_Pause` (`self.IsInstructionActive`) ; 説明書が開いた状態かどうか
        (:`NewEnumerator0`
          (`/Game/Pause/WBP_Pause.InstructionsReturn` (`self.GetWBP_Pause`)) ; 開いていたら説明書から戻る処理
        )
        (:`NewEnumerator1`
          (`/Game/Pause/WBP_Pause.fPauseDecision` (`self.GetWBP_Pause`)) ; ポーズメニューの決定処理
        )))))

(event `Key|AnyKey`
  (params (Key :type "Key Structure"))
  (bind _mwbp_pause (`self.GetWBP_Pause`))
  ;[1 1 1] ゲームパッドでいずれかのボタンを押されたとき
  (:`Pressed`
    (if (`KismetInputLibrary.Key_IsGamepadKey` Key)
      (if (`|EnumEquality` (`self.GetMPauseState`) "NewEnumerator0")
        (`/Game/Pause/WBP_Pause.PushGamePadAnyKey` _mwbp_pause) ; ポーズメニューで何かしらのキーを押したときの処理
        (set `self.bShowMouseCursor` false)
        (else
          (`/Game/Pause/WBP_Pause.ResetGamePadAnyKey` _mwbp_pause))))))

(event `InputAction|SelectUp`
  (params (Key :type "Key Structure"))
  (bind _mwbp_pause (`self.GetWBP_Pause`))
  ;[1 1 1] ゲームパッドのキー操作処理
  (:`Pressed`
    (if (`|EnumEquality` (`self.GetMPauseState`) "NewEnumerator0")
      (switch `/Game/Pause/EN_Pause` (`self.IsInstructionActive`) ; 説明書が開いた状態かどうか
        (:`NewEnumerator0`
          (`/Game/Pause/WBP_Pause.ShowInstructionsIconEmphasis` _mwbp_pause "Visible"))
        (:`NewEnumerator1`
          (`/Game/Pause/WBP_Pause.fGamePadSelect` _mwbp_pause -1))))))

(event `InputAction|SelectDown`
  (params (Key :type "Key Structure"))
  (bind _mwbp_pause (`self.GetWBP_Pause`))
  ;[1 1 1] ゲームパッドのキー操作処理
  (:`Pressed`
    (if (`|EnumEquality` (`self.GetMPauseState`) "NewEnumerator0")
      (switch `/Game/Pause/EN_Pause` (`self.IsInstructionActive`) ; 説明書が開いた状態かどうか
        (:`NewEnumerator0`
          (`/Game/Pause/WBP_Pause.ShowInstructionsIconEmphasis` _mwbp_pause "Visible"))
        (:`NewEnumerator1`
          (`/Game/Pause/WBP_Pause.fGamePadSelect` _mwbp_pause 1))))))

(event `InputAction|UpSoundGauge`
  (params (Key :type "Key Structure"))
  ;[1 1 1] ゲームパッド操作時の音量調整
  (:`Pressed`
    (switch `/Game/Pause/EN_Pause` (`self.IsInstructionActive`) ; 説明書が開いた状態かどうか
      (:`NewEnumerator1`
        (`/Game/Pause/WBP_Pause.GamePadChangeSoundVolume` (`self.GetWBP_Pause`) 0.1)))))

(event `InputAction|DownSoundGauge`
  (params (Key :type "Key Structure"))
  ;[1 1 1] ゲームパッド操作時の音量調整
  (:`Pressed`
    (switch `/Game/Pause/EN_Pause` (`self.IsInstructionActive`) ; 説明書が開いた状態かどうか
      (:`NewEnumerator1`
        (`/Game/Pause/WBP_Pause.GamePadChangeSoundVolume` (`self.GetWBP_Pause`) -0.1)))))

(fn `fCameraUpdate`
  (locals (SPRING_ARM :type "Float (double-precision)" :default 0.08))
  (bind _msavecameramovevel (`self.mSaveCameraMoveVel`))
  (bind _returnvalue (`self.K2_GetActorLocation` (`/Game/Title/Controller/PC_Title.mBP_Camera` (cast `/Game/Title/Controller/PC_Title` (`GameplayStatics.GetPlayerController` 0) :!pure true))))
  (if (`KismetMathLibrary.NotEqualExactly_VectorVector` (`self.mSaveCameraMoveVel`))
    (`self.K2_SetActorLocation` (`/Game/Title/Controller/PC_Title.mBP_Camera` (cast `/Game/Title/Controller/PC_Title` (`GameplayStatics.GetPlayerController` 0) :!pure true)) (`KismetMathLibrary.VLerp` _returnvalue (+ _returnvalue (`self.mSaveCameraMoveVel`)) (`local.SPRING_ARM`)) false true)
    (set `self.mSaveCameraMoveVel` (- _msavecameramovevel (* _msavecameramovevel (`local.SPRING_ARM`))))))

(fn `fCreateBuildingController`
  (set `self.mBP_Camera` (cast `/Game/Title/Controller/BP_TitleCamera` (`GameplayStatics.GetPlayerPawn` 0) :!pure true))
  (set `self.bShowMouseCursor` true) ; マウスカーソルを表示する
  (set `self.bEnableClickEvents` true) ; クリックイベントを有効にする
  (set `self.ClickEventKeys` (`self.mBuildingClickKeys`)) ; 使用するキーを設定
)

(fn `fTargetUpdate`
  (bind _returnvalue (* (`/Game/Play/Common/GroundObject/Car/BP_CarBase.mMoveDistance` (`/Game/Title/GameMode/GM_TitleCity.mTargetCar` (cast `/Game/Title/GameMode/GM_TitleCity` (`GameplayStatics.GetGameMode`) :!pure true))) (`/Game/Title/Controller/BP_TitleCamera.mCameraMoveSpeed` (`self.mBP_Camera`))))
  ;[1 1 1] 値が入っているときのみ処理
  (if (`KismetMathLibrary.NotEqualExactly_VectorVector` _returnvalue)
    (set `self.mSaveCameraMoveVel` (+ (`self.mSaveCameraMoveVel`) _returnvalue))
    (set `self.mTargetCameraVel` (+ _returnvalue (`self.K2_GetActorLocation` (`self.mBP_Camera`))))))

(fn `UserConstructionScript`)