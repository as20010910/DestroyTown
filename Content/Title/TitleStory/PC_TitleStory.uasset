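; Player controller for the title story screen, handling cursor setup and the screen's input actions.
; On BeginPlay it shows the mouse cursor and enables click events.
; GameEnd quits the game, and Decision calls SkipStory on the story widget held by GM_TitleStory.
; Pause toggles the MPause state in GMI_DestructionCIty and shows or hides the game mode's pause widget to match, without pausing the game itself.
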(event `self.ReceiveBeginPlay`
  (set `self.bShowMouseCursor` true) ; マウスカーソルを表示する
  (set `self.bEnableClickEvents` true) ; クリックイベントを有効にする
)

(event `InputAction|GameEnd`
  (params (Key :type "Key Structure"))
  ;[1 0 0] ゲーム終了処理
  (:`Pressed`
    (`KismetSystemLibrary.QuitGame` null "Quit")))

(event `InputAction|Decision`
  (params (Key :type "Key Structure"))
  ;[1 1 1] ストーリ―をスキップする
  (:`Pressed`
    (`/Game/Play/Story/WBP_Story.SkipStory` (`/Game/Title/TitleStory/GM_TitleStory.mWBP_Story` (cast `/Game/Title/TitleStory/GM_TitleStory` (`GameplayStatics.GetGameMode`) :!pure true)))))

(event `InputAction|Pause`
  (params (Key :type "Key Structure"))
  (bind _asgmi_destruction_city (cast `/Game/Play/Common/GameInstance/GMI_DestructionCIty` (`GameplayStatics.GetGameInstance`) :!pure true))
  (bind _mwbp_pause (`/Game/Title/TitleStory/GM_TitleStory.mWBP_Pause` (cast `/Game/Title/TitleStory/GM_TitleStory` (`GameplayStatics.GetGameMode`) :!pure true)))
  (:`Pressed`
    (if (`|EnumEquality` (`/Game/Play/Common/GameInstance/GMI_DestructionCIty.mPause` (cast `/Game/Play/Common/GameInstance/GMI_DestructionCIty` (`GameplayStatics.GetGameInstance`) :!pure true)) "NewEnumerator0")
      (set `/Game/Play/Common/GameInstance/GMI_DestructionCIty.mPause` "NewEnumerator1" _asgmi_destruction_city)
      ;[1 1 1] 表示切替処理
      (`Widget.SetVisibility` _mwbp_pause "Hidden")
      (else
        (set `/Game/Play/Common/GameInstance/GMI_DestructionCIty.mPause` "NewEnumerator0" _asgmi_destruction_city)
        (`Widget.SetVisibility` _mwbp_pause "Visible")))))

(fn `UserConstructionScript`)