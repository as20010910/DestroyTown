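; Destructible building actor for the title screen that breaks apart when damaged and fades out.
; BuildingApplyDamage passes damage and impulse to the destructible component, whose fracture event starts a looping timer at the GameMode's DELTATIME.
; Each tick lowers the materials' Opacity parameter, then sets a destroy flag at zero; the DestroyActor call is unwired.
; Helpers fetch building data and swap meshes through GameMode-owned data table managers.
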(event `BuildingApplyDamage`
  (params (AttackDamage :type "Float (double-precision)") (ImpluseDir :type "Vector Structure") (ImpulseStrength :type "Float (double-precision)"))
  ;[1 1 1] 建物にダメージを与える処理
  (`DestructibleComponent.ApplyDamage` (`self.Building`) AttackDamage (+ (`self.K2_GetActorLocation`) (`self.mDamageShiftPos`)) ImpluseDir ImpulseStrength))

(event `self.Building.OnComponentFracture`
  (params (HitPoint :type "Vector Structure (by ref)") (HitDirection :type "Vector Structure (by ref)"))
  ;[1 1 1] 建物が壊された時の処理
  ;;[1 1 1] タイトル用爆破処理
  (`KismetSystemLibrary.K2_SetTimerDelegate` (delegate `TitleTransparentBuilding`) (`/Game/Play/Common/GameMode/GM_DestructionCity.DELTA_TIME` (cast `/Game/Play/Common/GameMode/GM_DestructionCity` (`GameplayStatics.GetGameMode`) :!pure true)) true))

(event `TitleTransparentBuilding`
  (bind _returnvalue (- (`self.mNowMatAlpha`) (/ (`self.CLEAR_SPEED`) 8.0)))
  ;[1 1 1] 建物が壊された時の処理
  ;;[1 1 1] タイトル用爆破処理
  ;;;[1 1 1] 透過処理
  (set `self.mNowMatAlpha` _returnvalue) ; α値を減少させる
  (if (<= _returnvalue 0.0)
    (set `self.mDestroyFlag` true)
    (else
      (`self.fClear` _returnvalue) ; 透過処理
    )))

(fn `fClear`
  (params (ParameterValue :type "Float (double-precision)"))
  ;[1 1 1] 透明度の指定
  (`MeshComponent.SetScalarParameterValueOnMaterials` (`self.Building`) "Opacity" ParameterValue))

(fn `fGetBuildingData`
  (returns (NewParam :type "/Game/Play/Building/Data/ST_BuildingDataTable Structure"))
  ;[1 1 1] 建物データを取得する
  (bind _asgm_destruction_city (cast `/Game/Play/Common/GameMode/GM_DestructionCity` (`GameplayStatics.GetGameMode`)))
  (bind _value (`/Game/Play/Building/Data/BP_BuildingDataTableManager.fMap` (`/Game/Play/Destruction/BP_DestructionManager.mBP_BuildingDataTableManager` (`/Game/Play/Common/GameMode/GM_DestructionCity.mBP_DestructionManager` _asgm_destruction_city)) (`self.mBuilding`))) ; 建物に対応するデータテーブルを取得
  (return _value))

(fn `fResetMaterials`
  (bind _building (`self.Building`))
  (for (_ _array_index) (`MeshComponent.GetMaterials` _building)
    (`PrimitiveComponent.SetMaterial` _building _array_index null)))

(fn `fSetMesh`
  (params (NewParam :type "/Game/Play/Building/Data/EN_Building Enum" :default "NewEnumerator13"))
  (if (`|EnumEquality` NewParam "NewEnumerator13")
    (`DestructibleComponent.SetDestructibleMesh` (`self.Building`) null)
    (else
      (bind _value (`/Game/Play/Building/Data/BP_BuildingDataTableManager.fMap` (`/Game/Play/Building/BP_BuildingManager.mBP_BuildingDataTableManager` (`/Game/Play/Common/GameMode/GM_DestructionCity.mBP_BuildingManager` (cast `/Game/Play/Common/GameMode/GM_DestructionCity` (`GameplayStatics.GetGameMode`) :!pure true))) NewParam))
      (`DestructibleComponent.SetDestructibleMesh` (`self.Building`) (`.DestructibleMesh_28_C4AEC3F449FA69CAC7814881C59E681D` (break `/Game/Play/Building/Data/ST_BuildingDataTable` _value)))
      (`self.fResetMaterials`) ; マテリアル情報をリセットする
    )))

(fn `UserConstructionScript`)