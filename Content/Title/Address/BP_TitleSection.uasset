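; Title-screen city plot that manages one BP_TItleBuilding child actor through building, house-to-mansion development, destruction and respawn.
; FCompleteBuilding picks build or develop from MAfterCreate, taking new meshes from the GM_DestructionCity building data table.
; FBreakBuilding applies radial damage and an explosion, then a timer polls the destroy flag to recreate the child actor.
; A looping timer also sets a visibility flag by comparing camera-to-plot angle against a threshold.
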(event `self.ReceiveBeginPlay`
  (`KismetSystemLibrary.K2_SetTimerDelegate` (delegate `cusotm`) (`/Game/Play/Common/GameMode/GM_DestructionCity.DELTA_TIME` (cast `/Game/Play/Common/GameMode/GM_DestructionCity` (`GameplayStatics.GetGameMode`) :!pure true)) true))

(event `cusotm`
  (`self.fIsInView`))

(event `SetHouseBuilding`
  (bind _asbp_building_base (`self.fGetBuildingBase`))
  ;[1 1 1] 家作成処理
  ;;[1 1 1] 生成後情報から細かい情報を取得
  (bind _value (`/Game/Play/Building/Data/BP_BuildingDataTableManager.fMap` (`/Game/Play/Building/BP_BuildingManager.mBP_BuildingDataTableManager` (`/Game/Play/Common/GameMode/GM_DestructionCity.mBP_BuildingManager` (cast `/Game/Play/Common/GameMode/GM_DestructionCity` (`GameplayStatics.GetGameMode`) :!pure true))) (`self.mAfterCreate`)))
  (set `self.mHouseFlag` true)
  (set `self.mState` "NewEnumerator2") ; 状態を家状態に
  ;;[1 1 1] モデルを設定
  (`/Game/Title/Address/BP_TItleBuilding.fSetMesh` _asbp_building_base (break `/Game/Play/Building/Data/ST_BuildingDataTable` _value))
  (`/Game/Title/Address/BP_TItleBuilding.fClear` _asbp_building_base 1.0)
  (set `/Game/Title/Address/BP_TItleBuilding.mBuilding` (break `/Game/Play/Building/Data/ST_BuildingDataTable` _value) (`self.fGetBuildingBase`)))

(event `SetOtherBuilding`
  (bind _asbp_building_base (`self.fGetBuildingBase`))
  ;[1 1 1] 家以外作成処理
  ;;[1 1 1] 生成後情報から細かい情報を取得
  (bind _value (`/Game/Play/Building/Data/BP_BuildingDataTableManager.fMap` (`/Game/Play/Building/BP_BuildingManager.mBP_BuildingDataTableManager` (`/Game/Play/Common/GameMode/GM_DestructionCity.mBP_BuildingManager` (cast `/Game/Play/Common/GameMode/GM_DestructionCity` (`GameplayStatics.GetGameMode`) :!pure true))) (`self.mAfterCreate`)))
  (set `self.mHouseFlag` true)
  (set `self.mState` "NewEnumerator1") ; 状態を完成状態に
  ;;[1 1 1] モデルを設定
  (`/Game/Title/Address/BP_TItleBuilding.fSetMesh` _asbp_building_base (break `/Game/Play/Building/Data/ST_BuildingDataTable` _value))
  (`/Game/Title/Address/BP_TItleBuilding.fClear` _asbp_building_base 1.0)
  (set `/Game/Title/Address/BP_TItleBuilding.mBuilding` (break `/Game/Play/Building/Data/ST_BuildingDataTable` _value) (`self.fGetBuildingBase`)))

(event `SetDevelopment`
  (bind _asbp_building_base (`self.fGetBuildingBase`))
  ;[1 1 1] 建物発展処理
  (switch `/Game/Play/Building/Data/EN_Building` (`self.mAfterCreate`)
    (:`NewEnumerator0`
      ;;[1 1 1] モデルを設定
      (`/Game/Title/Address/BP_TItleBuilding.fSetMesh` (`self.fGetBuildingBase`) "NewEnumerator1")
      (set `/Game/Title/Address/BP_TItleBuilding.mBuilding` "NewEnumerator1" _asbp_building_base) ; 建物の種類を保存
    )
    (:`NewEnumerator2`
      (`/Game/Title/Address/BP_TItleBuilding.fSetMesh` (`self.fGetBuildingBase`) "NewEnumerator3")
      (set `/Game/Title/Address/BP_TItleBuilding.mBuilding` "NewEnumerator3" _asbp_building_base) ; 建物の種類を保存
    )
    (:`NewEnumerator4`
      (`/Game/Title/Address/BP_TItleBuilding.fSetMesh` (`self.fGetBuildingBase`) "NewEnumerator5")
      (set `/Game/Title/Address/BP_TItleBuilding.mBuilding` "NewEnumerator5" _asbp_building_base) ; 建物の種類を保存
    ))
  (`/Game/Title/Address/BP_TItleBuilding.fClear` _asbp_building_base 1.0)
  (set `self.mState` "NewEnumerator1"))

(event `ChackDestroyUpdate`
  (bind _returnvalue (`KismetSystemLibrary.K2_SetTimerDelegate` (delegate `ChackUpdate`) (`/Game/Play/Common/GameMode/GM_DestructionCity.DELTA_TIME` (cast `/Game/Title/GameMode/GM_TitleCity` (`GameplayStatics.GetGameMode`) :!pure true)) true)))

(event `ChackUpdate`
  (bind _finishflag (`self.fRefreshBuilding`))
  (if _finishflag
    (`KismetSystemLibrary.K2_ClearAndInvalidateTimerHandle` (stale `ChackDestroyUpdate` _returnvalue)) ; 再生したら処理終了
  ))

(fn `F Complete Building`
  (switch `/Game/Play/Building/Data/EN_Building` (`self.mAfterCreate`)
    (:`NewEnumerator0`
      (if (`self.mHouseFlag`) :!label _label
        (`self.SetDevelopment`) ; 家なら発展処理
        (else
          (`self.SetHouseBuilding`) ; 家なら家を建てる処理
        )))
    (:`NewEnumerator2`
      (goto _label))
    (:`NewEnumerator4`
      (goto _label))
    (:`NewEnumerator6`
      (`self.SetOtherBuilding` :!label _label_2))
    (:`NewEnumerator11`
      (goto _label_2))
    (:`NewEnumerator14`
      (goto _label_2))))

(fn `fBreakBuilding`
  (locals (ATTACK_NUM :type "Float (double-precision)" :default 500.0) (EFFECT_SCALE :type "Vector Structure" :default (0.3 0.3 0.3)))
  (bind (_returnvalue_location _returnvalue_rotation) (`KismetMathLibrary.BreakTransform` (`self.GetTransform`)))
  (bind _building (`/Game/Title/Address/BP_TItleBuilding.Building` (cast `/Game/Title/Address/BP_TItleBuilding` (`ChildActorComponent.ChildActor` (`self.BP_BuildingBase`)) :!pure true)))
  (set `self.mBreakFlag` true)
  (`/Engine/EditorBlueprintResources/StandardMacros.IsValid` _building
    (:`Is Valid`
      (`DestructibleComponent.ApplyRadiusDamage` _building (`local.ATTACK_NUM`) (+ (`self.K2_GetActorLocation`) (0.0 0.0 10.0)) 1.0 12500.0 true)
      (`GameplayStatics.SpawnEmitterAtLocation` "/Game/Title/Effect/Particles/Explosion/Fire_Exp_00.Fire_Exp_00" _returnvalue_location _returnvalue_rotation (`local.EFFECT_SCALE`))
      (`self.ChackDestroyUpdate`)
      (set `self.mState` "NewEnumerator0")
      (set `self.mAfterCreate` "NewEnumerator13")
      (set `self.mHouseFlag` false))))

(fn `fGetBuildingBase`
  (returns (`AsBP Building Base` :type "/Game/Title/Address/BP_TItleBuilding Object Reference"))
  (return (cast `/Game/Title/Address/BP_TItleBuilding` (`ChildActorComponent.ChildActor` (`self.BP_BuildingBase`)) :!pure true)))

(fn `fIsInView`
  (locals (THRESHOLD_ANGLE :type "Float (double-precision)" :default 30.0))
  (bind _returnvalue (`GameplayStatics.GetPlayerCameraManager` 0))
  (bind _returnvalue_2 (`KismetMathLibrary.DegAcos` (`KismetMathLibrary.Dot_VectorVector` (`SceneComponent.GetForwardVector` (`PlayerCameraManager.TransformComponent` _returnvalue)) (`KismetMathLibrary.GetForwardVector` (`KismetMathLibrary.FindLookAtRotation` (`self.K2_GetActorLocation` _returnvalue) (`self.K2_GetActorLocation`))))))
  (set `self.DEBUGF` _returnvalue_2)
  (set `self.mVisibleFlag` (< _returnvalue_2 (`KismetSystemLibrary.MakeLiteralDouble` (`local.THRESHOLD_ANGLE`)))))

(fn `fRefreshBuilding`
  (returns (FinishFlag :type Boolean))
  (if (`/Game/Title/Address/BP_TItleBuilding.mDestroyFlag` (cast `/Game/Title/Address/BP_TItleBuilding` (`ChildActorComponent.ChildActor` (`self.BP_BuildingBase`)) :!pure true))
    (set `self.mBreakFlag` false) ; 破壊時フラグを下す
    (`ChildActorComponent.SetChildActorClass` (`self.BP_BuildingBase`) "/Game/Title/Address/BP_TItleBuilding.BP_TItleBuilding_C")
    (return true)
    (else
      (return false))))

(fn `UserConstructionScript`)