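; Title-screen manager that animates the background city with changing buildings and cars.
; FTitleCreateManager spawns the building data, address, warp and car-creation managers, linking warp into car creation.
; A looping timer drives a state machine that, when the car-out flag is set, fades, recreates cars and resets the camera.
; SelectSection picks a random visible, unbroken section to build, evolve or demolish, remapping mansion picks to other building types.
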(event `self.ReceiveBeginPlay`
  ;[1 1 1] 区画の保存
  (bind _outactors (`GameplayStatics.GetAllActorsOfClass` "/Game/Title/Address/BP_TitleSection.BP_TitleSection_C")) ; 全ての区画を取得、保存する
  (set `self.mAllSections` _outactors)
  ;[1 1 1] 車更新用フェードの作成
  (bind _returnvalue (`|CreateWidget` "/Game/Play/Common/Fade/WBP_Fade.WBP_Fade_C"))
  (bind _output_get (set `self.WBP_CarRenewalFade` _returnvalue))
  (`UserWidget.AddToViewport` _output_get 0)
  (`KismetSystemLibrary.K2_SetTimerDelegate` (delegate `CarChackUpdate`) (`/Game/Play/Common/GameMode/GM_DestructionCity.DELTA_TIME` (cast `/Game/Title/GameMode/GM_TitleCity` (`GameplayStatics.GetGameMode`) :!pure true)) true))

(event `CarChackUpdate`
  (bind _asgm_title_city (cast `/Game/Title/GameMode/GM_TitleCity` (`GameplayStatics.GetGameMode`) :!pure true))
  (switch `/Game/Title/GameMode/EN_CarRenewalState` (`self.mEN_CarState`)
    (:`NewEnumerator6`
      (if (`self.mCarOutFlag`)
        (set `self.mEN_CarState` "NewEnumerator0")))
    (:`NewEnumerator0`
      (`/Game/Play/Common/Fade/WBP_Fade.FadeInitialize` (`self.WBP_CarRenewalFade`) "NewEnumerator0" 0.01)
      (set `self.mEN_CarState` "NewEnumerator1"))
    (:`NewEnumerator1`
      (if (`/Game/Play/Common/Fade/WBP_Fade.mEnd` (`self.WBP_CarRenewalFade`))
        (set `self.mEN_CarState` "NewEnumerator2")))
    (:`NewEnumerator2`
      (`/Game/Title/GameMode/GM_TitleCity.InitCarCreate` _asgm_title_city)
      (`/Game/Title/GameMode/GM_TitleCity.fCreateInitCar` _asgm_title_city)
      (`/Game/Title/Controller/PC_Title.PC_TitleCamera` (cast `/Game/Title/Controller/PC_Title` (`GameplayStatics.GetPlayerController` 0) :!pure true)) ; カメラ初期化処理
      (set `self.mEN_CarState` "NewEnumerator3"))
    (:`NewEnumerator3`
      (`/Game/Play/Common/Fade/WBP_Fade.FadeInitialize` (`self.WBP_CarRenewalFade`) "NewEnumerator1" 0.01)
      (set `self.mEN_CarState` "NewEnumerator4"))
    (:`NewEnumerator4`
      (if (`/Game/Play/Common/Fade/WBP_Fade.mEnd` (`self.WBP_CarRenewalFade`))
        (set `self.mEN_CarState` "NewEnumerator5")))
    (:`NewEnumerator5`
      (set `self.mCarOutFlag` false)
      (set `self.mEN_CarState` "NewEnumerator6"))))

(event `SelectSection`
  ;[1 1 1] 建物ランダム生成爆破処理
  (bind _output (`self.fGetOnScreenSection`))
  (`/Engine/EditorBlueprintResources/StandardMacros.IsValid` _output
    (:`Is Valid`
      (switch `/Game/Play/Building/Address/Section/EN_SectionState` (`/Game/Title/Address/BP_TitleSection.mState` _output)
        (:`NewEnumerator0`
          (bind _newparam (`self.F Rand Get Small Square`))
          (set `/Game/Title/Address/BP_TitleSection.mAfterCreate` _newparam _output)
          (`/Game/Title/Address/BP_TitleSection.F Complete Building` _output :!label _label))
        (:`NewEnumerator2`
          (if (`KismetMathLibrary.RandomBool`)
            (goto _label)
            (else
              (`/Game/Title/Address/BP_TitleSection.fBreakBuilding` _output))))
        (:`NewEnumerator1`
          (`/Game/Title/Address/BP_TitleSection.fBreakBuilding` _output))))))

(fn `F Rand Get Small Square`
  (returns (NewParam :type "/Game/Play/Building/Data/EN_Building Enum"))
  (locals (randNum :type Integer))
  (bind _output_get (set `local.randNum` (`KismetMathLibrary.RandomInteger` 6)))
  (switch `/Game/Play/Building/Data/EN_Building` (cast `/Game/Play/Building/Data/EN_Building` (`KismetMathLibrary.Conv_IntToByte` _output_get)) ; 表示されているものしか選ばれない
    (:`NewEnumerator13`
      (return "NewEnumerator14") ; なしは金色家に
    )
    (:`NewEnumerator0`
      _)
    (:`NewEnumerator1`
      (return "NewEnumerator6") ; 木造マンションは商店に
    )
    (:`NewEnumerator2`
      _)
    (:`NewEnumerator3`
      (return "NewEnumerator11") ; レンガマンションは風車に
    )
    (:`NewEnumerator4`
      _))
  (return (cast `/Game/Play/Building/Data/EN_Building` (`KismetMathLibrary.Conv_IntToByte` (`local.randNum`)))) ; マンション以外はそのまま返す
)

(fn `fCreateInitCar`)

(fn `fGetOnScreenSection`
  (returns (Output :type "/Game/Title/Address/BP_TitleSection Object Reference"))
  (locals (instantSectionArray :type "Array of /Game/Title/Address/BP_TitleSection Object Reference"))
  (for _array_element (`self.mAllSections`)
    (if (`/Game/Title/Address/BP_TitleSection.mVisibleFlag` _array_element)
      (if (not (`/Game/Title/Address/BP_TitleSection.mBreakFlag` _array_element))
        (`KismetArrayLibrary.Array_Add` (`local.instantSectionArray`) _array_element))))
  (return (`|GetArrayItem` (`local.instantSectionArray`) (`KismetMathLibrary.RandomInteger` (`KismetArrayLibrary.Array_Length` (`local.instantSectionArray`))))))

(fn `fTitleCreateManager`
  ;[1 1 1] データ管理クラスの作成
  (bind _returnvalue (`|SpawnActorFromClass` "/Game/Play/Building/Data/BP_BuildingDataTableManager.BP_BuildingDataTableManager_C" (`KismetMathLibrary.MakeTransform` (0.0 0.0 0.0)) "Undefined" "OverrideRootScale" null null))
  (set `self.mBP_BuildingDataTableManager` _returnvalue)
  ;[1 1 1] 区画管理クラスの作成
  (bind _returnvalue_2 (`|SpawnActorFromClass` "/Game/Play/Building/Address/BP_AddressManager.BP_AddressManager_C" (`KismetMathLibrary.MakeTransform` (0.0 0.0 0.0)) "Undefined" "OverrideRootScale" null null))
  (set `self.mBP_AddressManager` _returnvalue_2)
  ;[1 1 1] 車関連の生成処理
  ;;[1 1 1] 車転移管理クラスの生成処理
  (bind _returnvalue_3 (`|SpawnActorFromClass` "/Game/Play/Common/GroundObject/WarpPoint/BP_WarpManager.BP_WarpManager_C" (`KismetMathLibrary.MakeTransform` (0.0 0.0 0.0)) "Undefined" "OverrideRootScale" null null))
  (bind _output_get (set `self.mBP_WarpManager` _returnvalue_3))
  ;;[1 1 1] 車生成管理クラスの生成処理
  (bind _returnvalue_4 (`|SpawnActorFromClass` "/Game/Play/Common/GroundObject/Car/BP_CarCreateManager.BP_CarCreateManager_C" (`KismetMathLibrary.MakeTransform` (0.0 0.0 0.0)) "Undefined" "OverrideRootScale" null null))
  (bind _output_get_2 (set `self.mBP_CarCreateManager` _returnvalue_4))
  (`/Game/Play/Common/GroundObject/Car/BP_CarCreateManager.fSetCarMoveVel` _output_get_2 (`self.TITLE CAR MOVE VEL`))
  (`/Game/Play/Common/GroundObject/Car/BP_CarCreateManager.SetWarpManager` _output_get_2 _output_get))

(fn `UserConstructionScript`
  (`parent.UserConstructionScript`))