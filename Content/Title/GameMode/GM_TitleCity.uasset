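; Title-level game mode that stages a city backdrop and runs the sequence from title screen through story prologue into the stage level.
; BeginPlay spawns BP_TitleManager, sets up player controller and camera, creates title and fade widgets, and starts BGM.
; Initial car creation picks a target car and triggers building generation on randomly chosen sections.
; A looping timer drives the fade and prologue state machine, swapping recollection music before opening the stage.
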(event `self.ReceiveBeginPlay`
  ;[1 1 1] 全体管理クラス作成
  (bind _returnvalue (`|SpawnActorFromClass` "/Game/Title/GameMode/BP_TitleManager.BP_TitleManager_C" (`KismetMathLibrary.MakeTransform` (0.0 0.0 0.0)) "Undefined" "OverrideRootScale" null null))
  (set `self.mBP_BuildingManager` _returnvalue)
  (`/Game/Title/GameMode/BP_TitleManager.fTitleCreateManager` (`self.fGetTitleManager`)) ; 管理マネージャの作成
  (`/Game/Title/Controller/PC_Title.fCreateBuildingController` (cast `/Game/Title/Controller/PC_Title` (`GameplayStatics.GetPlayerController` 0) :!pure true)) ; 操作周りの生成処理
  (`self.InitCarCreate`) ; 視点車生成処理
  (`self.fCreateInitCar`) ; 最初の車生成処理
  (`/Game/Title/Controller/PC_Title.PC_TitleCamera` (cast `/Game/Title/Controller/PC_Title` (`GameplayStatics.GetPlayerController` 0) :!pure true)) ; カメラ初期化処理
  ;[1 1 1] UI生成処理
  (bind _returnvalue_2 (`|CreateWidget` "/Game/Title/WBP_Title.WBP_Title_C"))
  (bind _output_get (set `self.mWBP_Title` _returnvalue_2))
  (`UserWidget.AddToViewport` _output_get 0)
  (bind _returnvalue_3 (`|CreateWidget` "/Game/Play/Common/Fade/WBP_Fade.WBP_Fade_C"))
  (bind _output_get_2 (set `self.mWBP_Fade_0` _returnvalue_3))
  (`UserWidget.AddToViewport` _output_get_2 100)
  ;[1 1 1] BGM再生
  (bind _returnvalue_4 (`GameplayStatics.SpawnSound2D` "/Game/Title/Sound/BGM/BGM_Title.BGM_Title" 1.0 1.0 0.0 null))
  (set `self.mBGM_Title` _returnvalue_4)
  (`KismetSystemLibrary.K2_SetTimerDelegate` (delegate `TitleUpdate`) (`self.DELTA_TIME`) true) ; タイトルの更新処理
)

(event `TitleUpdate`
  (bind _mwbp_fade_0 (`self.mWBP_Fade_0`))
  (switch `/Game/Title/EN_Titlestate` (`self.mTItleState`)
    (:`NewEnumerator1`
      (if (`/Game/Play/Common/Fade/WBP_Fade.mEnd` _mwbp_fade_0)
        (`/Game/Play/Common/Fade/WBP_Fade.FadeInitialize` _mwbp_fade_0 "NewEnumerator1" 0.01)
        (set `self.mTItleState` "NewEnumerator2")
        ;[1 1 1] 回想シーン用
        (bind _returnvalue (`|CreateWidget` "/Game/Play/Story/WBP_Story.WBP_Story_C"))
        (bind _output_get (set `self.mWBP_Story` _returnvalue))
        (`UserWidget.AddToViewport` _output_get 10)
        (`AudioComponent.Stop` (`self.mBGM_Title`))
        (bind _returnvalue_2 (`GameplayStatics.SpawnSound2D` "/Game/Title/Sound/BGM/BGM_TitleRecollection1.BGM_TitleRecollection1" 1.0 1.0 0.0 null))
        (set `self.BGM_TitleRecollection1` _returnvalue_2)))
    (:`NewEnumerator2`
      (if (`/Game/Play/Common/Fade/WBP_Fade.mEnd` _mwbp_fade_0)
        (set `self.mTItleState` "NewEnumerator3") ; 回想へ
      ))
    (:`NewEnumerator3`
      (if (and (== (`/Game/Play/Story/WBP_Story.mNowStoryImageNum` (`self.mWBP_Story`)) 3) (`AudioComponent.IsPlaying` (`self.BGM_TitleRecollection1`)))
        (`AudioComponent.SetPaused` (`self.BGM_TitleRecollection1`) true)
        (bind _returnvalue_3 (`GameplayStatics.SpawnSound2D` "/Game/Title/Sound/BGM/BGM_TitleRecollection2.BGM_TitleRecollection2" 1.0 1.0 0.0 null))
        (set `self.BGM_TitleRecollection2` _returnvalue_3)
        (elif (`/Game/Play/Story/WBP_Story.IsStoryEnd` (`self.mWBP_Story`))
          (`GameplayStatics.OpenLevelBySoftObjectPtr` "/Game/Play/Stage/LBP_α-Stage.LBP_α-Stage"))))))

(event `InitCarCreate`
  (bind _mbp_carcreatemanager (`/Game/Play/Building/BP_BuildingManager.mBP_CarCreateManager` (`/Game/Play/Common/GameMode/GM_DestructionCity.mBP_BuildingManager` (cast `/Game/Play/Common/GameMode/GM_DestructionCity` (`GameplayStatics.GetGameMode`) :!pure true))))
  (bind _result (`/Engine/EditorBlueprintResources/StandardMacros.IncrementInt` (`/Game/Play/Common/GroundObject/Car/BP_CarCreateManager.mCarCreateNum` _mbp_carcreatemanager))
    (:`  `
      (set `/Game/Play/Common/GroundObject/Car/BP_CarCreateManager.mCarCreateNum` _result _mbp_carcreatemanager)
      (set `/Game/Play/Common/GroundObject/Car/BP_CarCreateManager.CarCreateFlag` true _mbp_carcreatemanager))))

(fn `fCreateInitBuilding`
  (locals (allSections :type "Array of /Game/Title/Address/BP_TitleSection Object Reference") (CREATE_RATIO :type "Float (double-precision)" :default 0.3) (CreateNum :type Integer) (createSections :type "Array of /Game/Title/Address/BP_TitleSection Object Reference"))
  (`|ExecutionSequence`
    (:`then_0`
      (bind _outactors (`GameplayStatics.GetAllActorsOfClass` "/Game/Title/Address/BP_TitleSection.BP_TitleSection_C")) ; 全ての区画を取得、保存する
      (bind _output_get (set `local.allSections` _outactors))
      ;[1 1 1] 生成数を準備
      (set `local.CreateNum` (`KismetMathLibrary.FTrunc` (* (`KismetArrayLibrary.Array_Length` _output_get) (`local.CREATE_RATIO`)))))
    (:`then_1`
      (for _ (range (+ (`local.CreateNum`) 1))
        ;[1 1 1] 乱数で配列番号を指定、生成区画を指定
        (`KismetArrayLibrary.Array_Add` (`local.createSections`) (`|GetArrayItem` (`local.allSections`) (`KismetMathLibrary.RandomInteger` (`KismetArrayLibrary.Array_Length` (`local.allSections`)))))))
    (:`then_2`
      (for _array_element (`local.createSections`)
        (if (`|EnumEquality` (`/Game/Title/Address/BP_TitleSection.mState` _array_element) "NewEnumerator0")
          (bind _newparam (`/Game/Title/GameMode/BP_TitleManager.F Rand Get Small Square` (cast `/Game/Title/GameMode/BP_TitleManager` (`self.mBP_BuildingManager`) :!pure true))) ; 乱数で建物を指定する
          (set `/Game/Title/Address/BP_TitleSection.mAfterCreate` _newparam _array_element)
          (`/Game/Title/Address/BP_TitleSection.F Complete Building` _array_element) ; 生成する
        )))))

(fn `fCreateInitCar`
  (locals (CAR_VEL :type "Float (double-precision)" :default 1.0) (COUNT_NUM :type "Float (double-precision)" :default 1000.0))
  (bind _mbp_carcreatemanager (`/Game/Play/Building/BP_BuildingManager.mBP_CarCreateManager` (`self.mBP_BuildingManager`)))
  (`/Game/Play/Common/GroundObject/Car/BP_CarCreateManager.fCarCreate` _mbp_carcreatemanager (`local.COUNT_NUM`) (`local.CAR_VEL`)) ; 最初の車生成
  ;[1 1 1] 生成した車を探す
  (for _array_element (`/Game/Play/Common/GroundObject/Car/BP_CarCreateManager.mCarType` _mbp_carcreatemanager)
    (bind _returnvalue (`GameplayStatics.GetActorOfClass` _array_element))
    (`/Engine/EditorBlueprintResources/StandardMacros.IsValid` _returnvalue
      (:`Is Valid`
        (set `self.mTargetCar` (cast `/Game/Play/Common/GroundObject/Car/BP_CarBase` _returnvalue :!pure true))
        (`self.fCreateInitBuilding`)))))

(fn `fGetTitleManager`
  (returns (`AsBP Title Manager` :type "/Game/Title/GameMode/BP_TitleManager Object Reference"))
  (bind _asbp_title_manager (cast `/Game/Title/GameMode/BP_TitleManager` (`self.mBP_BuildingManager`)))
  (return _asbp_title_manager))

(fn `UserConstructionScript`
  (`parent.UserConstructionScript`))