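; Title-screen ranking showcase that displays the local ranking, then the online ranking if its status check passes, then restores the title widget.
; A looping timer event drives an MState state machine while MActiveFlag is set.
; BP_Timer times each display, and GM_TitleCity's shared fade widget covers the transitions.
; MTitleBackFlag cuts either display short to fade back to the title.
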(event `Init`
  (`UserWidget.AddToViewport` (`self.WBP_LocalRanking`) 0) ; ローカルランキングの表示
  (`/Game/Play/Common/Fade/WBP_Fade.FadeInitialize` (`self.GetFade`) "NewEnumerator1" (`self.GetFadeTime`)))

(event `InitFadeOut`
  (if (`/Game/Play/Common/Fade/WBP_Fade.mEnd` (`self.GetFade`))
    (set `self.mState` "NewEnumerator1")))

(event `self.ReceiveBeginPlay`
  (bind _returnvalue (`|SpawnActorFromClass` "/Game/Play/Common/GroundObject/BP_Timer.BP_Timer_C" (`KismetMathLibrary.MakeTransform` (0.0 0.0 0.0)) "Undefined" "OverrideRootScale" null null))
  (bind _output_get (set `self.mBP_CountTimer` _returnvalue))
  (`/Game/Play/Common/GroundObject/BP_Timer.fSetMaxTime` _output_get 3.0)
  ;[1 1 1] ウィジェットの作成
  (bind _returnvalue_2 (`|CreateWidget` "/Game/DataRanking/WBP_OnLineRanking.WBP_OnLineRanking_C"))
  (bind _output_get_2 (set `self.WBP_OnlineRanking` _returnvalue_2))
  (`UserWidget.AddToViewport` _output_get_2 0)
  (`Widget.RemoveFromParent` _output_get_2)
  (bind _returnvalue_3 (`|CreateWidget` "/Game/DataRanking/WBP_LocalRanking.WBP_LocalRanking_C"))
  (set `self.WBP_LocalRanking` _returnvalue_3)
  (`KismetSystemLibrary.K2_SetTimerDelegate` (delegate `Update`) (`self.GetDeltaTime`) true))

(event `DrawLocalRanking`
  (bind _newparam (`/Game/Play/Common/GroundObject/BP_Timer.fCountUp` (`self.mBP_CountTimer`) (`self.GetDeltaTime`))) ; 時間が終わったら
  (if _newparam
    (`/Game/Play/Common/Fade/WBP_Fade.FadeInitialize` (`self.GetFade`) "NewEnumerator0" (`self.GetFadeTime`))
    (set `self.mState` "NewEnumerator2")
    (`/Game/Play/Common/GroundObject/BP_Timer.fReset` (`self.mBP_CountTimer`))))

(event `Update`
  (if (`self.mActiveFlag`)
    (switch `/Game/DataRanking/EN_DataRankingState` (`self.mState`)
      (:`NewEnumerator1`
        (`self.DrawLocalRanking`)
        (if (and (`self.mTitleBackFlag`) (`|EnumInequality` (`self.mState`) "NewEnumerator5") (`|EnumInequality` (`self.mState`) "NewEnumerator6") (`|EnumInequality` (`self.mState`) "NewEnumerator8")) :!label _label
          (set `self.mTitleBackFlag` false)
          (set `self.mState` "NewEnumerator5") ; Clickされていたら
          (`/Game/Play/Common/Fade/WBP_Fade.FadeInitialize` (`self.GetFade`) "NewEnumerator0" (`self.GetFadeTime`))))
      (:`NewEnumerator2`
        (`self.LocalRankingFadeIn`))
      (:`NewEnumerator3`
        (`self.LocalRankingFadeOut`))
      (:`NewEnumerator4`
        (`self.DrawOnlineRanking`)
        (goto _label))
      (:`NewEnumerator5`
        (`self.OnlineRankingFadeIn`))
      (:`NewEnumerator6`
        (`self.OnlineRankingFadeOut`))
      (:`NewEnumerator8`
        (`self.End`)))
    (elif (`|EnumInequality` (`self.mState`) "NewEnumerator1")
      (set `self.mState` "NewEnumerator1"))))

(event `LocalRankingFadeIn`
  (if (`/Game/Play/Common/Fade/WBP_Fade.mEnd` (`self.GetFade`))
    (`Widget.RemoveFromParent` (`self.WBP_LocalRanking`)) ; ローカルランキングの非表示
    (`/Game/Play/Common/Fade/WBP_Fade.FadeInitialize` (`self.GetFade`) "NewEnumerator1" (`self.GetFadeTime`))
    (if (`self.mTitleBackFlag`)
      (set `self.mTitleBackFlag` false)
      (set `self.mState` "NewEnumerator6") ; Clickされていたら
      (else
        (bind _newparam (`self.fChackOnline`))
        (if _newparam
          (`UserWidget.AddToViewport` (`self.WBP_OnlineRanking`) 0) ; オンラインランキングの表示
          (set `self.mState` "NewEnumerator3"))))))

(event `LocalRankingFadeOut`
  (if (`/Game/Play/Common/Fade/WBP_Fade.mEnd` (`self.GetFade`))
    (set `self.mState` "NewEnumerator4")))

(event `DrawOnlineRanking`
  (bind _newparam (`/Game/Play/Common/GroundObject/BP_Timer.fCountUp` (`self.mBP_CountTimer`) (`self.GetDeltaTime`))) ; 時間が終わったら
  (if _newparam
    (`/Game/Play/Common/Fade/WBP_Fade.FadeInitialize` (`self.GetFade`) "NewEnumerator0" (`self.GetFadeTime`))
    (set `self.mState` "NewEnumerator5")
    (`/Game/Play/Common/GroundObject/BP_Timer.fReset` (`self.mBP_CountTimer`))))

(event `OnlineRankingFadeIn`
  (if (`/Game/Play/Common/Fade/WBP_Fade.mEnd` (`self.GetFade`))
    (`Widget.RemoveFromParent` (`self.WBP_OnlineRanking`)) ; オンラインランキングの非表示
    (`/Game/Play/Common/Fade/WBP_Fade.FadeInitialize` (`self.GetFade`) "NewEnumerator1" (`self.GetFadeTime`))
    (set `self.mState` "NewEnumerator6")
    (`Widget.RemoveFromParent` (`self.WBP_LocalRanking`))
    (`Widget.SetVisibility` (`/Game/Title/GameMode/GM_TitleCity.mWBP_Title` (cast `/Game/Title/GameMode/GM_TitleCity` (`GameplayStatics.GetGameMode`) :!pure true)) "Visible")))

(event `OnlineRankingFadeOut`
  (if (`/Game/Play/Common/Fade/WBP_Fade.mEnd` (`self.GetFade`))
    (set `self.mState` "NewEnumerator8")
    (set `self.mTitleBackFlag` false)))

(event `End`
  (set `self.mActiveFlag` false))

(fn `fChackOnline`
  (returns (NewParam :type Boolean))
  (return (`|EnumInequality` (`/Game/DataRanking/WBP_OnLineRanking.mEN_SuccessState` (`self.WBP_OnlineRanking`)) "NewEnumerator1")))

(fn `UserConstructionScript`)