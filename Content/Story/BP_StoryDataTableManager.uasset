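; BP_StoryDataTableManager caches story image data and serves it by story state.
; On BeginPlay it loops over an enum's entry count, looks up DT_StoryImage rows named by index, and appends each found row to an array.
; FMap converts a given story state to an integer and returns the array element at that index.
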(event `self.ReceiveBeginPlay`
  (`self.fSetTableData`) ; ストーリーのデータテーブルの情報をセット
)

(fn `fMap`
  (params (story :type "/Game/Story/EN_Story Enum" :default "NewEnumerator0"))
  (returns (storyDatatable :type "/Game/Story/ST_StoryImageArray Structure"))
  (locals (NewLocalVar_0 :type "/Game/Play/Building/Data/ST_BuildingDataTable Structure") (NewLocalVar_1 :type "Array of /Game/Story/ST_StoryImageArray Structure"))
  ;[1 1 1] 取得したストーリー状態から対応するデータを返す
  (return (`|GetArrayItem` (`self.mST_StoryDataTable`) (`KismetMathLibrary.Conv_ByteToInt` story))))

(fn `fSetTableData`
  ;[1 1 1] ストーリーのデータテーブルの情報をセット
  (for _index (range (+ (enumcount `/Game/Story/EN_Story`) 1))
    (bind _returnvalue (`|GetDataTableRow` "/Game/Story/DT_StoryImage.DT_StoryImage" (`KismetStringLibrary.Conv_StringToName` (`KismetStringLibrary.Conv_IntToString` _index)))
      (:`then`
        (`KismetArrayLibrary.Array_Add` (`self.mST_StoryDataTable`) _returnvalue)))))

(fn `UserConstructionScript`)