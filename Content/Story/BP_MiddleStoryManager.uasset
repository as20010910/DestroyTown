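; BP_MiddleStoryManager is a manager Blueprint that shows the middle story segment in the DestructionCity game.
; MiddleStoryInitialize creates a WBP_Story widget with a story type, adds it to the viewport, then starts a looping timer at the game mode's DELTATIME.
; The timer's custom Tick checks the widget's IsStoryEnd but takes no action; the node setting MGameState on GM_DestructionCity is unconnected.
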(event `MiddleStoryInitialize`
  ;[1 1 1] 初期化処理
  (bind _returnvalue (`|CreateWidget` "/Game/Story/WBP_Story.WBP_Story_C" null "NewEnumerator1"))
  (bind _output_get (set `self.mWBP_Story` _returnvalue))
  (`UserWidget.AddToViewport` _output_get 1)
  (`KismetSystemLibrary.K2_SetTimerDelegate` (delegate `Tick`) (`/Game/Play/Common/GameMode/GM_DestructionCity.DELTA_TIME` (cast `/Game/Play/Common/GameMode/GM_DestructionCity` (`GameplayStatics.GetGameMode`) :!pure true)) true))

(event `Tick`
  ;[1 1 1] 更新処理
  (if (`/Game/Story/WBP_Story.IsStoryEnd` (`self.mWBP_Story`))
    _))

(fn `UserConstructionScript`)