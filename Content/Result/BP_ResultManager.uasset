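; Result-scene manager that shows the post-game newspaper and runs the epilogue or the return to title.
; Initialization spawns the sound and destruction-class data table managers, creates fade and newspaper widgets, and starts result BGM.
; The epilogue fades into a story widget with recollection BGM, using looping timers to poll fade and story completion before loading title.
; Separate return events stop BGM and reset the GameInstance, with a fade and delay when skipping the story.
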(event `ResultInitialize`
  ;[1 1 1] 初期化処理
  (`self.CreateResultSoundManager`) ; リザルトサウンドマネージャー生成処理
  (`self.CreateResultDestructionClassDataTable`) ; 被害規模クラスデータテーブル作成
  (`self.CreateFade`) ; フェードを生成
  (`self.CreateNewsPaper`) ; 新聞を生成
  (`/Game/Result/BP_ResultSoundManager.PlayBGM` (`self.mBP_ResultSoundManager`) "/Game/Result/Sounds/BGMResult.BGMResult") ; BGMを再生
)

(event `StartEpilogue`
  ;[1 1 1] エピローグ開始処理
  (`/Game/Play/Common/Fade/WBP_Fade.FadeInitialize` (`self.mBP_Fade`) "NewEnumerator0" 0.01)
  (bind _returnvalue (`KismetSystemLibrary.K2_SetTimerDelegate` (delegate `FadeInEnd`) (`self.GetDELTA_TIME`) true)))

(event `FadeInEnd`
  ;[1 1 1] フェードイン終了処理
  (if (`/Game/Play/Common/Fade/WBP_Fade.mEnd` (`self.mBP_Fade`))
    (`KismetSystemLibrary.K2_ClearAndInvalidateTimerHandle` (stale `StartEpilogue` _returnvalue))
    (bind _returnvalue (`|CreateWidget` "/Game/Play/Story/WBP_Story.WBP_Story_C" null "NewEnumerator2"))
    (bind _output_get (set `self.mWBP_Story` _returnvalue))
    (`UserWidget.AddToViewport` _output_get 2)
    (`KismetSystemLibrary.K2_SetTimerDelegate` (delegate `BeginEpilogue`) (`self.EPILOGUE_BEGIN_TIME`))))

(event `BeginEpilogue`
  ;[1 1 1] エピローグ開始処理
  (`/Game/Result/BP_ResultSoundManager.PlayBGM` (`self.mBP_ResultSoundManager`) "/Game/Result/Sounds/BGM_DestructionRecollection.BGM_DestructionRecollection") ; BGMを再生
  (`/Game/Play/Common/Fade/WBP_Fade.FadeInitialize` (`self.mBP_Fade`) "NewEnumerator1" 0.01)
  (bind _returnvalue (`KismetSystemLibrary.K2_SetTimerDelegate` (delegate `EpilogueTick`) (`self.GetDELTA_TIME`) true)))

(event `ReturnTitleScene`
  ;[1 1 1] タイトルへ戻る処理
  (`/Game/Result/BP_ResultSoundManager.StopBGM` (`self.mBP_ResultSoundManager`)) ; BGMを止める
  (`/Game/Play/Common/GameInstance/GMI_DestructionCIty.Reset` (cast `/Game/Play/Common/GameInstance/GMI_DestructionCIty` (`GameplayStatics.GetGameInstance`) :!pure true)) ; 値をリセット
  (`GameplayStatics.OpenLevelBySoftObjectPtr` "/Game/Title/LBP_Title-α-Stage.LBP_Title-α-Stage"))

(event `EpilogueTick`
  ;[1 1 1] エピローグの更新処理
  (if (`/Game/Play/Story/WBP_Story.IsStoryEnd` (`self.mWBP_Story`))
    (`KismetSystemLibrary.K2_ClearAndInvalidateTimerHandle` (stale `BeginEpilogue` _returnvalue))
    (`/Game/Play/Common/Fade/WBP_Fade.BlackOut` (`self.mBP_Fade`))
    (`KismetSystemLibrary.K2_SetTimerDelegate` (delegate `NextScene`) (`self.NEXT_SCENE_TIME`))))

(event `NextScene`
  ;[1 1 1] 次のシーンへ行く処理
  (`/Game/Result/BP_ResultSoundManager.StopBGM` (`self.mBP_ResultSoundManager`)) ; BGMを止める
  (`GameplayStatics.OpenLevel` "LBP_Title-α-Stage"))

(event `NotStoryReturnTitleScene`
  ;[1 1 1] ストーリーを見ずにタイトルへ戻る処理
  (`/Game/Result/BP_ResultSoundManager.StopBGM` (`self.mBP_ResultSoundManager`)) ; BGMを止める
  (`/Game/Play/Common/GameInstance/GMI_DestructionCIty.Reset` (cast `/Game/Play/Common/GameInstance/GMI_DestructionCIty` (`GameplayStatics.GetGameInstance`) :!pure true)) ; 値をリセット
  (`/Game/Play/Common/Fade/WBP_Fade.FadeInitialize` (`self.mBP_Fade`) "NewEnumerator0" 0.015)
  (`KismetSystemLibrary.Delay` 2.0)
  (`GameplayStatics.OpenLevelBySoftObjectPtr` "/Game/Title/LBP_Title-α-Stage.LBP_Title-α-Stage"))

(fn `CreateFade`
  ;[1 1 1] フェードを生成
  (bind _returnvalue (`|CreateWidget` "/Game/Play/Common/Fade/WBP_Fade.WBP_Fade_C"))
  (bind _output_get (set `self.mBP_Fade` _returnvalue))
  (`UserWidget.AddToViewport` _output_get 100)
  (`/Game/Play/Common/Fade/WBP_Fade.BlackOut` _output_get)
  (`/Game/Play/Common/Fade/WBP_Fade.FadeInitialize` _output_get "NewEnumerator1" 0.01))

(fn `CreateNewsPaper`
  ;[1 1 1] 新聞を生成
  (bind _returnvalue (`|CreateWidget` "/Game/Result/Widget/WBP_Newspaper.WBP_Newspaper_C"))
  (`UserWidget.AddToViewport` _returnvalue 0)
  (set `self.mWBP_Newspaper` _returnvalue))

(fn `CreateResultDestructionClassDataTable`
  ;[1 1 1] 被害規模クラスデータテーブル作成
  (bind _returnvalue (`|SpawnActorFromClass` "/Game/Result/Widget/BP_ResultDestructionClassDataTableManager.BP_ResultDestructionClassDataTableManager_C" (`KismetMathLibrary.MakeTransform` (0.0 0.0 0.0)) "Undefined" "OverrideRootScale" null null)) ; 被害規模クラスデータテーブル作成
  (set `self.mBP_ResultDestructionClassDataTable` _returnvalue))

(fn `CreateResultSoundManager`
  ;[1 1 1] リザルトサウンドマネージャー生成処理
  (bind _returnvalue (`|SpawnActorFromClass` "/Game/Result/BP_ResultSoundManager.BP_ResultSoundManager_C" (`KismetMathLibrary.MakeTransform` (0.0 0.0 0.0)) "Undefined" "OverrideRootScale" null null))
  (set `self.mBP_ResultSoundManager` _returnvalue))

(fn `UserConstructionScript`)