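; Destructible wooden house actor for the introductory video that the Mayor character can smash.
; When a BP_Mayor overlaps the house with its attack collision set to query and physics, the destructible takes damage and an impulse based on the Scene component's location.
; Fracturing triggers a short global slow-motion by lowering time dilation, then restoring it after a delay.
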(event `self.APEXM_WoodenHouse.OnComponentFracture`
  (params (HitPoint :type "Vector Structure (by ref)") (HitDirection :type "Vector Structure (by ref)"))
  (`GameplayStatics.SetGlobalTimeDilation` 0.2)
  (`KismetSystemLibrary.Delay` 0.2)
  (`GameplayStatics.SetGlobalTimeDilation` 1.0))

(event `self.APEXM_WoodenHouse.OnComponentBeginOverlap`
  (params (OverlappedComponent :type "PrimitiveComponent Object Reference") (OtherActor :type "Actor Object Reference") (OtherComp :type "PrimitiveComponent Object Reference") (OtherBodyIndex :type Integer) (bFromSweep :type Boolean) (SweepResult :type "HitResult Structure (by ref)"))
  (bind _returnvalue (`SceneComponent.K2_GetComponentLocation` (`self.Scene`)))
  (bind _asbp_mayor (cast `/Game/Play/Destruction/Mayor/BP_Mayor` OtherActor))
  (if (`|EnumEquality` (`PrimitiveComponent.GetCollisionEnabled` (`/Game/Play/Destruction/Mayor/BP_Mayor.AttackCollision` _asbp_mayor)) "QueryAndPhysics")
    (`DestructibleComponent.ApplyDamage` (`self.APEXM_WoodenHouse`) 100.0 _returnvalue _returnvalue 10000.0)))

(fn `UserConstructionScript`)