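; Game mode for the stage select screen, which sets up its UI and launches the chosen stage.
; On BeginPlay it creates the stage select widget, layers a fade widget above it and shows the mouse cursor.
; Its StartStage event starts the fade, waits on a fixed delay, then opens the level by the stage name stored in the select widget.
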(event `self.ReceiveBeginPlay`
  ;[1 1 1] 初期化処理
  (bind _returnvalue (`|CreateWidget` "/Game/StageSelect/Widgets/WBP_StageSelect.WBP_StageSelect_C"))
  (bind _output_get (set `self.mWBP_StageSelect` _returnvalue))
  (`UserWidget.AddToViewport` _output_get 0)
  (bind _returnvalue_2 (`|CreateWidget` "/Game/Play/Common/Fade/WBP_Fade.WBP_Fade_C"))
  (bind _output_get_2 (set `self.mWBP_Fade` _returnvalue_2))
  (`UserWidget.AddToViewport` _output_get_2 1)
  (set `PlayerController.bShowMouseCursor` true (`GameplayStatics.GetPlayerController` 0)))

(event `StartStage`
  ;[1 1 1] ステージを選択しスタートした際の処理
  (`/Game/Play/Common/Fade/WBP_Fade.FadeInitialize` (`self.mWBP_Fade`) "NewEnumerator0" 0.01)
  (`KismetSystemLibrary.Delay` 2.0)
  (`GameplayStatics.OpenLevel` (`/Game/StageSelect/Widgets/WBP_StageSelect.mSelectStageName` (`self.mWBP_StageSelect`))))

(fn `UserConstructionScript`)