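; BP_DestroyRoad is a destructible bridge-stage road piece with street lamps and poles, built from APEX destructible components.
; When BP_Mayor begins overlapping the road mesh, it applies heavy damage at Road3DestructionPos and passes the road to DestroyRoadObject.
; FAllDestroy shatters the road, lamps and poles together from the actor location, then calls DestroyRoadObject on each.
; Both paths pass a world position as the impulse direction.
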(event `self.APEXM_Road.OnComponentBeginOverlap`
  (params (OverlappedComponent :type "PrimitiveComponent Object Reference") (OtherActor :type "Actor Object Reference") (OtherComp :type "PrimitiveComponent Object Reference") (OtherBodyIndex :type Integer) (bFromSweep :type Boolean) (SweepResult :type "HitResult Structure (by ref)"))
  (bind _apexm_road (`self.APEXM_Road`))
  (bind _returnvalue (`SceneComponent.K2_GetComponentLocation` (`self.Road3DestructionPos`)))
  (cast `/Game/Play/Destruction/Mayor/BP_Mayor` OtherActor)
  (`DestructibleComponent.ApplyDamage` _apexm_road 1000.0 _returnvalue _returnvalue 0.0)
  (`self.DestroyRoadObject` _apexm_road))

(fn `fAllDestroy`
  (bind _returnvalue (`self.K2_GetActorLocation`))
  (`DestructibleComponent.ApplyDamage` (`self.APEXM_StreetLamp`) 1000.0 _returnvalue _returnvalue 0.0)
  (`DestructibleComponent.ApplyDamage` (`self.APEXM_Road`) 1000.0 _returnvalue _returnvalue 0.0)
  (`DestructibleComponent.ApplyDamage` (`self.APEXM_StreetLamp1`) 1000.0 _returnvalue _returnvalue 0.0)
  (`DestructibleComponent.ApplyDamage` (`self.APEXM_Pole`) 1000.0 _returnvalue _returnvalue 0.0)
  (`DestructibleComponent.ApplyDamage` (`self.APEXM_Pole2`) 1000.0 _returnvalue _returnvalue 0.0)
  (`DestructibleComponent.ApplyDamage` (`self.APEXM_Pole3`) 1000.0 _returnvalue _returnvalue 0.0)
  (`self.DestroyRoadObject` (`self.APEXM_StreetLamp`))
  (`self.DestroyRoadObject` (`self.APEXM_StreetLamp1`))
  (`self.DestroyRoadObject` (`self.APEXM_Pole`))
  (`self.DestroyRoadObject` (`self.APEXM_Pole2`))
  (`self.DestroyRoadObject` (`self.APEXM_Pole3`))
  (`self.DestroyRoadObject` (`self.APEXM_Road`)))

(fn `UserConstructionScript`
  (`parent.UserConstructionScript`))