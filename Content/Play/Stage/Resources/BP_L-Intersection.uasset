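; BP_L-Intersection is an L-shaped corner stage piece that sets up direction changes for both ways through the bend.
; On BeginPlay, a switch on the instance's left-turn exit direction derives the matching before and after compass directions for the left turn and the reverse right turn.
; It writes each pair into one of two BP_ChangeAngle child actors, reached through cast helper functions.
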(event `self.ReceiveBeginPlay`
  (bind _asbp_change_angle (`self.fGetChangeAngle`))
  (bind _asbp_change_angle_2 (`self.fGetChangeAngle1`))
  (bind _asbp_change_angle_3 (`self.fGetChangeAngle`))
  (bind _asbp_change_angle_4 (`self.fGetChangeAngle1`))
  (bind _asbp_change_angle_5 (`self.fGetChangeAngle`))
  (bind _asbp_change_angle_6 (`self.fGetChangeAngle1`))
  (bind _asbp_change_angle_7 (`self.fGetChangeAngle`))
  (bind _asbp_change_angle_8 (`self.fGetChangeAngle1`))
  (switch `/Game/Play/Common/GroundObject/Intersection/TraficLight/TraficLightDirection` (`self.INST_LeftAfterDirection`)
    (:`NewEnumerator0`
      (set `/Game/Play/Common/GroundObject/Car/BP_ChangeAngle.INST_AfterDirection` (`self.INST_LeftAfterDirection`) _asbp_change_angle_3)
      (set `/Game/Play/Common/GroundObject/Car/BP_ChangeAngle.INST_BeforeDirection` "NewEnumerator2" _asbp_change_angle_3)
      (set `/Game/Play/Common/GroundObject/Car/BP_ChangeAngle.INST_AfterDirection` "NewEnumerator3" _asbp_change_angle_4)
      (set `/Game/Play/Common/GroundObject/Car/BP_ChangeAngle.INST_BeforeDirection` "NewEnumerator1" _asbp_change_angle_4))
    (:`NewEnumerator1`
      (set `/Game/Play/Common/GroundObject/Car/BP_ChangeAngle.INST_AfterDirection` (`self.INST_LeftAfterDirection`) _asbp_change_angle_5)
      (set `/Game/Play/Common/GroundObject/Car/BP_ChangeAngle.INST_BeforeDirection` "NewEnumerator3" _asbp_change_angle_5)
      (set `/Game/Play/Common/GroundObject/Car/BP_ChangeAngle.INST_AfterDirection` "NewEnumerator2" _asbp_change_angle_6)
      (set `/Game/Play/Common/GroundObject/Car/BP_ChangeAngle.INST_BeforeDirection` "NewEnumerator0" _asbp_change_angle_6))
    (:`NewEnumerator2`
      (set `/Game/Play/Common/GroundObject/Car/BP_ChangeAngle.INST_AfterDirection` (`self.INST_LeftAfterDirection`) _asbp_change_angle_7)
      (set `/Game/Play/Common/GroundObject/Car/BP_ChangeAngle.INST_BeforeDirection` "NewEnumerator1" _asbp_change_angle_7)
      (set `/Game/Play/Common/GroundObject/Car/BP_ChangeAngle.INST_AfterDirection` "NewEnumerator0" _asbp_change_angle_8)
      (set `/Game/Play/Common/GroundObject/Car/BP_ChangeAngle.INST_BeforeDirection` "NewEnumerator3" _asbp_change_angle_8))
    (:`NewEnumerator3`
      (set `/Game/Play/Common/GroundObject/Car/BP_ChangeAngle.INST_AfterDirection` (`self.INST_LeftAfterDirection`) _asbp_change_angle)
      (set `/Game/Play/Common/GroundObject/Car/BP_ChangeAngle.INST_BeforeDirection` "NewEnumerator0" _asbp_change_angle)
      (set `/Game/Play/Common/GroundObject/Car/BP_ChangeAngle.INST_AfterDirection` "NewEnumerator1" _asbp_change_angle_2)
      (set `/Game/Play/Common/GroundObject/Car/BP_ChangeAngle.INST_BeforeDirection` "NewEnumerator2" _asbp_change_angle_2))))

(fn `fGetChangeAngle`
  (returns (`AsBP Change Angle` :type "/Game/Play/Common/GroundObject/Car/BP_ChangeAngle Object Reference"))
  (bind _asbp_change_angle (cast `/Game/Play/Common/GroundObject/Car/BP_ChangeAngle` (`ChildActorComponent.ChildActor` (`self.BP_ChangeAngle`))))
  (return _asbp_change_angle))

(fn `fGetChangeAngle1`
  (returns (`AsBP Change Angle` :type "/Game/Play/Common/GroundObject/Car/BP_ChangeAngle Object Reference"))
  (bind _asbp_change_angle (cast `/Game/Play/Common/GroundObject/Car/BP_ChangeAngle` (`ChildActorComponent.ChildActor` (`self.BP_ChangeAngle1`))))
  (return _asbp_change_angle))

(fn `UserConstructionScript`)