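; BP_SaveAddressManager converts the stage's city state to and from save data, covering money, population and each address section's building.
; FExtractSectionBuilding walks addresses and their sections, collecting building types per address into MSTSaveBuilding.
; FCreate restores totals to the GameInstance and reapplies saved building types and meshes by index, skipping one enum value.
; FSaveInfo copies only money and population from the GameMode's building manager into the save data.
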(fn `F Extract Section Building`
  (locals (insArray :type "Array of /Game/Play/Building/Data/EN_Building Enum"))
  (for _array_element (`self.mAddress`)
    (for _array_element_2 (`/Game/Play/Building/Address/BP_Address.mSections` _array_element)
      (`KismetArrayLibrary.Array_Add` (`local.insArray`) (`/Game/Play/Building/BP_Building/BP_BuildingBase.mBuilding` (`/Game/Play/Building/Address/Section/BP_Section.fGetBuildingBase` _array_element_2))))
    (`KismetArrayLibrary.Array_Add` (`self.mST_SaveBuilding`) (make `/Game/Play/Stage/Only/Save/ST_SaveSectionBuilding` (`local.insArray`)))
    (`KismetArrayLibrary.Array_Clear` (`local.insArray`))))

(fn `fCreate`
  (bind _msavedata (`self.mSaveData`))
  (bind _asgmi_destruction_city (cast `/Game/Play/Common/GameInstance/GMI_DestructionCIty` (`GameplayStatics.GetGameInstance`) :!pure true))
  (set `/Game/Play/Common/GameInstance/GMI_DestructionCIty.mRemainingTotalMoney` (`/Game/Play/Stage/Only/Save/BP_LoadGame.mRemainingTotalMoney` _msavedata) _asgmi_destruction_city)
  (set `/Game/Play/Common/GameInstance/GMI_DestructionCIty.mTotalPeopleNum` (`/Game/Play/Stage/Only/Save/BP_LoadGame.mTotalPeopleNum` _msavedata) _asgmi_destruction_city)
  (for (_array_element _array_index) (`self.mAddress`)
    (for (_array_element_2 _array_index_2) (`/Game/Play/Building/Address/BP_Address.mSections` _array_element)
      (bind _output_sectionbuilding (break `/Game/Play/Stage/Only/Save/ST_SaveSectionBuilding` (`|GetArrayItem` (`/Game/Play/Stage/Only/Save/BP_LoadGame.mSectionInfo` (`self.mSaveData`)) _array_index)))
      (bind _output (`|GetArrayItem` _output_sectionbuilding _array_index_2))
      (if (`|EnumInequality` _output "NewEnumerator13")
        (bind _asbp_building_base (`/Game/Play/Building/Address/Section/BP_Section.fGetBuildingBase` _array_element_2))
        (set `/Game/Play/Building/BP_Building/BP_BuildingBase.mBuilding` _output _asbp_building_base)
        (`/Game/Play/Building/BP_Building/BP_BuildingBase.fSetMesh` _asbp_building_base _output)))))

(fn `fSaveInfo`
  (params (SaveData :type "/Game/Play/Stage/Only/Save/BP_LoadGame Object Reference"))
  (bind _mbp_buildingmanager (`/Game/Play/Common/GameMode/GM_DestructionCity.mBP_BuildingManager` (cast `/Game/Play/Common/GameMode/GM_DestructionCity` (`GameplayStatics.GetGameMode`) :!pure true)))
  (set `/Game/Play/Stage/Only/Save/BP_LoadGame.mRemainingTotalMoney` (`/Game/Play/Building/BP_BuildingManager.mTexNum` _mbp_buildingmanager) SaveData)
  (set `/Game/Play/Stage/Only/Save/BP_LoadGame.mTotalPeopleNum` (`/Game/Play/Building/BP_BuildingManager.mPeopleCountNum` _mbp_buildingmanager) SaveData))

(fn `UserConstructionScript`)