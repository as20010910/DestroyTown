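; Road stage piece that gives overlapping cars lane data and has street lamps and poles that BP_Mayor smashes.
; BeginPlay classifies the road as Height or Width from its yaw.
; Box1/Box2 overlaps store box and direction on BP_CarBase and sign its SHIFTVEL toward the box centre.
; Prop overlaps damage APEX destructibles, then call a shared delayed DestroyRoadObject, whose DoOnce removes only one component per road.
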(event `self.ReceiveBeginPlay`
  (bind (_returnvalue_roll _returnvalue_pitch _returnvalue_yaw) (`KismetMathLibrary.BreakRotator` (`self.K2_GetActorRotation`)))
  ;[1 1 1] 大雑把な道路の方向を指定
  (if (`KismetMathLibrary.NearlyEqual_FloatFloat` _returnvalue_yaw 90.0 20.0)
    (set `self.mPosition` "NewEnumerator0")
    (else
      (set `self.mPosition` "NewEnumerator1")))
  (for _array_element (`self.K2_GetComponentsByClass` "/Script/ApexDestruction.DestructibleComponent")
    (`SceneComponent.SetWorldScale3D` (cast `DestructibleComponent` _array_element :!pure true) (1.0 1.0 1.0))))

(event `self.Box1.OnComponentBeginOverlap`
  (params (OverlappedComponent :type "PrimitiveComponent Object Reference") (OtherActor :type "Actor Object Reference") (OtherComp :type "PrimitiveComponent Object Reference") (OtherBodyIndex :type Integer) (bFromSweep :type Boolean) (SweepResult :type "HitResult Structure (by ref)"))
  (bind (_asbp_car_base _bsuccess) (cast `/Game/Play/Common/GroundObject/Car/BP_CarBase` OtherActor :!pure true))
  (bind _savecar (`self.saveCar`))
  (bind _savecar_2 (`self.saveCar`))
  (bind _savecar_3 (`self.saveCar`))
  (bind _returnvalue_x (`KismetMathLibrary.BreakVector` (`self.K2_GetActorLocation` (`self.saveCar`))))
  (bind (_returnvalue_x_2 _returnvalue_y) (`KismetMathLibrary.BreakVector` (`self.K2_GetActorLocation` (`self.saveCar`))))
  (bind _returnvalue_x_3 (`KismetMathLibrary.BreakVector` (`SceneComponent.K2_GetComponentLocation` (`self.box`))))
  (bind (_returnvalue_x_4 _returnvalue_y_2) (`KismetMathLibrary.BreakVector` (`SceneComponent.K2_GetComponentLocation` (`self.box`))))
  (bind _returnvalue (`KismetMathLibrary.Abs` (`/Game/Play/Common/GroundObject/Car/BP_CarBase.SHIFT_VEL` _savecar_2)))
  (bind _returnvalue_2 (`KismetMathLibrary.Abs` (`/Game/Play/Common/GroundObject/Car/BP_CarBase.SHIFT_VEL` _savecar)))
  ;[1 1 1] 当たったものが車か識別
  (if _bsuccess
    (set `self.box` (`self.Box1`))
    (set `self.saveCar` _asbp_car_base)
    (set `/Game/Play/Common/GroundObject/Car/BP_CarBase.mRideOnBox` (`self.box`) _savecar_3 :!label _label) ; 車に自身を保存しておく
    (set `/Game/Play/Common/GroundObject/Car/BP_CarBase.mRideOnRode` (`self.mPosition`) _savecar_3)
    (switch `/Game/Play/Stage/EN_Angle` (`self.mPosition`)
      (:`NewEnumerator0`
        (if (> _returnvalue_y _returnvalue_y_2)
          (set `/Game/Play/Common/GroundObject/Car/BP_CarBase.SHIFT_VEL` (* -1 _returnvalue_2) _savecar)
          (else
            (set `/Game/Play/Common/GroundObject/Car/BP_CarBase.SHIFT_VEL` _returnvalue_2 _savecar))))
      (:`NewEnumerator1`
        (if (> _returnvalue_x_3 _returnvalue_x)
          (set `/Game/Play/Common/GroundObject/Car/BP_CarBase.SHIFT_VEL` _returnvalue _savecar_2)
          (else
            (set `/Game/Play/Common/GroundObject/Car/BP_CarBase.SHIFT_VEL` (* -1 _returnvalue) _savecar_2)))))))

(event `self.Box2.OnComponentBeginOverlap`
  (params (OverlappedComponent :type "PrimitiveComponent Object Reference") (OtherActor :type "Actor Object Reference") (OtherComp :type "PrimitiveComponent Object Reference") (OtherBodyIndex :type Integer) (bFromSweep :type Boolean) (SweepResult :type "HitResult Structure (by ref)"))
  (bind (_asbp_car_base _bsuccess) (cast `/Game/Play/Common/GroundObject/Car/BP_CarBase` OtherActor :!pure true))
  ;[1 1 1] 当たったものが車か識別
  (if _bsuccess
    (set `self.box` (`self.Box2`))
    (set `self.saveCar` _asbp_car_base)
    (goto _label)))

(event `self.StreetLampCollision.OnComponentBeginOverlap`
  (params (OverlappedComponent :type "PrimitiveComponent Object Reference") (OtherActor :type "Actor Object Reference") (OtherComp :type "PrimitiveComponent Object Reference") (OtherBodyIndex :type Integer) (bFromSweep :type Boolean) (SweepResult :type "HitResult Structure (by ref)"))
  (bind _apexm_streetlamp (`self.APEXM_StreetLamp`))
  (bind _returnvalue (`SceneComponent.K2_GetComponentLocation` (`self.StreetLampDestructionPos`)))
  (cast `/Game/Play/Destruction/Mayor/BP_Mayor` OtherActor)
  (`DestructibleComponent.ApplyDamage` _apexm_streetlamp 1000.0 _returnvalue _returnvalue 0.0)
  (`self.DestroyRoadObject` _apexm_streetlamp))

(event `self.StreetLamp1Collision.OnComponentBeginOverlap`
  (params (OverlappedComponent :type "PrimitiveComponent Object Reference") (OtherActor :type "Actor Object Reference") (OtherComp :type "PrimitiveComponent Object Reference") (OtherBodyIndex :type Integer) (bFromSweep :type Boolean) (SweepResult :type "HitResult Structure (by ref)"))
  (bind _apexm_streetlamp1 (`self.APEXM_StreetLamp1`))
  (bind _returnvalue (`SceneComponent.K2_GetComponentLocation` (`self.StreetLamp1DestructionPos`)))
  (cast `/Game/Play/Destruction/Mayor/BP_Mayor` OtherActor)
  (`DestructibleComponent.ApplyDamage` _apexm_streetlamp1 1000.0 _returnvalue _returnvalue 0.0)
  (`self.DestroyRoadObject` _apexm_streetlamp1))

(event `self.PoleCollision.OnComponentBeginOverlap`
  (params (OverlappedComponent :type "PrimitiveComponent Object Reference") (OtherActor :type "Actor Object Reference") (OtherComp :type "PrimitiveComponent Object Reference") (OtherBodyIndex :type Integer) (bFromSweep :type Boolean) (SweepResult :type "HitResult Structure (by ref)"))
  (bind _apexm_pole (`self.APEXM_Pole`))
  (bind _returnvalue (`SceneComponent.K2_GetComponentLocation` (`self.PoleDestructionPos`)))
  (cast `/Game/Play/Destruction/Mayor/BP_Mayor` OtherActor)
  (`DestructibleComponent.ApplyDamage` _apexm_pole 1000.0 _returnvalue _returnvalue 0.0)
  (`self.DestroyRoadObject` _apexm_pole))

(event `self.Pole1Collision.OnComponentBeginOverlap`
  (params (OverlappedComponent :type "PrimitiveComponent Object Reference") (OtherActor :type "Actor Object Reference") (OtherComp :type "PrimitiveComponent Object Reference") (OtherBodyIndex :type Integer) (bFromSweep :type Boolean) (SweepResult :type "HitResult Structure (by ref)"))
  (bind _apexm_pole1 (`self.APEXM_Pole1`))
  (bind _returnvalue (`SceneComponent.K2_GetComponentLocation` (`self.Pole1DestructionPos`)))
  (cast `/Game/Play/Destruction/Mayor/BP_Mayor` OtherActor)
  (`DestructibleComponent.ApplyDamage` _apexm_pole1 1000.0 _returnvalue _returnvalue 0.0)
  (`self.DestroyRoadObject` _apexm_pole1))

(event `self.Pole2Collision.OnComponentBeginOverlap`
  (params (OverlappedComponent :type "PrimitiveComponent Object Reference") (OtherActor :type "Actor Object Reference") (OtherComp :type "PrimitiveComponent Object Reference") (OtherBodyIndex :type Integer) (bFromSweep :type Boolean) (SweepResult :type "HitResult Structure (by ref)"))
  (bind _apexm_pole2 (`self.APEXM_Pole2`))
  (bind _returnvalue (`SceneComponent.K2_GetComponentLocation` (`self.Pole2DestructionPos`)))
  (cast `/Game/Play/Destruction/Mayor/BP_Mayor` OtherActor)
  (`DestructibleComponent.ApplyDamage` _apexm_pole2 1000.0 _returnvalue _returnvalue 0.0)
  (`self.DestroyRoadObject` _apexm_pole2))

(event `self.Pole3Collision.OnComponentBeginOverlap`
  (params (OverlappedComponent :type "PrimitiveComponent Object Reference") (OtherActor :type "Actor Object Reference") (OtherComp :type "PrimitiveComponent Object Reference") (OtherBodyIndex :type Integer) (bFromSweep :type Boolean) (SweepResult :type "HitResult Structure (by ref)"))
  (bind _apexm_pole3 (`self.APEXM_Pole3`))
  (bind _returnvalue (`SceneComponent.K2_GetComponentLocation` (`self.Pole3DestructionPos`)))
  (cast `/Game/Play/Destruction/Mayor/BP_Mayor` OtherActor)
  (`DestructibleComponent.ApplyDamage` _apexm_pole3 1000.0 _returnvalue _returnvalue 0.0)
  (`self.DestroyRoadObject` _apexm_pole3))

(event `DestroyRoadObject`
  (params (DestructibleComponent :type "DestructibleComponent Object Reference"))
  (`KismetSystemLibrary.Delay` 1.0)
  (`/Engine/EditorBlueprintResources/StandardMacros.DoOnce` false
    (:`Completed`
      (`ActorComponent.K2_DestroyComponent` DestructibleComponent))))

(fn `UserConstructionScript`)