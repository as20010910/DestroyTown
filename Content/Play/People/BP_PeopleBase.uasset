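; Base pedestrian for the city destruction game that wanders and flees from the mayor.
; A looping timer with a randomized interval moves it left or right along its initial facing's right vector via AIMoveTo.
; Tick sends it back to its stored initial location while its capsule is outside a BP_PeopleManager area.
; When BP_Mayor enters its view range in a specific game state, it triggers AIC_People's escape, speeds up and despawns after a delay.
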(event `self.ReceiveTick`
  (params (DeltaSeconds :type "Float (single-precision)"))
  ;[1 1 1] 更新処理
  (if (`self.mRunFlag`)
    _
    (elif (not (`self.mInRange`))
      (set `self.mWalkEnd` true)
      (`AITask_MoveTo.AIMoveTo` (`AIBlueprintHelperLibrary.GetAIController` self) (`self.mInitializePeopleLocation`) null))))

(event `self.ReceiveBeginPlay`
  ;[1 1 1] 初期化
  (set `self.mPeopleRotation` (`self.K2_GetActorRotation`))
  (`KismetSystemLibrary.K2_SetTimerDelegate` (delegate `Walk`) (`KismetMathLibrary.RandomFloatInRange` (`self.MIN_WALK_INTERVAL`) (`self.MAX_WALK_INTERVAL`)) true))

(event `Walk`
  (bind _returnvalue (`self.K2_GetActorLocation`))
  (bind _returnvalue_2 (* (`KismetMathLibrary.GetRightVector` (`self.mPeopleRotation`)) (`KismetMathLibrary.RandomFloatInRange` 0.0 (`self.mWalkDistance`))))
  ;[1 1 1] 歩く処理
  (if (and (not (`self.mRunFlag`)) (`self.mWalkEnd`))
    (set `self.mWalkEnd` false)
    (if (`KismetMathLibrary.RandomBool`)
      (set `self.mTargetLocation` (+ _returnvalue _returnvalue_2))
      (else
        (set `self.mTargetLocation` (- _returnvalue _returnvalue_2))))
    (`AITask_MoveTo.AIMoveTo` (`AIBlueprintHelperLibrary.GetAIController` self) (`self.mTargetLocation`) null
      (:`OnMoveFinished`
        (set `self.mWalkEnd` true)))))

(event `self.TargetViewRunRange.OnComponentBeginOverlap`
  (params (OverlappedComponent :type "PrimitiveComponent Object Reference") (OtherActor :type "Actor Object Reference") (OtherComp :type "PrimitiveComponent Object Reference") (OtherBodyIndex :type Integer) (bFromSweep :type Boolean) (SweepResult :type "HitResult Structure (by ref)"))
  ;[1 1 1] 逃げる処理
  (cast `/Game/Play/Destruction/Mayor/BP_Mayor` OtherActor)
  (if (`|EnumEquality` (`/Game/Play/Common/GameMode/GM_DestructionCity.mGameState` (cast `/Game/Play/Common/GameMode/GM_DestructionCity` (`GameplayStatics.GetGameMode`) :!pure true)) "NewEnumerator1")
    (bind _asaic_people (cast `/Game/Play/People/AIC_People` (`AIBlueprintHelperLibrary.GetAIController` self)))
    (`/Game/Play/People/AIC_People.EventEscape` _asaic_people)
    (set `CharacterMovementComponent.MaxWalkSpeed` (`self.mRunSpeed`) (`self.CharacterMovement`))
    (set `self.mRunFlag` true)
    (`KismetSystemLibrary.Delay` 5.0)
    (`self.K2_DestroyActor`)))

(event `self.CapsuleComponent.OnComponentBeginOverlap`
  (params (OverlappedComponent :type "PrimitiveComponent Object Reference") (OtherActor :type "Actor Object Reference") (OtherComp :type "PrimitiveComponent Object Reference") (OtherBodyIndex :type Integer) (bFromSweep :type Boolean) (SweepResult :type "HitResult Structure (by ref)"))
  ;[1 1 1] 今現在人間が動ける範囲内かチェック
  (cast `/Game/Play/People/BP_PeopleManager` OtherActor)
  (set `self.mInRange` true))

(event `self.CapsuleComponent.OnComponentEndOverlap`
  (params (OverlappedComponent :type "PrimitiveComponent Object Reference") (OtherActor :type "Actor Object Reference") (OtherComp :type "PrimitiveComponent Object Reference") (OtherBodyIndex :type Integer))
  ;[1 1 1] 今現在人間が動ける範囲内かチェック
  (cast `/Game/Play/People/BP_PeopleManager` OtherActor)
  (set `self.mInRange` false))

(fn `fCheckPeopleWalkRange`)

(fn `UserConstructionScript`)