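; Manager actor that spawns AI pedestrians for an assigned road.
; On BeginPlay it scales its spawn range to the road, then starts a looping timer whose random interval is rolled once.
; Each tick spawns a random man or woman pawn with a shared behavior tree at the first spawn point, storing that origin on it.
; Spawning is capped by a per-manager running count and the level-wide pedestrian total.
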(event `self.ReceiveBeginPlay`
  ;[1 1 1] 初期化処理
  (`self.fSetPeopleSpawnRange`) ; 人のトランスフォーム・移動距離を算出
  (`KismetSystemLibrary.K2_SetTimerDelegate` (delegate `SpawnPeople`) (`KismetMathLibrary.RandomFloatInRange` (`self.mMinPeopleSpawnInterval`) (`self.mMaxPeopleSpawnInterval`)) true))

(event `SpawnPeople`
  ;[1 1 1] 人の生成処理
  (bind _ismax (`self.fIsMaxSpawnPeopleNum`))
  (if (and (not _ismax) (< (`self.mSpawnPeopleNum`) (`self.MAX_SPAWN_ROAD_PEOPLE_NUM`)))
    (`/Engine/EditorBlueprintResources/StandardMacros.IncrementInt` (`self.mSpawnPeopleNum`)
      (:`  `
        (`self.fSetPeopleTransformAndDistance` 0) ; 人のトランスフォーム・移動距離を算出
        (switch `int` (`KismetMathLibrary.RandomIntegerInRange` 0 (`self.TOTAL_PEOPLE_NUM`))
          (:`0`
            (bind _returnvalue (`AIBlueprintHelperLibrary.SpawnAIFromClass` "/Game/Play/People/BP_PeopleMan01.BP_PeopleMan01_C" "/Game/Play/People/BT_PeopleNormal.BT_PeopleNormal" (`self.mPeopleSpawnTransform`) (`self.K2_GetActorRotation`) false null))
            (bind _asbp_people_man_01 (cast `/Game/Play/People/BP_PeopleMan01` _returnvalue))
            (set `/Game/Play/People/BP_PeopleBase.mInitializePeopleLocation` (`SceneComponent.K2_GetComponentLocation` (`self.PeopleSpawnPos1`)) _asbp_people_man_01))
          (:`1`
            (bind _returnvalue_2 (`AIBlueprintHelperLibrary.SpawnAIFromClass` "/Game/Play/People/BP_PeopleMan02.BP_PeopleMan02_C" "/Game/Play/People/BT_PeopleNormal.BT_PeopleNormal" (`self.mPeopleSpawnTransform`) (`self.K2_GetActorRotation`) false null))
            (bind _asbp_people_man_02 (cast `/Game/Play/People/BP_PeopleMan02` _returnvalue_2))
            (set `/Game/Play/People/BP_PeopleBase.mInitializePeopleLocation` (`SceneComponent.K2_GetComponentLocation` (`self.PeopleSpawnPos1`)) _asbp_people_man_02))
          (:`2`
            (bind _returnvalue_3 (`AIBlueprintHelperLibrary.SpawnAIFromClass` "/Game/Play/People/BP_PeopleWoman01.BP_PeopleWoman01_C" "/Game/Play/People/BT_PeopleNormal.BT_PeopleNormal" (`self.mPeopleSpawnTransform`) (`self.K2_GetActorRotation`) false null))
            (bind _asbp_people_woman_01 (cast `/Game/Play/People/BP_PeopleWoman01` _returnvalue_3))
            (set `/Game/Play/People/BP_PeopleBase.mInitializePeopleLocation` (`SceneComponent.K2_GetComponentLocation` (`self.PeopleSpawnPos1`)) _asbp_people_woman_01)))))))

(fn `fIsMaxSpawnPeopleNum`
  (returns (IsMax :type Boolean))
  ;[1 1 1] すでに人が出る最大人数を超えているか
  (bind _outactors (`GameplayStatics.GetAllActorsOfClass` "/Game/Play/People/BP_PeopleBase.BP_PeopleBase_C"))
  (return (>= (`KismetArrayLibrary.Array_Length` _outactors) (`self.MAX_SPAWN_PEOPLE_NUM`))))

(fn `fSetPeopleSpawnRange`
  (bind _mroad (`self.mRoad`))
  ;[1 1 1] 人を生成する範囲をセット
  (`/Engine/EditorBlueprintResources/StandardMacros.IsValid` _mroad
    (:`Is Valid`
      (`SceneComponent.SetWorldScale3D` (`self.PeopleSpawnRange`) (* (`self.GetActorScale3D` _mroad) (`self.GetActorScale3D`))))))

(fn `fSetPeopleTransformAndDistance`
  (params (PeopleNum :type Integer))
  ;[1 1 1] 人のトランスフォーム・移動距離を算出
  (set `self.mPeopleSpawnTransform` (`SceneComponent.K2_GetComponentLocation` (`self.PeopleSpawnPos1`))))

(fn `UserConstructionScript`)