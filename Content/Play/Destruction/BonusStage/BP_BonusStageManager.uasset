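; Manager actor that moves the player's Mayor character into the bonus stage and back.
; On BeginPlay it caches the first BP_BonusStageStart actor as the entry point.
; StartBonusStage saves the Mayor's location, moves them to that point and displays a WBP_BonusStageTimer widget.
; EndBonusStage restores the saved location behind a DoOnce that is never reset here, so the return fires only once.
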(event `StartBonusStage`
  ;[1 1 1] ボーナスステージに行く処理
  (bind _asbp_mayor (cast `/Game/Play/Destruction/Mayor/BP_Mayor` (`GameplayStatics.GetPlayerCharacter` 0)))
  (set `self.MayorBeforeLocation` (`self.K2_GetActorLocation` _asbp_mayor)) ; 市長がボーナスステージに行く前の座標をセット
  (`self.K2_SetActorLocation` _asbp_mayor (`self.K2_GetActorLocation` (`self.mBP_BonusStageStart`)) false false) ; 市長の座標をボーナスステージのスタート地点に
  (bind _returnvalue (`|CreateWidget` "/Game/Play/Destruction/BonusStage/Widget/WBP_BonusStageTimer.WBP_BonusStageTimer_C")) ; ボーナスステージタイマーウィジェットを作成
  (`UserWidget.AddToViewport` _returnvalue 0))

(event `self.ReceiveBeginPlay`
  ;[1 1 1] 初期化処理
  (bind _outactors (`GameplayStatics.GetAllActorsOfClass` "/Game/Play/Destruction/BonusStage/BP_BonusStageStart.BP_BonusStageStart_C"))
  (set `self.mBP_BonusStageStart` (`|GetArrayItem` _outactors)) ; ボーナスステージのスタート地点をセット
)

(event `EndBonusStage`
  ;[1 1 1] ボーナスステージから戻る処理
  (`/Engine/EditorBlueprintResources/StandardMacros.DoOnce` false
    (:`Completed`
      (bind _asbp_mayor (cast `/Game/Play/Destruction/Mayor/BP_Mayor` (`GameplayStatics.GetPlayerCharacter` 0)))
      (`self.K2_SetActorLocation` _asbp_mayor (`self.MayorBeforeLocation`) false false) ; 市長がボーナスステージに行く前の座標をセット
    )))

(fn `UserConstructionScript`)