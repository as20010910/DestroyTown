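; Player controller for the city destruction scene, routing input to the player's Mayor character.
; Caches the game mode and Mayor on BeginPlay, then drives camera-relative movement and look from axis inputs.
; A looping timer at the game mode's delta time, rather than Tick, clamps camera pitch.
; Attack switching is delegated to the game mode's attack-state widget, while attacking itself only prints the current state.
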(event `self.ReceiveBeginPlay`
  ;[1 1 1] 初期化
  (`self.SetGameMode`) ; ゲームモードをセット
  (`self.SetDestructionReference`) ; 破壊シーンに必要な参照をセット
  (`KismetSystemLibrary.K2_SetTimerDelegate` (delegate `EventTick`) (`/Game/Play/Destruction/GameMode/GM_DestructionCity.DELTA_TIME` (`self.mGM_DestructionCity`)) true))

(event `EventTick`
  ;[1 1 1] 更新処理
  (`self.Mayor Limit Camera Pitch` 0.0) ; 市長の縦方向の視点を制限
)

(event `SetGameMode`
  ;[1 1 1] ゲームモードをセット
  (set `self.mGM_DestructionCity` (cast `/Game/Play/Destruction/GameMode/GM_DestructionCity` (`GameplayStatics.GetGameMode`) :!pure true)))

(event `SetDestructionReference`
  ;[1 1 1] 破壊シーンに必要な参照をセット
  (bind _asbp_mayor (cast `/Game/Play/Destruction/Mayor/BP_Mayor` (`GameplayStatics.GetPlayerCharacter` 0)))
  (set `self.mBP_Mayor` _asbp_mayor) ; 市長のオブジェクト参照をセット
)

(event `InputAxis|MayorTurn`
  (params (AxisValue :type "Float (single-precision)"))
  ;[1 1 1] 市長の視点操作処理
  (`Pawn.AddControllerYawInput` (`self.mBP_Mayor`) AxisValue) ; 縦方向の視点
)

(event `InputAxis|MayorLookUp`
  (params (AxisValue :type "Float (single-precision)"))
  ;[1 1 1] 市長の視点操作処理
  (`Pawn.AddControllerPitchInput` (`self.mBP_Mayor`) AxisValue) ; 横方向の視点
)

(event `InputAxis|MayorMoveForward`
  (params (AxisValue :type "Float (single-precision)"))
  ;[1 1 1] 市長の移動処理
  (if (!= AxisValue 0.0)
    (`Pawn.AddMovementInput` (`self.mBP_Mayor`) (`KismetMathLibrary.GetForwardVector` (`KismetMathLibrary.MakeRotator` 0.0 0.0 (.yaw (`Pawn.GetControlRotation` (`self.mBP_Mayor`))))) AxisValue false) ; 移動させる
  ))

(event `InputAxis|MayorMoveRight`
  (params (AxisValue :type "Float (single-precision)"))
  ;[1 1 1] 市長の移動処理
  (if (!= AxisValue 0.0)
    (`Pawn.AddMovementInput` (`self.mBP_Mayor`) (`KismetMathLibrary.GetRightVector` (`KismetMathLibrary.MakeRotator` 0.0 0.0 (.yaw (`Pawn.GetControlRotation` (`self.mBP_Mayor`))))) AxisValue false) ; 移動させる
  ))

(event `InputAction|MayorAttack`
  (params (Key :type "Key Structure"))
  ;[1 1 1] 市長の攻撃処理
  (:`Pressed`
    ;[1 0.9179 0.03245] 市長が攻撃した状態を通知
    (bind _asbp_mayor (cast `/Game/Play/Destruction/Mayor/BP_Mayor` (`GameplayStatics.GetPlayerCharacter` 0)))
    (`KismetSystemLibrary.PrintString` (`KismetStringLibrary.Concat_StrStr` (`|GetEnumeratorNameAsString` (`/Game/Play/Destruction/Mayor/BP_Mayor.mEN_MayorAttackState` _asbp_mayor)) "で市長が攻撃した"))))

(event `InputAction|SwitchLeftMayorAttack`
  (params (Key :type "Key Structure"))
  ;[1 1 1] 攻撃状態を左に移動
  (:`Pressed`
    (`/Game/Play/Destruction/Widget/WBP_AttackState.SwitchLeftMayorAttacState` (`/Game/Play/Destruction/GameMode/GM_DestructionCity.mWBP_AttackState` (`self.mGM_DestructionCity`)))))

(event `InputAction|SwitchRightMayorAttack`
  (params (Key :type "Key Structure"))
  ;[1 1 1] 攻撃状態を右に移動
  (:`Pressed`
    (`/Game/Play/Destruction/Widget/WBP_AttackState.SwitchRightMayorAttacState` (`/Game/Play/Destruction/GameMode/GM_DestructionCity.mWBP_AttackState` (`self.mGM_DestructionCity`)))))

(fn `Mayor Limit Camera Pitch`
  (params (AxisValue :type "Float (double-precision)"))
  (locals (MinCameraPitch :type "Float (double-precision)" :default 5.0) (MaxCameraPitch :type "Float (double-precision)" :default 50.0))
  (bind (_returnvalue_roll _returnvalue_pitch _returnvalue_yaw) (`KismetMathLibrary.BreakRotator` (`self.GetControlRotation`)))
  ;[1 1 1] 市長の縦方向の視点を制限
  (`self.SetControlRotation` (`KismetMathLibrary.MakeRotator` _returnvalue_roll (`KismetMathLibrary.ClampAxis` (`KismetMathLibrary.ClampAngle` (+ AxisValue _returnvalue_pitch) (`local.MinCameraPitch`) (`local.MaxCameraPitch`))) _returnvalue_yaw)))

(fn `UserConstructionScript`)