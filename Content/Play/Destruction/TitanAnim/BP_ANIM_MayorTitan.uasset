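; Cutscene actor that plays the mayor's transformation into a titan in the destruction game mode.
; On BeginPlay it moves to the BP_MayorTitanAnimStart transform, takes the player's view, plays the voice and animation, and scales the mesh via a timeline.
; A looping timer tilts its camera's pitch up to a limit.
; When the timeline ends, it fades, flags completion, returns the view to BP_Mayor and destroys itself.
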(event `self.ReceiveBeginPlay`
  ;[1 1 1] 初期化
  (`self.fSetANIM_MayorTitan_Location`) ; 市長の巨人化アニメーション演出の初期トランスフォームをセット
  (`self.fChangeAnim_MayorTitanCamera`) ; カメラ視点を市長の巨人化アニメーション演出に
  (`self.fPlayMayorTitanVoice`) ; 市長が巨人化する際の声を再生
  (`SkeletalMeshComponent.PlayAnimation` (`self.SkeletalMesh`) (`self.mMayorTitanAnim`) false) ; 巨人化アニメーション演出を再生
  (bind _returnvalue (`KismetSystemLibrary.K2_SetTimerDelegate` (delegate `CameraMove`) (`self.GetDELTA_TIME`) true))
  (bind (_direction `_新規track_0`) (`Timeline|タイムライン_0` :!via `PlayFromStart`)
    (:`Update`
      (`SceneComponent.SetWorldScale3D` (`self.SkeletalMesh`) (`KismetMathLibrary.Conv_DoubleToVector` `_新規track_0`)) ; 市長のモデルのスケールをセット
    )
    (:`Finished`
      (`/Engine/EditorBlueprintResources/StandardMacros.DoOnce` false
        (:`Completed`
          (`self.Finalize`) ; 終了処理
        )))))

(event `CameraMove`
  (bind (_returnvalue_roll _returnvalue_pitch _returnvalue_yaw) (`KismetMathLibrary.BreakRotator` (`SceneComponent.K2_GetComponentRotation` (`self.Anim_MayorTitanCamera`))))
  (bind _returnvalue (+ _returnvalue_pitch (`self.mCameraMoveSpeed`)))
  ;[1 1 1] カメラの回転処理
  (if (<= (`self.MAX_CAMERA_ROTY`) _returnvalue)
    (`KismetSystemLibrary.K2_ClearAndInvalidateTimerHandle` (stale `self.ReceiveBeginPlay` _returnvalue))
    (else
      (bind _output_get (set `self.mCameraRotY` _returnvalue))
      (`SceneComponent.K2_SetWorldRotation` (`self.Anim_MayorTitanCamera`) (`KismetMathLibrary.MakeRotator` _returnvalue_roll _output_get _returnvalue_yaw) false false))))

(event `Finalize`
  ;[1 1 1] 終了処理
  (bind _asgm_destruction_city (cast `/Game/Play/Common/GameMode/GM_DestructionCity` (`GameplayStatics.GetGameMode`)))
  (`/Game/Play/Common/Fade/WBP_Fade.FadeInitialize` (`/Game/Play/Common/GameMode/GM_DestructionCity.mWBP_Fade` _asgm_destruction_city) "NewEnumerator0" 0.01)
  (`KismetSystemLibrary.Delay` 2.0)
  (set `self.mIsAnimTitanEnd` true) ; 巨人化アニメーション終了フラグをtrueに
  (`self.fResetAnim_MayorTitanCamera`) ; カメラ視点を市長のカメラにリセット
  (`SceneComponent.SetHiddenInGame` (`self.SkeletalMesh`) true false)
  (`KismetSystemLibrary.Delay` 0.2)
  (`self.K2_DestroyActor`))

(fn `fChangeAnim_MayorTitanCamera`
  ;[1 1 1] カメラ視点を市長の巨人化アニメーション演出に
  (`PlayerController.SetViewTargetWithBlend` (`GameplayStatics.GetPlayerController` 0) self 0.0 "VTBlend_Linear" 0.0 false))

(fn `fPlayMayorTitanVoice`
  ;[1 1 1] 市長が巨人化する際の声を再生
  (`/Game/Play/Destruction/Sounds/BP_DestructionSoundManager.PlaySoundEffects` (`/Game/Play/Destruction/BP_DestructionManager.mBP_DestructionSoundManager` (`/Game/Play/Common/GameMode/GM_DestructionCity.mBP_DestructionManager` (cast `/Game/Play/Common/GameMode/GM_DestructionCity` (`GameplayStatics.GetGameMode`) :!pure true))) "/Game/Play/Destruction/Sounds/SoundWave/Mayor/SoundEffect_MayorTitanVoice.SoundEffect_MayorTitanVoice" (0.0 0.0 0.0) 0.0))

(fn `fResetAnim_MayorTitanCamera`
  ;[1 1 1] カメラ視点を市長のカメラにリセット
  (bind _asbp_mayor (cast `/Game/Play/Destruction/Mayor/BP_Mayor` (`GameplayStatics.GetPlayerCharacter` 0)))
  (`PlayerController.SetViewTargetWithBlend` (`GameplayStatics.GetPlayerController` 0) _asbp_mayor 0.0 "VTBlend_Linear" 0.0 false))

(fn `fSetANIM_MayorTitan_Location`
  ;[1 1 1] 市長の巨人化アニメーション演出の初期トランスフォームをセット
  (bind _outactors (`GameplayStatics.GetAllActorsOfClass` "/Game/Play/Destruction/TitanAnim/BP_MayorTitanAnimStart.BP_MayorTitanAnimStart_C"))
  (`self.K2_SetActorTransform` (`self.GetTransform` (`|GetArrayItem` _outactors))))

(fn `UserConstructionScript`)