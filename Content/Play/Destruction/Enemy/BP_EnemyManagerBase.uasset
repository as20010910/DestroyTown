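; BP_EnemyManagerBase is a base enemy spawner that repeatedly creates enemies at its EnemySpawPos component.
; BeginPlay starts a looping timer at the configured interval.
; Each tick spawns the configured enemy class, either through SpawnAIFromClass with BT_Enemy or as a plain actor, depending on the AI flag.
; SetEnemyManagerInfo sets the enemy class, spawn interval and AI flag.
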(event `self.ReceiveBeginPlay`
  ;[1 1 1] 初期化処理
  (`KismetSystemLibrary.K2_SetTimerDelegate` (delegate `SpawnEnemy`) (`self.mEnemySpawnInterval`) true))

(event `SpawnEnemy`
  (bind _returnvalue (`SceneComponent.K2_GetComponentToWorld` (`self.EnemySpawPos`)))
  ;[1 1 1] 敵の生成処理
  (if (`self.mUseBehaviorAI`)
    (`AIBlueprintHelperLibrary.SpawnAIFromClass` (`self.mSpawnEnemy`) "/Game/Play/Destruction/Enemy/AI/BT_Enemy.BT_Enemy" (.location _returnvalue) (.rotation _returnvalue) false null) ; ビヘイビアAIを使用する敵の生成処理
    (else
      (`|SpawnActorFromClass` (`self.mSpawnEnemy`) _returnvalue "Undefined" "OverrideRootScale" null null) ; ビヘイビアAIを使用しない敵の生成処理
    )))

(fn `SetEnemyManagerInfo`
  (params (SpawnEnemy :type "/Game/Play/Destruction/Enemy/BP_EnemyBase Class Reference") (EnemySpawnInterval :type "Float (double-precision)") (UseAI :type Boolean))
  ;[1 1 1] 敵マネージャーの情報をセット
  (set `self.mSpawnEnemy` SpawnEnemy) ; 生成する敵クラスの参照
  (set `self.mEnemySpawnInterval` EnemySpawnInterval) ; 敵を生成する間隔
  (set `self.mUseBehaviorAI` UseAI) ; ビヘイビアAIを使用するかどうか
)

(fn `UserConstructionScript`)