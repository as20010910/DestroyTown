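; BP_EnemyStraight is an enemy in the Destruction City game mode that moves straight ahead.
; BeginPlay sets its enemy info by type, runs the parent setup, then starts a looping timer at the game mode's DELTATIME.
; That timer drives the straight-movement function in place of Event Tick.
; When the enemy mesh fractures, the enemy is destroyed through DestroyEnemy.
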(event `self.ReceiveBeginPlay`
  ;[1 1 1] 初期化処理
  (`self.fSetEnemyInfo` "NewEnumerator0") ; 敵の情報をセット
  (`parent.ReceiveBeginPlay`)
  (`KismetSystemLibrary.K2_SetTimerDelegate` (delegate `TIck`) (`/Game/Play/Common/GameMode/GM_DestructionCity.DELTA_TIME` (cast `/Game/Play/Common/GameMode/GM_DestructionCity` (`GameplayStatics.GetGameMode`) :!pure true)) true))

(event `self.EnemyMesh.OnComponentFracture`
  (params (HitPoint :type "Vector Structure (by ref)") (HitDirection :type "Vector Structure (by ref)"))
  ;[1 1 1] 敵が破壊されたときの処理
  (`self.DestroyEnemy`))

(event `TIck`
  ;[1 1 1] 更新処理
  (`self.fMove Straight`) ; 直進処理
)

(fn `UserConstructionScript`
  (`parent.UserConstructionScript`))