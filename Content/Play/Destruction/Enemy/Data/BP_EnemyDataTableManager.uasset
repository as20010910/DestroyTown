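; BP_EnemyDataTableManager caches enemy data from DT_EnemyData and serves it by enemy type.
; On BeginPlay, FSetTableData loops over the enum entry count, looks up rows named by index number, and appends each found row to MSTEnemyDataTable.
; FMap converts an enemy type to an integer to index that array, so lookups rely on row names matching enum order without gaps.
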(event `self.ReceiveBeginPlay`
  (`self.fSetTableData`) ; 敵のデータテーブルの情報をセット
)

(fn `fMap`
  (params (enemyType :type "/Game/Play/Destruction/Enemy/Data/EN_EnemyType Enum" :default "NewEnumerator0"))
  (returns (enemyDataTable :type "/Game/Play/Destruction/Enemy/Data/ST_EnemyDataTable Structure"))
  (locals (NewLocalVar_0 :type "/Game/Play/Building/Data/ST_BuildingDataTable Structure"))
  ;[1 1 1] 取得した敵の種類から対応するデータを返す
  (return (`|GetArrayItem` (`self.mST_EnemyDataTable`) (`KismetMathLibrary.Conv_ByteToInt` enemyType))))

(fn `fSetTableData`
  ;[1 1 1] 市長のデータテーブルの情報をセット
  (for _index (range (+ (enumcount `/Game/Play/Destruction/Mayor/Data/EN_MayorAttackState`) 1))
    (bind _returnvalue (`|GetDataTableRow` "/Game/Play/Destruction/Enemy/Data/DT_EnemyData.DT_EnemyData" (`KismetStringLibrary.Conv_StringToName` (`KismetStringLibrary.Conv_IntToString` _index)))
      (:`then`
        (`KismetArrayLibrary.Array_Add` (`self.mST_EnemyDataTable`) _returnvalue)))))

(fn `UserConstructionScript`)