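; Base enemy actor for the city destruction game, configured by type with a destructible mesh and damage-cost value from the manager's data table.
; Looping timers count down its lifetime and, for shooter types, spawn bullets, while a helper steps it straight forward.
; It outlines itself while the Mayor overlaps and passes hits to the destructible mesh.
; When destroyed, it adds its cost to the GameInstance's damage total, then removes itself after a delay.
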(event `self.ReceiveBeginPlay`
  ;[1 1 1] 初期化処理
  (`KismetSystemLibrary.K2_SetTimerDelegate` (delegate `DecreaseLife`) (`/Game/Play/Common/GameMode/GM_DestructionCity.DELTA_TIME` (cast `/Game/Play/Common/GameMode/GM_DestructionCity` (`GameplayStatics.GetGameMode`) :!pure true)) true)
  (if (`self.IsUseBullet`)
    (`KismetSystemLibrary.K2_SetTimerDelegate` (delegate `ShotBullet`) (`self.mBulletShotInterval`) true)))

(event `DecreaseLife`
  ;[1 1 1] ライフを徐々に減らす
  (bind _output_get (set `self.mLife` (- (`self.mLife`) (`/Game/Play/Common/GameMode/GM_DestructionCity.DELTA_TIME` (cast `/Game/Play/Common/GameMode/GM_DestructionCity` (`GameplayStatics.GetGameMode`) :!pure true)))))
  (if (<= _output_get 0.0)
    (`self.K2_DestroyActor`) ; 自身を削除
  ))

(event `ShotBullet`
  ;[1 1 1] 弾を発射
  (if (not (`self.IsDestroyed`))
    (`|SpawnActorFromClass` "/Game/Play/Destruction/Enemy/BP_EnemyBullet.BP_EnemyBullet_C" (`SceneComponent.K2_GetComponentToWorld` (`self.BulletSpawnPos`)) "Undefined" "OverrideRootScale" null null) ; 弾を発射
  ))

(event `EnemyApplyDamage`
  (params (AttackDamage :type "Float (double-precision)") (ImpluseDir :type "Vector Structure"))
  ;[1 1 1] 敵にダメージを与える処理
  (`DestructibleComponent.ApplyDamage` (`self.EnemyMesh`) AttackDamage (`SceneComponent.K2_GetComponentLocation` (`self.HitLocation`)) ImpluseDir 5000.0))

(event `self.DamageCollision.OnComponentBeginOverlap`
  (params (OverlappedComponent :type "PrimitiveComponent Object Reference") (OtherActor :type "Actor Object Reference") (OtherComp :type "PrimitiveComponent Object Reference") (OtherBodyIndex :type Integer) (bFromSweep :type Boolean) (SweepResult :type "HitResult Structure (by ref)"))
  ;[1 1 1] アウトライン処理
  (cast `/Game/Play/Destruction/Mayor/BP_Mayor` OtherActor)
  (if (not (`self.IsDestroyed`))
    (`SceneComponent.SetVisibility` (`self.OutLineMesh`) true false)))

(event `AddAmoutDamage`
  ;[1 1 1] 被害総額を加算する処理
  (bind _enemydatatable (`self.fGetEnemyData`)) ; 敵タイプに対応するデータの取得
  (bind _asgmi_destruction_city (cast `/Game/Play/Common/GameInstance/GMI_DestructionCIty` (`GameplayStatics.GetGameInstance`)))
  (`/Game/Play/Common/GameInstance/GMI_DestructionCIty.AddAmoutDamage` _asgmi_destruction_city (`.AmountDamage_6_A2721C0D45BCD5687997F084ABEEA959` (break `/Game/Play/Destruction/Enemy/Data/ST_EnemyDataTable` _enemydatatable))) ; 被害総額を加算
)

(event `self.DamageCollision.OnComponentEndOverlap`
  (params (OverlappedComponent :type "PrimitiveComponent Object Reference") (OtherActor :type "Actor Object Reference") (OtherComp :type "PrimitiveComponent Object Reference") (OtherBodyIndex :type Integer))
  ;[1 1 1] アウトライン処理
  (cast `/Game/Play/Destruction/Mayor/BP_Mayor` OtherActor)
  (if (not (`self.IsDestroyed`))
    (`SceneComponent.SetVisibility` (`self.OutLineMesh`) false false)))

(event `DestroyEnemy`
  ;[1 1 1] 敵が破壊された時の処理
  (set `self.IsDestroyed` true) ; 破壊されたにチェック
  (`PrimitiveComponent.SetCollisionEnabled` (`self.OutLineMesh`) "NoCollision")
  (`PrimitiveComponent.SetCollisionEnabled` (`self.DamageCollision`) "NoCollision")
  (`SceneComponent.SetVisibility` (`self.OutLineMesh`) false false) ; アウトラインを非表示
  (`self.AddAmoutDamage`) ; 被害総額を加算する処理
  (`KismetSystemLibrary.Delay` 2.0)
  (`self.K2_DestroyActor`))

(fn `fGetEnemyData`
  (returns (EnemyDataTable :type "/Game/Play/Destruction/Enemy/Data/ST_EnemyDataTable Structure"))
  ;[1 1 1] 敵タイプに対応するデータの取得
  (bind _asgm_destruction_city (cast `/Game/Play/Common/GameMode/GM_DestructionCity` (`GameplayStatics.GetGameMode`)))
  (bind _enemydatatable (`/Game/Play/Destruction/Enemy/Data/BP_EnemyDataTableManager.fMap` (`/Game/Play/Destruction/BP_DestructionManager.mBP_EnemyDataTableManager` (`/Game/Play/Common/GameMode/GM_DestructionCity.mBP_DestructionManager` _asgm_destruction_city)) (`self.mEnemyType`))) ; 敵のタイプに対応するデータを取得
  (return _enemydatatable))

(fn `fMove Straight`
  ;[1 1 1] 直進処理
  (if (not (`self.IsDestroyed`))
    (`self.K2_SetActorLocation` (+ (`self.K2_GetActorLocation`) (* (`KismetMathLibrary.GetForwardVector` (`self.K2_GetActorRotation`)) (`self.mMoveSpeed`))))))

(fn `fSetEnemyInfo`
  (params (EnemyType :type "/Game/Play/Destruction/Enemy/Data/EN_EnemyType Enum" :default "NewEnumerator0") (Life :type "Float (double-precision)") (UseBullet :type Boolean) (BulletShotInterval :type "Float (double-precision)"))
  ;[1 1 1] 敵の情報をセット
  (set `self.mEnemyType` EnemyType) ; 敵のタイプ
  (set `self.mLife` Life) ; ライフ
  (set `self.IsUseBullet` UseBullet) ; 弾を発射するかどうか
  (set `self.mBulletShotInterval` BulletShotInterval) ; 弾の発射間隔
  (bind _enemydatatable (`self.fGetEnemyData`)) ; 敵タイプに対応するデータの取得
  (set `DestructibleComponent.DestructibleMesh` (`.DestructibleMesh_11_3B3A8E4E4B4CDC0113A015AF2C99D1AE` (break `/Game/Play/Destruction/Enemy/Data/ST_EnemyDataTable` _enemydatatable)) (`self.EnemyMesh`)) ; メッシュをセット
)

(fn `UserConstructionScript`)