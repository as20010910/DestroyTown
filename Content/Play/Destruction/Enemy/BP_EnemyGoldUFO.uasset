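; Gold UFO enemy for the Destruction City mode that circles around its actor origin until destroyed.
; BeginPlay sets its enemy type and life, runs the parent logic, then offsets the outline, mesh, hit location and damage collision by the move radius vector.
; A looping DELTATIME timer adds yaw to the actor, swinging those offset components in an orbit.
; Fracture of the enemy mesh triggers DestroyEnemy.
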(event `self.ReceiveBeginPlay`
  ;[1 1 1] 初期化処理
  (`self.fSetEnemyInfo` "NewEnumerator2" (`self.ENEMY_GOLDUFO_LIFE`)) ; 敵の情報をセット
  (`parent.ReceiveBeginPlay`)
  (`self.SetMoveRotRadius`) ; 回転移動する半径をセット
  (`KismetSystemLibrary.K2_SetTimerDelegate` (delegate `TIck`) (`/Game/Play/Common/GameMode/GM_DestructionCity.DELTA_TIME` (cast `/Game/Play/Common/GameMode/GM_DestructionCity` (`GameplayStatics.GetGameMode`) :!pure true)) true))

(event `self.EnemyMesh.OnComponentFracture`
  (params (HitPoint :type "Vector Structure (by ref)") (HitDirection :type "Vector Structure (by ref)"))
  ;[1 1 1] 敵が破壊されたときの処理
  (`self.DestroyEnemy`))

(event `TIck`
  (bind (_returnvalue_roll _returnvalue_pitch _returnvalue_yaw) (`KismetMathLibrary.BreakRotator` (`self.K2_GetActorRotation`)))
  ;[1 1 1] 更新処理
  (if (not (`self.IsDestroyed`))
    (`self.K2_SetActorRotation` (`KismetMathLibrary.MakeRotator` _returnvalue_roll _returnvalue_pitch (+ _returnvalue_yaw (`self.mRotMoveSpeed`))))))

(fn `Add Location`
  (params (Location :type "Vector Structure") (AddLocation :type "Vector Structure") (Component :type "SceneComponent Object Reference"))
  ;[1 1 1] 座標の加算処理
  (`SceneComponent.K2_SetWorldLocation` Component (+ Location AddLocation) false false))

(fn `SetMoveRotRadius`
  (bind _enemymesh (`self.EnemyMesh`))
  (bind _hitlocation (`self.HitLocation`))
  (bind _damagecollision (`self.DamageCollision`))
  (bind _outlinemesh (`self.OutLineMesh`))
  ;[1 1 1] 回転移動する半径をセット
  (`self.Add Location` (`SceneComponent.K2_GetComponentLocation` _outlinemesh) (`self.mMoveRotRadius`) _outlinemesh) ; アウトラインメッシュ
  (`self.Add Location` (`SceneComponent.K2_GetComponentLocation` _enemymesh) (`self.mMoveRotRadius`) _enemymesh) ; 敵のメッシュ
  (`self.Add Location` (`SceneComponent.K2_GetComponentLocation` _hitlocation) (`self.mMoveRotRadius`) _hitlocation) ; ダメージを与える場所
  (`self.Add Location` (`SceneComponent.K2_GetComponentLocation` _damagecollision) (`self.mMoveRotRadius`) _damagecollision) ; ダメージを受けるコリジョン
)

(fn `UserConstructionScript`
  (`parent.UserConstructionScript`))