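; BP_EnemyManagerGoldUFO schedules the one-time appearance of the gold UFO enemy during play.
; On BeginPlay it sets a non-looping timer with a random delay between the minimum and maximum spawn times.
; When the timer fires, it spawns BP_EnemyGoldUFO at the BP_Mayor player character's transform and adds the WBP_SpawnGoldUFO announcement widget to the viewport.
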(event `self.ReceiveBeginPlay`
  ;[1 1 1] 初期化処理
  (`KismetSystemLibrary.K2_SetTimerDelegate` (delegate `SpawnEnemyGoldUFO`) (`KismetMathLibrary.RandomFloatInRange` (`self.MinSpawnTime`) (`self.MaxSpawnTime`))))

(event `SpawnEnemyGoldUFO`
  ;[1 1 1] 金のUFO出現処理
  (bind _asbp_mayor (cast `/Game/Play/Destruction/Mayor/BP_Mayor` (`GameplayStatics.GetPlayerCharacter` 0)))
  (`|SpawnActorFromClass` "/Game/Play/Destruction/Enemy/BP_EnemyGoldUFO.BP_EnemyGoldUFO_C" (`self.GetTransform` _asbp_mayor) "Undefined" "OverrideRootScale" null null) ; 金のUFOをスポーン
  (bind _returnvalue (`|CreateWidget` "/Game/Play/Destruction/Widget/WBP_SpawnGoldUFO.WBP_SpawnGoldUFO_C")) ; 金のUFOが出現した演出ウィジェットを生成
  (`UserWidget.AddToViewport` _returnvalue 0))

(fn `UserConstructionScript`)