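; BP_EnemyBullet is an enemy projectile in the Destruction game mode that damages the mayor on contact.
; A looping timer at the game mode's DELTATIME interval counts down its life and destroys it at zero.
; When its collision overlaps BP_Mayor, it applies bullet damage, spawns a damage particle at its own transform, then destroys itself after a short delay.
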(event `self.ReceiveBeginPlay`
  ;[1 1 1] 初期化処理
  (`KismetSystemLibrary.K2_SetTimerDelegate` (delegate `DecreaseLife`) (`/Game/Play/Common/GameMode/GM_DestructionCity.DELTA_TIME` (cast `/Game/Play/Common/GameMode/GM_DestructionCity` (`GameplayStatics.GetGameMode`) :!pure true)) true))

(event `DecreaseLife`
  ;[1 1 1] ライフを徐々に減らす
  (bind _output_get (set `self.mLife` (- (`self.mLife`) (`/Game/Play/Common/GameMode/GM_DestructionCity.DELTA_TIME` (cast `/Game/Play/Common/GameMode/GM_DestructionCity` (`GameplayStatics.GetGameMode`) :!pure true)))))
  (if (<= _output_get 0.0)
    (`self.K2_DestroyActor`) ; 自身を削除
  ))

(event `self.BulletCollision.OnComponentBeginOverlap`
  (params (OverlappedComponent :type "PrimitiveComponent Object Reference") (OtherActor :type "Actor Object Reference") (OtherComp :type "PrimitiveComponent Object Reference") (OtherBodyIndex :type Integer) (bFromSweep :type Boolean) (SweepResult :type "HitResult Structure (by ref)"))
  (bind (_returnvalue_location _returnvalue_rotation _returnvalue_scale) (`KismetMathLibrary.BreakTransform` (`self.GetTransform`)))
  ;[1 1 1] 弾が市長に当たった際の処理
  (bind _asbp_mayor (cast `/Game/Play/Destruction/Mayor/BP_Mayor` OtherActor))
  (`/Game/Play/Destruction/Mayor/BP_Mayor.fAddDamage` _asbp_mayor (`self.mBulletDamage`)) ; 市長に弾のダメージを与える
  (`GameplayStatics.SpawnEmitterAtLocation` "/Game/UseEffect/P_MayorDamage.P_MayorDamage" _returnvalue_location _returnvalue_rotation _returnvalue_scale) ; 市長がダメージを受けた際のエフェクトを生成
  (`KismetSystemLibrary.Delay` 0.2)
  (`self.K2_DestroyActor`) ; 自信を削除
)

(fn `UserConstructionScript`)