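; Data manager Blueprint that serves the mayor's attack settings from DT_MayorAttack by attack state.
; On BeginPlay it loops over enum indices, looks up rows named by those numbers and appends each found row to an array.
; FMap returns the array element at the attack state's integer value, so missing rows would shift that mapping.
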(event `self.ReceiveBeginPlay`
  (`self.fSetTableData`) ; 市長のデータテーブルの情報をセット
)

(fn `fMap`
  (params (mayorAttackState :type "/Game/Play/Destruction/Data/EN_MayorAttackState Enum" :default "NewEnumerator0"))
  (returns (mayorDataTable :type "/Game/Play/Destruction/Data/ST_MayorDatatable Structure"))
  (locals (NewLocalVar_0 :type "/Game/Play/Building/Data/ST_BuildingDataTable Structure"))
  ;[1 1 1] 取得した攻撃状態から対応するデータを返す
  (return (`|GetArrayItem` (`self.mST_BuildingDataTable`) (`KismetMathLibrary.Conv_ByteToInt` mayorAttackState))))

(fn `fSetTableData`
  ;[1 1 1] 市長のデータテーブルの情報をセット
  (for _index (range (+ (enumcount `/Game/Play/Destruction/Data/EN_MayorAttackState`) 1))
    (bind _returnvalue (`|GetDataTableRow` "/Game/Play/Destruction/Data/DT_MayorAttack.DT_MayorAttack" (`KismetStringLibrary.Conv_StringToName` (`KismetStringLibrary.Conv_IntToString` _index)))
      (:`then`
        (`KismetArrayLibrary.Array_Add` (`self.mST_BuildingDataTable`) _returnvalue)))))

(fn `UserConstructionScript`)