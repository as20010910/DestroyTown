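; Sound manager Blueprint for the Destruction game mode, handling background music and positional sound effects.
; BGM plays, stops and changes volume through a single audio component, while effects play at a given location using the stored effects volume.
; A looping timer at the game mode's DELTATIME interval copies both volume settings from the game instance's pause structure while the pause menu is active.
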(event `self.ReceiveBeginPlay`
  ;[1 1 1] 初期化
  (bind _asgm_destruction_city (cast `/Game/Play/Common/GameMode/GM_DestructionCity` (`GameplayStatics.GetGameMode`)))
  (`KismetSystemLibrary.K2_SetTimerDelegate` (delegate `Tick`) (`/Game/Play/Common/GameMode/GM_DestructionCity.DELTA_TIME` _asgm_destruction_city) true))

(event `Tick`
  (bind _asgmi_destruction_city (cast `/Game/Play/Common/GameInstance/GMI_DestructionCIty` (`GameplayStatics.GetGameInstance`) :!pure true))
  (bind (_mst_pausestructure_mbgmpercent _mst_pausestructure_msepercent) (break `/Game/Pause/ST_PauseStructure` (`/Game/Play/Common/GameInstance/GMI_DestructionCIty.mST_PauseStructure` _asgmi_destruction_city)))
  ;[1 1 1] 更新処理
  (if (`|EnumEquality` (`/Game/Play/Common/GameInstance/GMI_DestructionCIty.mPause` _asgmi_destruction_city) "NewEnumerator0")
    (bind _output_get (set `self.mBGMVolume` _mst_pausestructure_mbgmpercent)) ; BGMの音量をセット
    (`self.ChangeBGMVolume` _output_get)
    (bind _output_get_2 (set `self.mSoundEffectVolume` _mst_pausestructure_msepercent)) ; 効果音の音量をセット
    (`self.ChangeSoundEffectsVolume` _output_get_2)))

(fn `ChangeBGMVolume`
  (params (Volume :type "Float (double-precision)"))
  ;[1 1 1] BGMの音量調整
  (`AudioComponent.SetVolumeMultiplier` (`self.BGM`) Volume))

(fn `ChangeSoundEffectsVolume`
  (params (Volume :type "Float (double-precision)"))
  ;[1 1 1] 効果音の音量調整
  (set `self.mSoundEffectVolume` Volume))

(fn `PlayBGM`
  (params (BGM :type "SoundBase Object Reference"))
  (bind _bgm (`self.BGM`))
  ;[1 1 1] ＢＧＭを再生
  (`/Engine/EditorBlueprintResources/StandardMacros.IsValid` BGM
    (:`Is Valid`
      (`AudioComponent.SetSound` _bgm BGM)
      (`AudioComponent.SetVolumeMultiplier` _bgm (`self.mBGMVolume`))
      (`AudioComponent.Play` _bgm 0.0))))

(fn `PlaySoundEffects`
  (params (SoundEffects :type "SoundBase Object Reference") (Location :type "Vector Structure") (StartTime :type "Float (double-precision)"))
  ;[1 1 1] 効果音を再生
  (`/Engine/EditorBlueprintResources/StandardMacros.IsValid` SoundEffects
    (:`Is Valid`
      (`GameplayStatics.PlaySoundAtLocation` SoundEffects Location (struct) (`self.mSoundEffectVolume`) 1.0 StartTime null null null))))

(fn `StopBGM`
  ;[1 1 1] BGMを止める
  (`AudioComponent.Stop` (`self.BGM`)))

(fn `UserConstructionScript`)