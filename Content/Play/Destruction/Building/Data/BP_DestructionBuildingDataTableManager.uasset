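; Building data manager for the destruction gameplay, serving DT_DestructionBuildingDataTable rows by building type.
; On BeginPlay, FSetTableData loops over an enum's entry count, looks up rows named by index and appends those found to an array.
; FMap converts a building type to an integer, decrements it and returns that array element only when the index is above zero.
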(event `self.ReceiveBeginPlay`
  (`self.fSetTableData`) ; 建物のデータテーブルの情報をセット
)

(fn `fMap`
  (params (BuildingType :type "/Game/Play/Building/Data/EN_Building Enum" :default "NewEnumerator13"))
  (returns (buildingDataTable :type "/Game/Play/Destruction/Building/Data/ST_DestructionBuilidngData Structure"))
  ;[1 1 1] 取得した建物タイプから対応するデータを返す
  (bind _result (`/Engine/EditorBlueprintResources/StandardMacros.DecrementInt` (`KismetMathLibrary.Conv_ByteToInt` BuildingType))
    (:`  `
      (if (> _result 0)
        (return (`|GetArrayItem` (`self.mST_DestructionBuildingDataTable`) _result))))))

(fn `fSetTableData`
  ;[1 1 1] 建物のデータテーブルの情報をセット
  (for _index (range (+ (enumcount `/Game/Play/Building/Data/EN_Building`) 1))
    (bind _returnvalue (`|GetDataTableRow` "/Game/Play/Destruction/Building/Data/DT_DestructionBuildingDataTable.DT_DestructionBuildingDataTable" (`KismetStringLibrary.Conv_StringToName` (`KismetStringLibrary.Conv_IntToString` _index)))
      (:`then`
        (`KismetArrayLibrary.Array_Add` (`self.mST_DestructionBuildingDataTable`) _returnvalue)))))

(fn `UserConstructionScript`)