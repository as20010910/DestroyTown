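; Fire-spread actor for the destruction city game that carries fire from one wooden building to the next.
; On BeginPlay it plays a sound, spawns a fire emitter and starts a looping timer that counts down its life.
; Wooden, unburned buildings overlapping FireRange may, after a delay and weighted roll, take damage, get flagged and spawn another BP_SpreadOfFire, chaining the spread.
; At end of life, a timeline rescales the emitter before destroying it and the actor.
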(event `self.ReceiveBeginPlay`
  (bind _mspreadfiresound (`self.mSpreadFireSound`))
  ;[1 1 1] 初期化処理
  (`/Engine/EditorBlueprintResources/StandardMacros.IsValid` _mspreadfiresound
    (:`Is Valid`
      (`GameplayStatics.PlaySoundAtLocation` _mspreadfiresound (`self.K2_GetActorLocation`) (struct) 1.0 1.0 0.0 null null null) ; 建物延焼の効果音を再生
      (`self.SpawnEffectSpreadOfFire`) ; 建物延焼時のエフェクトを生成
      (`KismetSystemLibrary.K2_SetTimerDelegate` (delegate `Tick`) (`/Game/Play/Common/GameMode/GM_DestructionCity.DELTA_TIME` (cast `/Game/Play/Common/GameMode/GM_DestructionCity` (`GameplayStatics.GetGameMode`) :!pure true)) true))))

(event `self.FireRange.OnComponentBeginOverlap`
  (params (OverlappedComponent :type "PrimitiveComponent Object Reference") (OtherActor :type "Actor Object Reference") (OtherComp :type "PrimitiveComponent Object Reference") (OtherBodyIndex :type Integer) (bFromSweep :type Boolean) (SweepResult :type "HitResult Structure (by ref)"))
  ;[1 1 1] 延焼範囲に触れた時の処理
  (bind _asbp_building_base (cast `/Game/Play/Building/BP_Building/BP_BuildingBase` OtherActor))
  (if (`KismetSystemLibrary.IsValid` _asbp_building_base)
    (bind _iswooden (`self.fCheckWoodenBuilding` _asbp_building_base)) ; 建物が木造がどうか調べる
    (if (and _iswooden (not (`/Game/Play/Building/BP_Building/BP_BuildingBase.mIsSpreadOfFire` _asbp_building_base)))
      (`self.Further Spread Of Fire` _asbp_building_base) ; さらに延焼する処理
    )))

(event `Tick`
  ;[1 1 1] 更新処理
  (bind _output_get (set `self.mLife` (- (`self.mLife`) (`/Game/Play/Common/GameMode/GM_DestructionCity.DELTA_TIME` (cast `/Game/Play/Common/GameMode/GM_DestructionCity` (`GameplayStatics.GetGameMode`) :!pure true)))))
  (if (<= _output_get 0.0)
    (`/Engine/EditorBlueprintResources/StandardMacros.DoOnce` false
      (:`Completed`
        (`self.DestroyEffect`) ; エフェクトを削除する処理
      ))))

(event `Further Spread Of Fire`
  (params (NewParam :type "/Game/Play/Building/BP_Building/BP_BuildingBase Object Reference"))
  (bind (_returnvalue_location _returnvalue_rotation) (`KismetMathLibrary.BreakTransform` (`self.GetTransform` NewParam)))
  ;[1 1 1] さらに延焼する処理
  (`KismetSystemLibrary.Delay` 0.8)
  (if (`KismetMathLibrary.RandomBoolWithWeight` (`self.ProbabilityOfSpreadOfFire`))
    (`self.fApplyDamageWoodenBuilding` NewParam) ; 木造建物にダメージ
    (set `/Game/Play/Building/BP_Building/BP_BuildingBase.mIsSpreadOfFire` true NewParam) ; 延焼状態フラグをオンに
    (`|SpawnActorFromClass` "BP_SpreadOfFire_C" (`KismetMathLibrary.MakeTransform` _returnvalue_location _returnvalue_rotation) "Undefined" "OverrideRootScale" null null) ; さらに延焼アクタを追加
  ))

(event `SpawnEffectSpreadOfFire`
  (bind (_returnvalue_location _returnvalue_rotation) (`KismetMathLibrary.BreakTransform` (`self.GetTransform`)))
  ;[1 1 1] 建物延焼時のエフェクトを生成
  (bind _returnvalue (`GameplayStatics.SpawnEmitterAtLocation` "/Game/UseEffect/P_SpreadOfFire.P_SpreadOfFire" _returnvalue_location _returnvalue_rotation (3.0 3.0 3.0)))
  (set `self.mSpreadOfFireEffect` _returnvalue))

(event `DestroyEffect`
  (bind _mspreadoffireeffect (`self.mSpreadOfFireEffect`))
  ;[1 1 1] エフェクトを削除する処理
  (bind (_direction `_新規track_0`) (`Timeline|TL_SpreadOfFireEffectScale` :!via `PlayFromStart`)
    (:`Update`
      (`SceneComponent.SetWorldScale3D` _mspreadoffireeffect (* (`SceneComponent.K2_GetComponentScale` _mspreadoffireeffect) `_新規track_0`)) ; 延焼エフェクトのスケールをセット
    )
    (:`Finished`
      (`ActorComponent.K2_DestroyComponent` (`self.mSpreadOfFireEffect`)) ; 延焼エフェクトを削除
      (`self.K2_DestroyActor`) ; 終わったら自身を削除
    )))

(fn `fApplyDamageWoodenBuilding`
  (params (HitBuilding :type "/Game/Play/Building/BP_Building/BP_BuildingBase Object Reference"))
  (locals (SPREAD_OF_FIRE_DAMAGE :type "Float (double-precision)" :default 300.0))
  ;[1 1 1] 当たった木造の家にダメージを与える
  (if (`KismetSystemLibrary.IsValid` HitBuilding)
    (`/Game/Play/Building/BP_Building/BP_BuildingBase.BuildingApplyDamage` HitBuilding (`local.SPREAD_OF_FIRE_DAMAGE`) (0.0 0.0 0.0) 500.0)))

(fn `fCheckWoodenBuilding`
  (params (HitBuilding :type "/Game/Play/Building/BP_Building/BP_BuildingBase Object Reference"))
  (returns (IsWooden :type Boolean))
  (bind _mbuilding (`/Game/Play/Building/BP_Building/BP_BuildingBase.mBuilding` HitBuilding))
  ;[1 1 1] 建物が木造がどうか調べる
  (return (or (`|EnumEquality` _mbuilding "NewEnumerator0") (`|EnumEquality` _mbuilding "NewEnumerator1"))))

(fn `fFurther Spread Of Fire`
  (params (HitBuilding :type "/Game/Play/Building/BP_Building/BP_BuildingBase Object Reference"))
  (bind (_returnvalue_location _returnvalue_rotation) (`KismetMathLibrary.BreakTransform` (`self.GetTransform` HitBuilding)))
  ;[1 1 1] さらに延焼する処理
  (if (`KismetMathLibrary.RandomBoolWithWeight` (`self.ProbabilityOfSpreadOfFire`))
    (`self.fApplyDamageWoodenBuilding` HitBuilding) ; 木造建物にダメージ
    (set `/Game/Play/Building/BP_Building/BP_BuildingBase.mIsSpreadOfFire` true HitBuilding) ; 延焼状態フラグをオンに
    (`|SpawnActorFromClass` "BP_SpreadOfFire_C" (`KismetMathLibrary.MakeTransform` _returnvalue_location _returnvalue_rotation) "Undefined" "OverrideRootScale" null null) ; さらに延焼アクタを追加
    (else
      (`KismetSystemLibrary.PrintString` "Hello"))))

(fn `UserConstructionScript`)