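; BP_MayorStatusUpRatio calculates status-up multipliers for the Mayor's HP and attack damage.
; The HP ratio is one hundredth of the remaining total money and the attack ratio one hundredth of the total people count, both read from the GMI_DestructionCIty game instance.
; A shared helper, fLimitRatio, clamps each result between that stat's minimum and maximum limits.
; The event graph and construction script are empty.
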(fn `fGetMayorAttackDamageUpRatio`
  (returns (AttackDamageupRatio :type "Float (double-precision)"))
  (locals (MAX_ATTACKDAMAGE_UP_RATIO :type "Float (double-precision)" :default 1.3) (MIN_ATTACKDAMAGE_UP_RATIO :type "Float (double-precision)" :default 1.0) (AttackDamageUpRatioValue :type "Float (double-precision)"))
  ;[1 1 1] 攻撃力の倍率計算
  (bind _output_get (set `local.AttackDamageUpRatioValue` (* (`KismetMathLibrary.Conv_IntToDouble` (`/Game/Play/Common/GameInstance/GMI_DestructionCIty.mTotalPeopleNum` (cast `/Game/Play/Common/GameInstance/GMI_DestructionCIty` (`GameplayStatics.GetGameInstance`) :!pure true))) 0.01)))
  (bind _revalue (`self.fLimitRatio` _output_get (`local.MAX_ATTACKDAMAGE_UP_RATIO`) (`local.MIN_ATTACKDAMAGE_UP_RATIO`))) ; 値の最小値・最大値の制限
  (return _revalue))

(fn `fGetMayorHPUpRatio`
  (returns (HPupRatio :type "Float (double-precision)"))
  (locals (MAX_HPUP_RATIO :type "Float (double-precision)" :default 1.3) (MIN_HPUP_RATIO :type "Float (double-precision)") (HPUpRatioValue :type "Float (double-precision)"))
  ;[1 1 1] HPUpの倍率計算
  (bind _output_get (set `local.HPUpRatioValue` (* (`KismetMathLibrary.Conv_IntToDouble` (`/Game/Play/Common/GameInstance/GMI_DestructionCIty.mRemainingTotalMoney` (cast `/Game/Play/Common/GameInstance/GMI_DestructionCIty` (`GameplayStatics.GetGameInstance`) :!pure true))) 0.01)))
  (bind _revalue (`self.fLimitRatio` _output_get (`local.MAX_HPUP_RATIO`) (`local.MIN_HPUP_RATIO`))) ; 値の最小値・最大値の制限
  (return _revalue))

(fn `fLimitRatio`
  (params (Value :type "Float (double-precision)") (MaxValue :type "Float (double-precision)") (MinValue :type "Float (double-precision)"))
  (returns (ReValue :type "Float (double-precision)"))
  (locals (Value_ :type "Float (double-precision)") (MaxValue_ :type "Float (double-precision)") (MinValue_ :type "Float (double-precision)"))
  ;[1 1 1] 値の最小値・最大値の制限
  (set `local.Value_` Value)
  (set `local.MaxValue_` MaxValue)
  (set `local.MinValue_` MinValue)
  (if (>= (`local.Value_`) (`local.MaxValue_`))
    (set `local.Value_` (`local.MaxValue_`))
    (elif (<= (`local.Value_`) (`local.MinValue_`))
      (set `local.Value_` (`local.MinValue_`))))
  (return (`local.Value_`)))

(fn `UserConstructionScript`)