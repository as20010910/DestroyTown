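; BP_MiddleStoryManager runs the mid-game story scene, from its opening fade and BGM to shutdown.
; Initialization triggers the game mode's fade widget, spawns BP_MiddleStorySoundManager and starts a looping DELTATIME timer as its update.
; Once the story widget (built by FCreateStory, not called here) reports its end, it stops the BGM, sets a finish flag after a short delay and destroys the sound manager.
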(event `MiddleStoryInitialize`
  ;[1 1 1] 初期化処理
  (`self.fStartFadeOut`) ; 中盤ストーリーのフェード開始処理
  (`self.fCreateMiddleStorySoundManager`) ; 中盤ストーリーシーンのサウンドマネージャーの生成処理
  (`KismetSystemLibrary.K2_SetTimerDelegate` (delegate `Tick`) (`/Game/Play/Common/GameMode/GM_DestructionCity.DELTA_TIME` (cast `/Game/Play/Common/GameMode/GM_DestructionCity` (`GameplayStatics.GetGameMode`) :!pure true)) true))

(event `Tick`
  ;[1 1 1] 更新処理
  (if (`/Game/Play/Story/WBP_Story.IsStoryEnd` (`self.mWBP_Story`))
    (`/Engine/EditorBlueprintResources/StandardMacros.DoOnce` false
      (:`Completed`
        (`self.Finalize`) ; 終了処理
      ))))

(event `Finalize`
  (bind _mmiddlestorysoundmanager (`self.mMiddleStorySoundManager`))
  ;[1 1 1] 終了処理
  (`/Engine/EditorBlueprintResources/StandardMacros.DoOnce` false
    (:`Completed`
      (`/Game/Play/Story/BP_MiddleStorySoundManager.StopBGM` _mmiddlestorysoundmanager) ; BGMを止める
      (`KismetSystemLibrary.Delay` 0.2)
      (set `self.mFinish` true) ; 中盤ストーリーシーンが終了したか確認フラグをTrueに
      (`self.K2_DestroyActor` _mmiddlestorysoundmanager))))

(fn `fCreateMiddleStorySoundManager`
  ;[1 1 1] 中盤ストーリーシーンのサウンドマネージャーの生成処理
  (bind _returnvalue (`|SpawnActorFromClass` "/Game/Play/Story/BP_MiddleStorySoundManager.BP_MiddleStorySoundManager_C" (`KismetMathLibrary.MakeTransform` (0.0 0.0 0.0)) "Undefined" "OverrideRootScale" null null))
  (bind _output_get (set `self.mMiddleStorySoundManager` _returnvalue))
  (`/Game/Play/Story/BP_MiddleStorySoundManager.PlayBGM` _output_get) ; BGMを再生
)

(fn `fCreateStory`
  ;[1 1 1] ストーリーウィジェットを生成
  (bind _returnvalue (`|CreateWidget` "/Game/Play/Story/WBP_Story.WBP_Story_C" null "NewEnumerator1"))
  (bind _output_get (set `self.mWBP_Story` _returnvalue))
  (`UserWidget.AddToViewport` _output_get 1))

(fn `fStartFadeIn`
  ;[1 1 1] 中盤ストーリーのフェードイン開始処理
  (`/Engine/EditorBlueprintResources/StandardMacros.DoOnce` false
    (:`Completed`
      (`/Game/Play/Common/Fade/WBP_Fade.FadeInitialize` (`/Game/Play/Common/GameMode/GM_DestructionCity.mWBP_Fade` (cast `/Game/Play/Common/GameMode/GM_DestructionCity` (`GameplayStatics.GetGameMode`) :!pure true)) "NewEnumerator0" 0.005))))

(fn `fStartFadeOut`
  ;[1 1 1] 中盤ストーリーのフェードアウト開始処理
  (`/Engine/EditorBlueprintResources/StandardMacros.DoOnce` false
    (:`Completed`
      (`/Game/Play/Common/Fade/WBP_Fade.FadeInitialize` (`/Game/Play/Common/GameMode/GM_DestructionCity.mWBP_Fade` (cast `/Game/Play/Common/GameMode/GM_DestructionCity` (`GameplayStatics.GetGameMode`) :!pure true)) "NewEnumerator1" 0.05))))

(fn `UserConstructionScript`)