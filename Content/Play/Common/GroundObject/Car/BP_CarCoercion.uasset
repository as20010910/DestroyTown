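; Car-related ground object that shifts its own position when a car touches one of its two box colliders.
; Hit and overlap events on both boxes act only for BP_CarBase actors whose traffic-light contact equals their Reset value, meaning no light contact.
; Coercion then teleports this actor to the touched box's X or Y, chosen by INSTNorthSouthFlag, keeping the other coordinates.
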(event `self.ReceiveActorBeginOverlap`
  (params (OtherActor :type "Actor Object Reference")))

(event `self.Box.OnComponentHit`
  (params (HitComponent :type "PrimitiveComponent Object Reference") (OtherActor :type "Actor Object Reference") (OtherComp :type "PrimitiveComponent Object Reference") (NormalImpulse :type "Vector Structure") (Hit :type "HitResult Structure (by ref)"))
  (bind (_asbp_car_base _bsuccess) (cast `/Game/Play/Common/GroundObject/Car/BP_CarBase` OtherActor :!pure true))
  ;[1 1 1] 衝突したものが車だったら
  (if _bsuccess
    ;[1 1 1] 衝突した車が信号機に触れていなかったら
    (if (== (`/Game/Play/Common/GroundObject/Car/BP_CarBase.HitTraficLight` _asbp_car_base) (`/Game/Play/Common/GroundObject/Car/BP_CarBase.Reset` _asbp_car_base))
      (`self.Coercion` (`self.Box`)))))

(event `self.Box1.OnComponentHit`
  (params (HitComponent :type "PrimitiveComponent Object Reference") (OtherActor :type "Actor Object Reference") (OtherComp :type "PrimitiveComponent Object Reference") (NormalImpulse :type "Vector Structure") (Hit :type "HitResult Structure (by ref)"))
  (bind (_asbp_car_base _bsuccess) (cast `/Game/Play/Common/GroundObject/Car/BP_CarBase` OtherActor :!pure true))
  ;[1 1 1] 衝突したものが車だったら
  (if _bsuccess
    ;[1 1 1] 衝突した車が信号機に触れていなかったら
    (if (== (`/Game/Play/Common/GroundObject/Car/BP_CarBase.HitTraficLight` _asbp_car_base) (`/Game/Play/Common/GroundObject/Car/BP_CarBase.Reset` _asbp_car_base))
      (`self.Coercion` (`self.Box1`)))))

(event `self.Box.OnComponentBeginOverlap`
  (params (OverlappedComponent :type "PrimitiveComponent Object Reference") (OtherActor :type "Actor Object Reference") (OtherComp :type "PrimitiveComponent Object Reference") (OtherBodyIndex :type Integer) (bFromSweep :type Boolean) (SweepResult :type "HitResult Structure (by ref)"))
  (bind (_asbp_car_base _bsuccess) (cast `/Game/Play/Common/GroundObject/Car/BP_CarBase` OtherActor :!pure true))
  ;[1 1 1] 衝突したものが車だったら
  (if _bsuccess
    ;[1 1 1] 衝突した車が信号機に触れていなかったら
    (if (== (`/Game/Play/Common/GroundObject/Car/BP_CarBase.HitTraficLight` _asbp_car_base) (`/Game/Play/Common/GroundObject/Car/BP_CarBase.Reset` _asbp_car_base))
      (`self.Coercion` (`self.Box`)))))

(event `self.Box1.OnComponentBeginOverlap`
  (params (OverlappedComponent :type "PrimitiveComponent Object Reference") (OtherActor :type "Actor Object Reference") (OtherComp :type "PrimitiveComponent Object Reference") (OtherBodyIndex :type Integer) (bFromSweep :type Boolean) (SweepResult :type "HitResult Structure (by ref)"))
  (bind (_asbp_car_base _bsuccess) (cast `/Game/Play/Common/GroundObject/Car/BP_CarBase` OtherActor :!pure true))
  ;[1 1 1] 衝突したものが車だったら
  (if _bsuccess
    ;[1 1 1] 衝突した車が信号機に触れていなかったら
    (if (== (`/Game/Play/Common/GroundObject/Car/BP_CarBase.HitTraficLight` _asbp_car_base) (`/Game/Play/Common/GroundObject/Car/BP_CarBase.Reset` _asbp_car_base))
      (`self.Coercion` (`self.Box1`)))))

(fn `Coercion`
  (params (HitCollider :type "SceneComponent Object Reference"))
  (bind (_returnvalue_x _returnvalue_y _returnvalue_z) (`KismetMathLibrary.BreakVector` (`self.K2_GetActorLocation`)))
  (bind (_returnvalue_x_2 _returnvalue_y_2) (`KismetMathLibrary.BreakVector` (`SceneComponent.K2_GetComponentLocation` HitCollider)))
  (bind (_returnvalue_x_3 _returnvalue_y_3 _returnvalue_z_2) (`KismetMathLibrary.BreakVector` (`self.K2_GetActorLocation`)))
  (bind _returnvalue_x_4 (`KismetMathLibrary.BreakVector` (`SceneComponent.K2_GetComponentLocation` HitCollider)))
  (if (`self.INST_NorthSouthFlag`)
    (`self.K2_SetActorLocation` (`KismetMathLibrary.MakeVector` _returnvalue_x_4 _returnvalue_y_3 _returnvalue_z_2) false true)
    (else
      (`self.K2_SetActorLocation` (`KismetMathLibrary.MakeVector` _returnvalue_x _returnvalue_y_2 _returnvalue_z) false true))))

(fn `UserConstructionScript`)