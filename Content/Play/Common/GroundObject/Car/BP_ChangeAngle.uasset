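; BP_ChangeAngle is a car ground object that turns cars when they overlap it.
; On overlap, it casts the other actor to BP_CarBase and acts only if that car's direction matches INSTBeforeDirection.
; It then sets the car's direction to INSTAfterDirection and snaps its rotation to the matching entry in MSpawnAngle's AngleToRotation map.
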(event `self.ReceiveActorBeginOverlap`
  (params (OtherActor :type "Actor Object Reference"))
  (bind (_asbp_car_base _bsuccess) (cast `/Game/Play/Common/GroundObject/Car/BP_CarBase` OtherActor :!pure true))
  (bind _inst_afterdirection (`self.INST_AfterDirection`))
  (bind _mspawnangle_angletorotation (break `/Game/Play/Common/GroundObject/WarpPoint/SpawnAngle` (`self.mSpawnAngle`)))
  (if _bsuccess
    (if (`|EnumEquality` (`/Game/Play/Common/GroundObject/Car/BP_CarBase.mCarDirection` _asbp_car_base) (`self.INST_BeforeDirection`))
      ;[1 1 1] 車の進む方向を変える
      (`/Game/Play/Common/GroundObject/Car/BP_CarBase.SetCarDirection` _asbp_car_base _inst_afterdirection)
      (`self.K2_SetActorRotation` _asbp_car_base (`BlueprintMapLibrary.Map_Find` _mspawnangle_angletorotation _inst_afterdirection) false))))

(fn `UserConstructionScript`)