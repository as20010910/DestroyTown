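; BP_CarCreateManager spawns a limited number of cars for the DestructionCity game mode.
; A looping timer at the game mode's DELTATIME ticks a child BP_Timer, which gates each spawn to a half-second interval.
; Each spawn picks a random car class, sets its velocity and sequential number, then passes it to the warp manager's overlap handler.
; Spawning stops once the remaining count runs out.
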(event `self.ReceiveBeginPlay`
  (`/Game/Play/Common/GroundObject/BP_Timer.fSetMaxTime` (cast `/Game/Play/Common/GroundObject/BP_Timer` (`ChildActorComponent.ChildActor` (`self.BP_Timer`)) :!pure true) 0.5) ; 車の生成間隔を設定
  (`KismetSystemLibrary.K2_SetTimerDelegate` (delegate `CarCreate`) (`/Game/Play/Common/GameMode/GM_DestructionCity.DELTA_TIME` (cast `/Game/Play/Common/GameMode/GM_DestructionCity` (`GameplayStatics.GetGameMode`) :!pure true)) true))

(event `CarCreate`
  (if (`self.CarCreateFlag`)
    (`self.fCarCreate` (`/Game/Play/Common/GameMode/GM_DestructionCity.DELTA_TIME` (cast `/Game/Play/Common/GameMode/GM_DestructionCity` (`GameplayStatics.GetGameMode`) :!pure true)) (`self.mCarMoveVel`)) ; 車生成処理
  ))

(fn `fCarCreate`
  (params (tick :type "Float (double-precision)") (vel :type "Float (double-precision)"))
  (locals (moveVel :type "Float (double-precision)"))
  (set `local.moveVel` vel) ; 保存
  (if (> (`self.mCarCreateNum`) 0)
    (bind _newparam (`/Game/Play/Common/GroundObject/BP_Timer.fCountUp` (cast `/Game/Play/Common/GroundObject/BP_Timer` (`ChildActorComponent.ChildActor` (`self.BP_Timer`)) :!pure true) tick))
    (if _newparam
      (bind _returnvalue (`|SpawnActorFromClass` (`|GetArrayItem` (`self.mCarType`) (`KismetMathLibrary.RandomInteger` (`KismetArrayLibrary.Array_Length` (`self.mCarType`)))) (`self.mInstantVector3`) "AlwaysSpawn" "OverrideRootScale" null null))
      (bind _asbp_car_base (cast `/Game/Play/Common/GroundObject/Car/BP_CarBase` _returnvalue :!pure true))
      (`/Game/Play/Common/GroundObject/Car/BP_CarBase.fSetMoveVel` _asbp_car_base (`local.moveVel`)) ; 移動速度を設定
      (bind _output_get (set `/Game/Play/Common/GroundObject/Car/BP_CarBase.mCarNumber` (`self.mCarModelNumber`) _asbp_car_base))
      (bind _result (`/Engine/EditorBlueprintResources/StandardMacros.IncrementInt` _output_get)
        (:`  `
          (set `self.mCarModelNumber` _result)
          (`/Game/Play/Common/GroundObject/WarpPoint/BP_WarpManager.WarpPointBeginOverlap` (`self.mWarpManager`) null _returnvalue)
          (bind _result_2 (`/Engine/EditorBlueprintResources/StandardMacros.DecrementInt` (`self.mCarCreateNum`))
            (:`  `
              (set `self.mCarCreateNum` _result_2))))))
    (else
      (set `self.CarCreateFlag` false))))

(fn `fSetCarMoveVel`
  (params (CarMoveVel :type "Float (double-precision)"))
  (set `self.mCarMoveVel` CarMoveVel))

(fn `SetWarpManager`
  (params (mWarpManager :type "/Game/Play/Common/GroundObject/WarpPoint/BP_WarpManager Object Reference"))
  (set `self.mWarpManager` mWarpManager))

(fn `UserConstructionScript`)