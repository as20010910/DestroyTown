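; Base traffic car for the building scene, driving along cardinal directions on a looping timer with a positioned engine sound.
; A front collider queues it behind other cars, and tagged traffic-light boxes make it check signals, stop on red or yellow and pick random turns.
; Lookup maps resolve each turn's rotation and new heading.
; A second timer destroys cars stationary too long and requests a replacement, halting when the scene finishes.
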(event `self.ReceiveBeginPlay`
  (bind _asgm_destruction_city (cast `/Game/Play/Common/GameMode/GM_DestructionCity` (`GameplayStatics.GetGameMode`) :!pure true))
  (bind _mbp_buildingsoundmanager (`/Game/Play/Building/BP_BuildingManager.mBP_BuildingSoundManager` (`/Game/Play/Common/GameMode/GM_DestructionCity.mBP_BuildingManager` _asgm_destruction_city)))
  (`/Engine/EditorBlueprintResources/StandardMacros.IsValid` _mbp_buildingsoundmanager
    (:`Is Valid`
      (bind _index (`/Game/Play/Building/Sound/BP_BuildingSoundManager.fCreateSound` _mbp_buildingsoundmanager "NewEnumerator5" (`self.K2_GetActorLocation`))) ; 走行音作成
      (set `self.mSoundNumber` _index) ; 管理番号を保存
    )
    (:`Is Not Valid`
      _))
  (`KismetSystemLibrary.K2_SetTimerDelegate` (delegate `CarUpdate`) (`/Game/Play/Common/GameMode/GM_DestructionCity.DELTA_TIME` _asgm_destruction_city) true) ; 更新処理
  (bind _returnvalue (`|SpawnActorFromClass` "/Game/Play/Common/GroundObject/BP_Timer.BP_Timer_C" (`self.GetTransform`) "Undefined" "OverrideRootScale" null null))
  (bind _output_get (set `self.mBP_StopTimer` _returnvalue))
  (`/Game/Play/Common/GroundObject/BP_Timer.fSetMaxTime` _output_get (`self.DELETE_TIME`))
  (bind _returnvalue_2 (`KismetSystemLibrary.K2_SetTimerDelegate` (delegate `StopTimer`) (`/Game/Play/Common/GameMode/GM_DestructionCity.DELTA_TIME` (cast `/Game/Play/Common/GameMode/GM_DestructionCity` (`GameplayStatics.GetGameMode`) :!pure true)) true)) ; タイマー更新処理
)

(event `StopTimer`
  (bind _mbp_stoptimer (`self.mBP_StopTimer`))
  (bind _asgm_destruction_city (cast `/Game/Play/Common/GameMode/GM_DestructionCity` (`GameplayStatics.GetGameMode`) :!pure true))
  (if (`/Game/Play/Building/BP_BuildingManager.mFinish` (`/Game/Play/Common/GameMode/GM_DestructionCity.mBP_BuildingManager` _asgm_destruction_city))
    (`KismetSystemLibrary.K2_ClearAndInvalidateTimerHandle` (stale `self.ReceiveBeginPlay` _returnvalue_2)) ; イベント停止
    (`self.StopCar`)
    (set `self.MOVE_VEL` 0.0)
    (else
      (bind _flag (`self.fChackMove`)) ; 動いているか確認
      (if _flag
        (`/Game/Play/Common/GroundObject/BP_Timer.fReset` _mbp_stoptimer) ; 動いたらリセット
        (else
          (bind _newparam (`/Game/Play/Common/GroundObject/BP_Timer.fCountUp` _mbp_stoptimer (`/Game/Play/Common/GameMode/GM_DestructionCity.DELTA_TIME` _asgm_destruction_city))) ; 時間更新
          (if _newparam
            (`self.fCreateCar`) ; 車生成
            (`self.K2_DestroyActor`) ; 自分自身を破棄
          ))))))

(event `CarUpdate`
  ;[1 1 1] 更新処理
  (`self.MoveCar`) ; 車の移動処理
)

(event `self.CarFrontCollider.OnComponentBeginOverlap`
  (params (OverlappedComponent :type "PrimitiveComponent Object Reference") (OtherActor :type "Actor Object Reference") (OtherComp :type "PrimitiveComponent Object Reference") (OtherBodyIndex :type Integer) (bFromSweep :type Boolean) (SweepResult :type "HitResult Structure (by ref)"))
  (bind (_asbp_car_base _bsuccess) (cast `/Game/Play/Common/GroundObject/Car/BP_CarBase` OtherActor :!pure true))
  ;[1 1 1] 車前の衝突判定
  (if _bsuccess
    (if (!= (`/Game/Play/Common/GroundObject/Car/BP_CarBase.mCarNumber` _asbp_car_base) (`self.mCarNumber`))
      (if (== (`/Game/Play/Common/GroundObject/Car/BP_CarBase.CarMesh` _asbp_car_base) OtherComp)
        (`self.StopCar`)))))

(event `self.CarGaze.OnComponentBeginOverlap`
  (params (OverlappedComponent :type "PrimitiveComponent Object Reference") (OtherActor :type "Actor Object Reference") (OtherComp :type "PrimitiveComponent Object Reference") (OtherBodyIndex :type Integer) (bFromSweep :type Boolean) (SweepResult :type "HitResult Structure (by ref)"))
  (bind (_asbp_trafic_light _bsuccess) (cast `/Game/Play/Common/GroundObject/Intersection/TraficLight/BP_TraficLight` OtherActor :!pure true))
  ;[1 1 1] 当たったものが信号機か識別
  (if _bsuccess
    ;[1 1 1] 信号機用判定処理
    (`self.Trafic Light Update` _asbp_trafic_light OtherComp)))

(event `self.CarFrontCollider.OnComponentEndOverlap`
  (params (OverlappedComponent :type "PrimitiveComponent Object Reference") (OtherActor :type "Actor Object Reference") (OtherComp :type "PrimitiveComponent Object Reference") (OtherBodyIndex :type Integer))
  (bind (_asbp_car_base _bsuccess) (cast `/Game/Play/Common/GroundObject/Car/BP_CarBase` OtherActor :!pure true))
  ;[1 1 1] 車停止後、車発進処理
  (if _bsuccess
    (if (== (`/Game/Play/Common/GroundObject/Car/BP_CarBase.CarMesh` _asbp_car_base) OtherComp)
      (if (not (`self.ColorRedFlag`))
        (`KismetSystemLibrary.Delay` 0.5)
        (`self.MoveStartCar`)))))

(event `MoveCar`
  ;[1 1 1] 移動処理
  (`self.DEBUG_Move`)
  (if (`self.ColorRedFlag`)
    (`self.ChangeLightUpdate`)))

(fn `CarUpdate_ColorRed`
  (if (`self.ColorRedFlag`)
    ;[1 1 1] 0以下なら0に合わせる
    (bind _output_get (set `self.mMoveVel` (- (`self.mMoveVel`) (`self.mDeceleration`))))
    (if (< _output_get 0.0)
      (set `self.mMoveVel` 0.0)
      (return)
      (else
        (return)))
    (else
      (return))))

(fn `Chack Trafic Light`
  (bind _mtraficlightcolor (`/Game/Play/Common/GroundObject/Intersection/TraficLight/BP_TraficLight.GetLightColor` (`self.HitTraficLight`)))
  (switch `/Game/Play/Common/GroundObject/Intersection/TraficLight/TraficLightColor` _mtraficlightcolor
    (:`NewEnumerator0`
      _)
    (:`NewEnumerator1`
      _))
  ;[1 1 1] 信号を赤にして減速処理を追加する
  (set `self.ColorRedFlag` true))

(fn `ChangeLightUpdate`
  (bind _mtraficlightcolor (`/Game/Play/Common/GroundObject/Intersection/TraficLight/BP_TraficLight.GetLightColor` (`self.HitTraficLight`)))
  (switch `/Game/Play/Common/GroundObject/Intersection/TraficLight/TraficLightColor` _mtraficlightcolor
    (:`NewEnumerator0`
      ;[1 1 1] まだ信号が赤なら何もしない
      (return))
    (:`NewEnumerator2`
      (`self.MoveStartCar`))))

(fn `DEBUG_Move`
  (bind (_returnvalue_x _returnvalue_y _returnvalue_z) (`KismetMathLibrary.BreakVector` (`self.K2_GetActorLocation`)))
  (bind (_returnvalue_x_2 _returnvalue_y_2 _returnvalue_z_2) (`KismetMathLibrary.BreakVector` (`self.K2_GetActorLocation`)))
  (bind (_returnvalue_x_3 _returnvalue_y_3 _returnvalue_z_3) (`KismetMathLibrary.BreakVector` (`self.K2_GetActorLocation`)))
  (bind _returnvalue_x_4 (`KismetMathLibrary.BreakVector` (`self.K2_GetActorLocation`)))
  (bind (_returnvalue_x_5 _returnvalue_y_4) (`KismetMathLibrary.BreakVector` (`self.K2_GetActorLocation`)))
  (bind (_returnvalue_x_6 _returnvalue_y_5 _returnvalue_z_4) (`KismetMathLibrary.BreakVector` (`self.K2_GetActorLocation`)))
  (bind (_returnvalue_x_7 _returnvalue_y_6 _returnvalue_z_5) (`KismetMathLibrary.BreakVector` (`self.K2_GetActorLocation`)))
  (bind _shift_vel (`self.SHIFT_VEL`))
  (bind _shift_vel_2 (`self.SHIFT_VEL`))
  (bind _returnvalue_x_8 (`KismetMathLibrary.BreakVector` (`SceneComponent.K2_GetComponentLocation` (`self.mRideOnBox`))))
  (bind (_returnvalue_x_9 _returnvalue_y_7) (`KismetMathLibrary.BreakVector` (`SceneComponent.K2_GetComponentLocation` (`self.mRideOnBox`))))
  (bind _mbp_buildingsoundmanager (`/Game/Play/Building/BP_BuildingManager.mBP_BuildingSoundManager` (`/Game/Play/Common/GameMode/GM_DestructionCity.mBP_BuildingManager` (cast `/Game/Play/Common/GameMode/GM_DestructionCity` (`GameplayStatics.GetGameMode`) :!pure true))))
  (set `self.mMoveDistance` (0.0 0.0 0.0))
  (switch `/Game/Play/Common/GroundObject/Intersection/TraficLight/TraficLightDirection` (`self.mCarDirection`)
    (:`NewEnumerator0`
      ;[1 1 1] 仮の移動処理
      (`self.K2_SetActorLocation` (`KismetMathLibrary.MakeVector` (+ _returnvalue_x_2 (`self.mMoveVel`)) _returnvalue_y_2 _returnvalue_z_2) false true)
      ;;[1 1 1] 移動量保存
      (set `self.mMoveDistance` (`KismetMathLibrary.MakeVector` (`self.mMoveVel`))))
    (:`NewEnumerator1`
      (`self.K2_SetActorLocation` (`KismetMathLibrary.MakeVector` (- _returnvalue_x (`self.mMoveVel`)) _returnvalue_y _returnvalue_z) false true)
      (set `self.mMoveDistance` (`KismetMathLibrary.MakeVector` (* -1 (`self.mMoveVel`)))))
    (:`NewEnumerator2`
      (`self.K2_SetActorLocation` (`KismetMathLibrary.MakeVector` _returnvalue_x_3 (- _returnvalue_y_3 (`self.mMoveVel`)) _returnvalue_z_3) false true)
      (set `self.mMoveDistance` (`KismetMathLibrary.MakeVector` 0.0 (* -1 (`self.mMoveVel`)))))
    (:`NewEnumerator3`
      (`self.K2_SetActorLocation` (`KismetMathLibrary.MakeVector` _returnvalue_x_6 (+ _returnvalue_y_5 (`self.mMoveVel`)) _returnvalue_z_4) false true)
      (set `self.mMoveDistance` (`KismetMathLibrary.MakeVector` 0.0 (`self.mMoveVel`)))))
  ;[1 1 1] 動いているのに再生されていなかったら
  (`/Engine/EditorBlueprintResources/StandardMacros.IsValid` _mbp_buildingsoundmanager
    (:`Is Valid`
      (bind _soundvalue (`/Game/Play/Building/Sound/BP_BuildingSoundManager.fGetSoundArray` _mbp_buildingsoundmanager "NewEnumerator5" (`self.mSoundNumber`)))
      (if (and (`|EnumEquality` (`AudioComponent.GetPlayState` _soundvalue) "Paused") (`KismetMathLibrary.NotEqualExactly_VectorVector` (`KismetMathLibrary.Vector_GetAbs` (`self.mMoveDistance`))))
        (`AudioComponent.SetPaused` _soundvalue false) ; 一時停止解除
      )
      (`/Game/Play/Building/Sound/BP_BuildingSoundManager.fMoveSound` _mbp_buildingsoundmanager "NewEnumerator5" (`self.mSoundNumber`) (`self.K2_GetActorLocation`)) ; 音発生位置を移動させる
    )
    (:`Is Not Valid`
      _))
  (`/Engine/EditorBlueprintResources/StandardMacros.IsValid` (`self.mRideOnBox`)
    (:`Is Valid`
      ;[1 1 1] 位置補正処理
      (switch `/Game/Play/Stage/EN_Angle` (`self.mRideOnRode`) ; 道の向きによって処理を変える
        (:`NewEnumerator0`
          (if (< _returnvalue_y_7 _returnvalue_y_4)
            (`self.K2_SetActorLocation` (`KismetMathLibrary.MakeVector` _returnvalue_x_7 (+ _returnvalue_y_6 _shift_vel_2) _returnvalue_z_5) false true)
            (set `self.mMoveDistance` (+ (`self.mMoveDistance`) (`KismetMathLibrary.MakeVector` 0.0 _shift_vel_2)))
            (else
              (set `self.mRideOnBox` null)
              (set `self.mRideOnRode` "NewEnumerator2"))))
        (:`NewEnumerator1`
          (if (< _returnvalue_x_4 _returnvalue_x_8)
            (`self.K2_SetActorLocation` (`KismetMathLibrary.MakeVector` (+ _returnvalue_x_7 _shift_vel) _returnvalue_y_6 _returnvalue_z_5) false true)
            (set `self.mMoveDistance` (+ (`self.mMoveDistance`) (`KismetMathLibrary.MakeVector` _shift_vel)))
            (else
              (set `self.mRideOnBox` null)
              (set `self.mRideOnRode` "NewEnumerator2"))))))))

(fn `Direction Left`
  (returns (`Left orStraightFlag` :type Boolean))
  (locals (intersectionAngleAfterDirectionMap :type "/Game/Play/Common/GroundObject/Intersection/TraficLight/AfterAngle/IntersectionAngleAfterDirectionMap Structure"))
  (bind (_returnvalue_roll _returnvalue_pitch _returnvalue_yaw) (`KismetMathLibrary.BreakRotator` (`self.K2_GetActorRotation`)))
  (bind _mintersectionflagmap_direction (break `/Game/Play/Common/GroundObject/Intersection/TraficLight/DirectionAngle/IntersectionAngleDirectionMap` (`self.mIntersectionFlagMap`)))
  (bind _intersectionangleafterdirectionmap_direction (break `/Game/Play/Common/GroundObject/Intersection/TraficLight/AfterAngle/IntersectionAngleAfterDirectionMap` (`local.intersectionAngleAfterDirectionMap`)))
  ;[1 1 1] 左曲がりか確認
  (switch `/Game/Play/Common/GroundObject/Car/IntersectionAngle` (`self.mTurnAngle`)
    (:`NewEnumerator0`
      ;[1 1 1] 直進して終了した
      (return true))
    (:`NewEnumerator1`
      ;[1 1 1] 曲がらずに終了した
      (return false))
    (:`NewEnumerator2`
      ;[1 1 1] 信号機の方向を取得
      (bind _mtraficlightangle (`/Game/Play/Common/GroundObject/Intersection/TraficLight/BP_TraficLight.GetTraficLightAngle` (`self.HitTraficLight`)))
      (bind _value (`BlueprintMapLibrary.Map_Find` (break `/Game/Play/Common/GroundObject/Intersection/TraficLight/DirectionAngle/IntersectionAngleMap` (`BlueprintMapLibrary.Map_Find` _mintersectionflagmap_direction _mtraficlightangle)) (`self.mTurnAngle`)))
      ;[1 1 1] 車を回転
      (`self.K2_SetActorRotation` (`KismetMathLibrary.MakeRotator` (+ (.roll _value) _returnvalue_roll) (+ (.pitch _value) _returnvalue_pitch) (+ (.yaw _value) _returnvalue_yaw)))
      ;[1 1 1] 現在向いている方向と、曲がる方向から進む方向を求める
      (set `self.mCarDirection` (`BlueprintMapLibrary.Map_Find` (break `/Game/Play/Common/GroundObject/Intersection/TraficLight/AfterAngle/IntersectionAfterAngleMap` (`BlueprintMapLibrary.Map_Find` _intersectionangleafterdirectionmap_direction (`self.mCarDirection`))) (`self.mTurnAngle`)))
      ;[1 1 1] 曲がって終了した
      (return true))))

(fn `DirectionRight`
  (returns (RightFlag :type Boolean))
  (locals (intersectionAngleAfterDirectionMap :type "/Game/Play/Common/GroundObject/Intersection/TraficLight/AfterAngle/IntersectionAngleAfterDirectionMap Structure" :default (struct :`direction` (struct :`(NewEnumerator3, (Angle` "((NewEnumerator0, NewEnumerator3),(NewEnumerator1, NewEnumerator1),(NewEnumerator2, NewEnumerator0))))" :`(NewEnumerator2, (Angle` "((NewEnumerator0, NewEnumerator2),(NewEnumerator1, NewEnumerator0),(NewEnumerator2, NewEnumerator1))))" :`(NewEnumerator1, (Angle` "((NewEnumerator0, NewEnumerator1),(NewEnumerator1, NewEnumerator2),(NewEnumerator2, NewEnumerator3))))" :`(NewEnumerator0, (Angle` "((NewEnumerator0, NewEnumerator0),(NewEnumerator1, NewEnumerator3),(NewEnumerator2, NewEnumerator2))))"))))
  (bind (_returnvalue_roll _returnvalue_pitch _returnvalue_yaw) (`KismetMathLibrary.BreakRotator` (`self.K2_GetActorRotation`)))
  (bind _intersectionangleafterdirectionmap_direction (break `/Game/Play/Common/GroundObject/Intersection/TraficLight/AfterAngle/IntersectionAngleAfterDirectionMap` (`local.intersectionAngleAfterDirectionMap`)))
  (bind _mintersectionflagmap_direction (break `/Game/Play/Common/GroundObject/Intersection/TraficLight/DirectionAngle/IntersectionAngleDirectionMap` (`self.mIntersectionFlagMap`)))
  ;[1 1 1] 左曲がりか確認
  (switch `/Game/Play/Common/GroundObject/Car/IntersectionAngle` (`self.mTurnAngle`)
    (:`NewEnumerator0`
      ;[1 1 1] 直進して終了した
      (return true))
    (:`NewEnumerator1`
      ;[1 1 1] 信号機の方向を取得
      (bind _mtraficlightangle (`/Game/Play/Common/GroundObject/Intersection/TraficLight/BP_TraficLight.GetTraficLightAngle` (`self.HitTraficLight`)))
      (bind _value (`BlueprintMapLibrary.Map_Find` (break `/Game/Play/Common/GroundObject/Intersection/TraficLight/DirectionAngle/IntersectionAngleMap` (`BlueprintMapLibrary.Map_Find` _mintersectionflagmap_direction _mtraficlightangle)) (`self.mTurnAngle`)))
      ;[1 1 1] 車を回転
      (`self.K2_SetActorRotation` (`KismetMathLibrary.MakeRotator` (+ (.roll _value) _returnvalue_roll) (+ (.pitch _value) _returnvalue_pitch) (+ (.yaw _value) _returnvalue_yaw)))
      (set `self.mCarDirection` (`BlueprintMapLibrary.Map_Find` (break `/Game/Play/Common/GroundObject/Intersection/TraficLight/AfterAngle/IntersectionAfterAngleMap` (`BlueprintMapLibrary.Map_Find` _intersectionangleafterdirectionmap_direction (`self.mCarDirection`))) (`self.mTurnAngle`)))
      ;[1 1 1] 右曲がり
      (return true))
    (:`NewEnumerator2`
      ;[1 1 1] 曲がらずに終了した
      (return false))))

(fn `fChackMove`
  (returns (flag :type Boolean))
  (if (== (`self.mBeforePosition`) (`self.K2_GetActorLocation`))
    (return false) ; 動いてなかったらFALSE
    (else
      (set `self.mBeforePosition` (`self.K2_GetActorLocation`)) ; 更新
      (return true) ; 動いていたらTRUE
    )))

(fn `fCreateCar`
  (bind _mbp_carcreatemanager (`/Game/Play/Building/BP_BuildingManager.mBP_CarCreateManager` (`/Game/Play/Common/GameMode/GM_DestructionCity.mBP_BuildingManager` (cast `/Game/Play/Common/GameMode/GM_DestructionCity` (`GameplayStatics.GetGameMode`) :!pure true))))
  (bind _result (`/Engine/EditorBlueprintResources/StandardMacros.IncrementInt` (`/Game/Play/Common/GroundObject/Car/BP_CarCreateManager.mCarCreateNum` _mbp_carcreatemanager))
    (:`  `
      (set `/Game/Play/Common/GroundObject/Car/BP_CarCreateManager.mCarCreateNum` _result _mbp_carcreatemanager)
      (set `/Game/Play/Common/GroundObject/Car/BP_CarCreateManager.CarCreateFlag` true _mbp_carcreatemanager))))

(fn `fSetMoveVel`
  (params (mMoveVel :type "Float (double-precision)"))
  (bind _output_get (set `self.mMoveVel` mMoveVel))
  (set `self.MOVE_VEL` _output_get))

(fn `MoveStartCar`
  (locals (ResetTraficLight :type "Object Object Reference"))
  (set `self.mMoveVel` (`self.MOVE_VEL`)))

(fn `Reset Trafic Light`
  (locals (resetLight :type "/Game/Play/Common/GroundObject/Intersection/TraficLight/BP_TraficLight Object Reference"))
  ;[1 1 1] 信号機情報
  (set `self.HitTraficLight` (`local.resetLight`))
  ;[1 1 1] 信号機の色
  (set `self.mTraficLightColor` 0)
  ;[1 1 1] 赤信号フラグ
  (set `self.ColorRedFlag` false)
  (set `self.mTurnAngle` "NewEnumerator0"))

(fn `SetCarDirection`
  (params (mCarDirection :type "/Game/Play/Common/GroundObject/Intersection/TraficLight/TraficLightDirection Enum" :default "NewEnumerator0"))
  (set `self.mCarDirection` mCarDirection))

(fn `Setting Turns Direction`
  (bind _hittraficlight (`self.HitTraficLight`))
  (switch `int` (`KismetMathLibrary.RandomInteger` 3) :!label _label
    (:`0`
      (set `self.mTurnAngle` "NewEnumerator0")
      ;[1 1 1] 道がない場合は別の道に
      (bind _mintersectionflag (`/Game/Play/Common/GroundObject/Intersection/TraficLight/BP_TraficLight.GetIntersectionAngle` _hittraficlight))
      (if (== (break `/Game/Play/Common/GroundObject/Intersection/TraficLight/IntersectionAngle` _mintersectionflag) false)
        (switch `int` (`KismetMathLibrary.RandomInteger` 2)
          (:`0`
            (set `self.mTurnAngle` "NewEnumerator1"))
          (:`1`
            (set `self.mTurnAngle` "NewEnumerator2")))))
    (:`1`
      (set `self.mTurnAngle` "NewEnumerator1")
      (bind _mintersectionflag_2 (`/Game/Play/Common/GroundObject/Intersection/TraficLight/BP_TraficLight.GetIntersectionAngle` _hittraficlight))
      (if (== (`.TurnRight_5_4FE532C64F8B2535A7665A9FBBF16290` (break `/Game/Play/Common/GroundObject/Intersection/TraficLight/IntersectionAngle` _mintersectionflag_2)) false)
        (goto _label)))
    (:`2`
      (set `self.mTurnAngle` "NewEnumerator2")
      (bind _mintersectionflag_3 (`/Game/Play/Common/GroundObject/Intersection/TraficLight/BP_TraficLight.GetIntersectionAngle` _hittraficlight))
      (if (== (`.TurnLeft_6_BD0921CD481D839BD9E1F6AA7822B81D` (break `/Game/Play/Common/GroundObject/Intersection/TraficLight/IntersectionAngle` _mintersectionflag_3)) false)
        (goto _label)))))

(fn `StopCar`
  (bind _mbp_buildingsoundmanager (`/Game/Play/Building/BP_BuildingManager.mBP_BuildingSoundManager` (`/Game/Play/Common/GameMode/GM_DestructionCity.mBP_BuildingManager` (cast `/Game/Play/Common/GameMode/GM_DestructionCity` (`GameplayStatics.GetGameMode`) :!pure true))))
  (set `self.mMoveVel` 0.0) ; 速度を０にする
  (`/Engine/EditorBlueprintResources/StandardMacros.IsValid` _mbp_buildingsoundmanager
    (:`Is Valid`
      (bind _soundvalue (`/Game/Play/Building/Sound/BP_BuildingSoundManager.fGetSoundArray` _mbp_buildingsoundmanager "NewEnumerator5" (`self.mSoundNumber`)))
      (`AudioComponent.SetPaused` _soundvalue true))))

(fn `Trafic Light Update`
  (params (InputPin :type "/Game/Play/Common/GroundObject/Intersection/TraficLight/BP_TraficLight Object Reference") (`ターゲット` :type "ActorComponent Object Reference"))
  (locals (saveTraficLight :type "/Game/Play/Common/GroundObject/Intersection/TraficLight/BP_TraficLight Object Reference") (resetTraficLight :type "/Game/Play/Common/GroundObject/Intersection/TraficLight/BP_TraficLight Object Reference"))
  (set `local.saveTraficLight` InputPin)
  (if (and (`ActorComponent.ComponentHasTag` `ターゲット` "StopBox") (== (`local.saveTraficLight`) (`self.HitTraficLight`)))
    ;[1 1 1] 赤の場合車停止処理
    (if (`self.ColorRedFlag`)
      (`self.StopCar`))
    (elif (and (`ActorComponent.ComponentHasTag` `ターゲット` "ChackTraficLightColorBox") (== (`local.saveTraficLight`) (`self.HitTraficLight`)))
      ;[1 1 1] 信号の色を取得し動作を決める処理
      (`self.Chack Trafic Light`)
      (elif (and (`ActorComponent.ComponentHasTag` `ターゲット` "SettingTurnsDirectionBox") (== (`local.saveTraficLight`) (`self.HitTraficLight`)))
        ;[1 1 1] 進む方向を決める処理
        (`self.Setting Turns Direction`)
        (elif (and (`ActorComponent.ComponentHasTag` `ターゲット` "DiscoverTraficLight") (== (`self.HitTraficLight`) (`local.resetTraficLight`)))
          (set `self.HitTraficLight` (`local.saveTraficLight`))
          (elif (and (`ActorComponent.ComponentHasTag` `ターゲット` "DirectionLeftBox") (== (`local.saveTraficLight`) (`self.HitTraficLight`)))
            ;[1 1 1] 左曲がりの処理
            (bind _left_orstraightflag (`self.Direction Left`))
            ;[1 1 1] 最終処理のため、情報をリセットする
            (if _left_orstraightflag
              (`self.Reset Trafic Light`)
              (`self.MoveStartCar`))
            (elif (and (`ActorComponent.ComponentHasTag` `ターゲット` "DirectionRightBox") (== (`local.saveTraficLight`) (`self.HitTraficLight`)))
              ;[1 1 1] 右曲がりの処理
              (bind _rightflag (`self.DirectionRight`))
              (if _rightflag
                (`self.Reset Trafic Light`)
                (`self.MoveStartCar`)))))))))

(fn `UserConstructionScript`)