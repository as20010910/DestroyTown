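; Traffic light actor for intersections that shows red, yellow or green and exposes its color and angle values through getters.
; ChangeColor swaps materials on three lamp meshes, lighting one and giving the others a shared unlit material.
; ChangeTraficLightColor advances green, yellow, red, then back to green through ChangeColor.
; BeginPlay and Tick are empty; the interval-based auto-cycle, initial green setup and debug material bodies are disconnected.
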(event `self.ReceiveBeginPlay`)

(event `self.ReceiveTick`
  (params (DeltaSeconds :type "Float (single-precision)")))

(fn `ChangeColor`
  (params (Color :type "/Game/Play/Common/GroundObject/Intersection/TraficLight/TraficLightColor Enum" :default "NewEnumerator0"))
  (switch `/Game/Play/Common/GroundObject/Intersection/TraficLight/TraficLightColor` Color
    (:`NewEnumerator0`
      ;[1 1 1] 赤信号
      (`PrimitiveComponent.SetMaterial` (`self.GreenLight`) 0 "/Game/Play/Common/GroundObject/Intersection/TraficLight/Resouce/polySurface18Mat.polySurface18Mat")
      (`PrimitiveComponent.SetMaterial` (`self.YellowLight`) 0 "/Game/Play/Common/GroundObject/Intersection/TraficLight/Resouce/polySurface18Mat.polySurface18Mat")
      (`PrimitiveComponent.SetMaterial` (`self.RedLight`) 0 "/Game/Play/Common/GroundObject/Intersection/TraficLight/Resouce/Red.Red")
      (set `self.mTraficLightColor` "NewEnumerator0"))
    (:`NewEnumerator1`
      ;[1 1 1] 黄信号
      (`PrimitiveComponent.SetMaterial` (`self.GreenLight`) 0 "/Game/Play/Common/GroundObject/Intersection/TraficLight/Resouce/polySurface18Mat.polySurface18Mat")
      (`PrimitiveComponent.SetMaterial` (`self.YellowLight`) 0 "/Game/Play/Common/GroundObject/Intersection/TraficLight/Resouce/Yellow.Yellow")
      (`PrimitiveComponent.SetMaterial` (`self.RedLight`) 0 "/Game/Play/Common/GroundObject/Intersection/TraficLight/Resouce/polySurface18Mat.polySurface18Mat")
      (set `self.mTraficLightColor` "NewEnumerator1"))
    (:`NewEnumerator2`
      ;[1 1 1] 青信号
      (`PrimitiveComponent.SetMaterial` (`self.GreenLight`) 0 "/Game/Play/Common/GroundObject/Intersection/TraficLight/Resouce/Green.Green")
      (`PrimitiveComponent.SetMaterial` (`self.YellowLight`) 0 "/Game/Play/Common/GroundObject/Intersection/TraficLight/Resouce/polySurface18Mat.polySurface18Mat")
      (`PrimitiveComponent.SetMaterial` (`self.RedLight`) 0 "/Game/Play/Common/GroundObject/Intersection/TraficLight/Resouce/polySurface18Mat.polySurface18Mat")
      (set `self.mTraficLightColor` "NewEnumerator2"))))

(fn `ChangeTraficLightColor`
  (params (NewParam :type "/Game/Play/Common/GroundObject/Intersection/TraficLight/TraficLightColor Enum" :default "NewEnumerator3"))
  (switch `/Game/Play/Common/GroundObject/Intersection/TraficLight/TraficLightColor` NewParam
    (:`NewEnumerator0`
      (set `self.mTraficLightColor` "NewEnumerator2"))
    (:`NewEnumerator1`
      (set `self.mTraficLightColor` "NewEnumerator0"))
    (:`NewEnumerator2`
      (set `self.mTraficLightColor` "NewEnumerator1")))
  (`self.ChangeColor` (`self.mTraficLightColor`))
  ;[1 1 1] DEBUG色変え
  (switch `/Game/Play/Common/GroundObject/Intersection/TraficLight/TraficLightColor` (`self.mTraficLightColor`)
    (:`NewEnumerator0`
      (`self.DEBUG_ChangeTraficLightMaterialRed`))
    (:`NewEnumerator1`
      (`self.DEBUG_ChangeTraficLightMaterialYellow`))
    (:`NewEnumerator2`
      (`self.DEBUG_ChangeTraficLightMaterialBlue`))))

(fn `DEBUG_ChangeTraficLightMaterialBlue`)

(fn `DEBUG_ChangeTraficLightMaterialRed`)

(fn `DEBUG_ChangeTraficLightMaterialYellow`)

(fn `GetIntersectionAngle`
  (returns (mIntersectionFlag :type "/Game/Play/Common/GroundObject/Intersection/TraficLight/IntersectionAngle Structure"))
  (return (`self.mIntersectionFlag`)))

(fn `GetLightColor`
  (returns (mTraficLightColor :type "/Game/Play/Common/GroundObject/Intersection/TraficLight/TraficLightColor Enum"))
  (return (`self.mTraficLightColor`)))

(fn `GetTraficLightAngle`
  (returns (mTraficLightAngle :type "/Game/Play/Common/GroundObject/Intersection/TraficLight/TraficLightDirection Enum"))
  (return (`self.mTraficLightAngle`)))

(fn `UserConstructionScript`)