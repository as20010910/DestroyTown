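; T-intersection actor that cycles its child-actor traffic lights between the single north light and the west/east pair.
; It starts with north green, then Tick uses CountTime to alternate timed green and yellow phases, with MColorGreenFlag tracking the green axis.
; After yellow, that axis turns red and a fixed Delay precedes the other's green.
; Each color change calls ChangeColor on BP_TraficLight plus a debug material setter.
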(event `self.ReceiveBeginPlay`
  (`self.NorthSouthChangeBlue`)
  (`self.EastWestChangeRed`))

(event `self.ReceiveTick`
  (params (DeltaSeconds :type "Float (single-precision)"))
  (bind _bp_northtraficlight (`self.BP_NorthTraficLight`))
  (if (`self.mYellowFlag`)
    (bind _changeflag (`self.CountTime` DeltaSeconds (`self.YELLOW_INTERVAL`)))
    (if _changeflag
      (if (`|EnumEquality` (`self.mColorGreenFlag`) "NewEnumerator0")
        (`self.NorthSouthChangeRed`)
        (`KismetSystemLibrary.Delay` 3.0)
        (`self.EastWestChangeBlue`)
        (else
          (`self.EastWestChangeRed`)
          (`KismetSystemLibrary.Delay` 3.0)
          (`self.NorthSouthChangeBlue`)))
      (set `self.mYellowFlag` false))
    (else
      ;[1 1 1] どちらかが青の時の処理
      (bind _changeflag_2 (`self.CountTime` DeltaSeconds (`self.INTERVAL`)))
      (if _changeflag_2
        (if (`|EnumEquality` (`self.mColorGreenFlag`) "NewEnumerator0")
          (`self.ChangeYellow` _bp_northtraficlight _bp_northtraficlight)
          (else
            (`self.ChangeYellow` (`self.BP_WestTraficLight`) (`self.BP_EastTraficLight`))))
        (set `self.mYellowFlag` true)))))

(fn `ChangeYellow`
  (params (TraficLight1 :type "ChildActorComponent Object Reference") (TraficLight2 :type "ChildActorComponent Object Reference"))
  (locals (SaveTraficLight1 :type "ChildActorComponent Object Reference") (SaveTraficLight2 :type "ChildActorComponent Object Reference"))
  (set `local.SaveTraficLight1` TraficLight1)
  (set `local.SaveTraficLight2` TraficLight2)
  (`/Game/Play/Common/GroundObject/Intersection/TraficLight/BP_TraficLight.ChangeColor` (cast `/Game/Play/Common/GroundObject/Intersection/TraficLight/BP_TraficLight` (`ChildActorComponent.ChildActor` (`local.SaveTraficLight1`)) :!pure true) "NewEnumerator1")
  (`/Game/Play/Common/GroundObject/Intersection/TraficLight/BP_TraficLight.ChangeColor` (cast `/Game/Play/Common/GroundObject/Intersection/TraficLight/BP_TraficLight` (`ChildActorComponent.ChildActor` (`local.SaveTraficLight2`)) :!pure true) "NewEnumerator1")
  ;[1 1 1] DEBUG色変え処理
  (`/Game/Play/Common/GroundObject/Intersection/TraficLight/BP_TraficLight.DEBUG_ChangeTraficLightMaterialYellow` (cast `/Game/Play/Common/GroundObject/Intersection/TraficLight/BP_TraficLight` (`ChildActorComponent.ChildActor` (`local.SaveTraficLight1`)) :!pure true))
  (`/Game/Play/Common/GroundObject/Intersection/TraficLight/BP_TraficLight.DEBUG_ChangeTraficLightMaterialYellow` (cast `/Game/Play/Common/GroundObject/Intersection/TraficLight/BP_TraficLight` (`ChildActorComponent.ChildActor` (`local.SaveTraficLight2`)) :!pure true)))

(fn `CountTime`
  (params (tick :type "Float (double-precision)") (maxTime :type Integer))
  (returns (ChangeFlag :type Boolean))
  ;[1 1 1] 時間カウント処理
  (bind _output_get (set `self.mIntervalTimer` (+ tick (`self.mIntervalTimer`))))
  ;[1 1 1] 規定の時間になったら
  (if (>= _output_get (`KismetMathLibrary.Conv_IntToDouble` maxTime))
    (set `self.mIntervalTimer` 0.0)
    (return true)
    (else
      (return false))))

(fn `EastWestChangeBlue`
  (set `self.mColorGreenFlag` "NewEnumerator1")
  ;[1 1 1] 青にする
  (`/Game/Play/Common/GroundObject/Intersection/TraficLight/BP_TraficLight.ChangeColor` (cast `/Game/Play/Common/GroundObject/Intersection/TraficLight/BP_TraficLight` (`ChildActorComponent.ChildActor` (`self.BP_WestTraficLight`)) :!pure true) "NewEnumerator2")
  (`/Game/Play/Common/GroundObject/Intersection/TraficLight/BP_TraficLight.ChangeColor` (cast `/Game/Play/Common/GroundObject/Intersection/TraficLight/BP_TraficLight` (`ChildActorComponent.ChildActor` (`self.BP_EastTraficLight`)) :!pure true) "NewEnumerator2")
  ;[1 1 1] DEBUG_青にする
  (`/Game/Play/Common/GroundObject/Intersection/TraficLight/BP_TraficLight.DEBUG_ChangeTraficLightMaterialBlue` (cast `/Game/Play/Common/GroundObject/Intersection/TraficLight/BP_TraficLight` (`ChildActorComponent.ChildActor` (`self.BP_WestTraficLight`)) :!pure true))
  (`/Game/Play/Common/GroundObject/Intersection/TraficLight/BP_TraficLight.DEBUG_ChangeTraficLightMaterialBlue` (cast `/Game/Play/Common/GroundObject/Intersection/TraficLight/BP_TraficLight` (`ChildActorComponent.ChildActor` (`self.BP_EastTraficLight`)) :!pure true)))

(fn `EastWestChangeRed`
  ;[1 1 1] 赤にする
  (`/Game/Play/Common/GroundObject/Intersection/TraficLight/BP_TraficLight.ChangeColor` (cast `/Game/Play/Common/GroundObject/Intersection/TraficLight/BP_TraficLight` (`ChildActorComponent.ChildActor` (`self.BP_WestTraficLight`)) :!pure true) "NewEnumerator0")
  (`/Game/Play/Common/GroundObject/Intersection/TraficLight/BP_TraficLight.ChangeColor` (cast `/Game/Play/Common/GroundObject/Intersection/TraficLight/BP_TraficLight` (`ChildActorComponent.ChildActor` (`self.BP_EastTraficLight`)) :!pure true) "NewEnumerator0")
  ;[1 1 1] DEBUG_赤にする
  (`/Game/Play/Common/GroundObject/Intersection/TraficLight/BP_TraficLight.DEBUG_ChangeTraficLightMaterialRed` (cast `/Game/Play/Common/GroundObject/Intersection/TraficLight/BP_TraficLight` (`ChildActorComponent.ChildActor` (`self.BP_WestTraficLight`)) :!pure true))
  (`/Game/Play/Common/GroundObject/Intersection/TraficLight/BP_TraficLight.DEBUG_ChangeTraficLightMaterialRed` (cast `/Game/Play/Common/GroundObject/Intersection/TraficLight/BP_TraficLight` (`ChildActorComponent.ChildActor` (`self.BP_EastTraficLight`)) :!pure true)))

(fn `NorthSouthChangeBlue`
  (set `self.mColorGreenFlag` "NewEnumerator0")
  ;[1 1 1] 青にする
  (`/Game/Play/Common/GroundObject/Intersection/TraficLight/BP_TraficLight.ChangeColor` (cast `/Game/Play/Common/GroundObject/Intersection/TraficLight/BP_TraficLight` (`ChildActorComponent.ChildActor` (`self.BP_NorthTraficLight`)) :!pure true) "NewEnumerator2")
  ;[1 1 1] DEBUG_青にする
  (`/Game/Play/Common/GroundObject/Intersection/TraficLight/BP_TraficLight.DEBUG_ChangeTraficLightMaterialBlue` (cast `/Game/Play/Common/GroundObject/Intersection/TraficLight/BP_TraficLight` (`ChildActorComponent.ChildActor` (`self.BP_NorthTraficLight`)) :!pure true)))

(fn `NorthSouthChangeRed`
  ;[1 1 1] 赤にする
  (`/Game/Play/Common/GroundObject/Intersection/TraficLight/BP_TraficLight.ChangeColor` (cast `/Game/Play/Common/GroundObject/Intersection/TraficLight/BP_TraficLight` (`ChildActorComponent.ChildActor` (`self.BP_NorthTraficLight`)) :!pure true) "NewEnumerator0")
  ;[1 1 1] DEBUG_赤にする
  (`/Game/Play/Common/GroundObject/Intersection/TraficLight/BP_TraficLight.DEBUG_ChangeTraficLightMaterialRed` (cast `/Game/Play/Common/GroundObject/Intersection/TraficLight/BP_TraficLight` (`ChildActorComponent.ChildActor` (`self.BP_NorthTraficLight`)) :!pure true)))

(fn `OffFinishFlag`
  (params (NewParam :type "ChildActorComponent Object Reference"))
  (set `/Game/Play/Common/GroundObject/Intersection/TraficLight/BP_TraficLight.mFinishFlag` false (cast `/Game/Play/Common/GroundObject/Intersection/TraficLight/BP_TraficLight` (`ChildActorComponent.ChildActor` NewParam) :!pure true)))

(fn `UserConstructionScript`)