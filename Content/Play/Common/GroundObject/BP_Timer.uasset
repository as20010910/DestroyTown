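; BP_Timer is a simple reusable timer Blueprint that counts up toward a configurable maximum time.
; FCountUp adds the passed tick value to an internal count, then returns true and resets the count to zero once it exceeds the maximum.
; FSetMaxTime sets that limit.
; Its own event graph is empty, so the timer advances only when FCountUp is called externally.
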(fn `fCountUp`
  (params (tick :type "Float (double-precision)"))
  (returns (NewParam :type Boolean))
  (bind _output_get (set `self.mCount` (+ tick (`self.mCount`))))
  (if (> _output_get (`self.mMaxTime`))
    (set `self.mCount` 0.0)
    (return true)
    (else
      (return false))))

(fn `fSetMaxTime`
  (params (mMaxTime :type "Float (double-precision)"))
  (set `self.mMaxTime` mMaxTime))

(fn `UserConstructionScript`)