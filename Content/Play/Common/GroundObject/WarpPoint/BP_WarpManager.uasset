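; Manager actor that teleports cars entering warp points to a new warp point, re-aiming them to match.
; On BeginPlay it gathers every BP_WarpPoint and groups XY positions by direction.
; A looping timer binds their overlap events, which relocate any BP_CarBase and set its direction and rotation.
; Both random branches currently choose West, and X and Y come from separate random picks among that side's points.
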(event `self.ReceiveBeginPlay`
  (`KismetSystemLibrary.K2_SetTimerDelegate` (delegate `BindWarpPointBeginOverlap`) (`/Game/Play/Common/GameMode/GM_DestructionCity.DELTA_TIME` (cast `/Game/Play/Common/GameMode/GM_DestructionCity` (`GameplayStatics.GetGameMode`) :!pure true)) true) ; 接触イベントを設定しておく
  (`self.fSetAllWarpPoint`))

(event `BindWarpPointBeginOverlap`
  (add `self.OnActorBeginOverlap` (`self.mWarpPoint`) (delegate `WarpPointBeginOverlap`)))

(event `WarpPointBeginOverlap` :!signature `self.OnActorBeginOverlap`
  (params (OverlappedActor :type "Actor Object Reference") (OtherActor :type "Actor Object Reference"))
  (bind (_asbp_car_base _bsuccess) (cast `/Game/Play/Common/GroundObject/Car/BP_CarBase` OtherActor :!pure true))
  (if _bsuccess
    (bind (_output_get _spawndirection1) (`self.CreateDirection`))
    (`self.WarpCar` _output_get _asbp_car_base _spawndirection1)))

(fn `CreateDirection`
  (returns (Output_Get :type "Vector Structure") (spawnDirection1 :type "/Game/Play/Common/GroundObject/Intersection/TraficLight/TraficLightDirection Enum"))
  (locals (spawnDirection :type "/Game/Play/Common/GroundObject/Intersection/TraficLight/TraficLightDirection Enum") (candidatePosition :type "Array of /Game/Vector2 Structure") (spawnPosition :type "Vector Structure"))
  (switch `int` (`KismetMathLibrary.RandomInteger` 2)
    (:`0`
      ;[1 1 1] スポーンする"位置"を設定
      (set `local.spawnDirection` "NewEnumerator3"))
    (:`1`
      (set `local.spawnDirection` "NewEnumerator3")))
  ;[1 1 1] 選ばれた方角の座標群を保存
  (bind _output_get (set `local.candidatePosition` (break `/Game/Play/Common/GroundObject/WarpPoint/WarpPointPosition` (`BlueprintMapLibrary.Map_Find` (`self.SpawnPointDirection`) (`local.spawnDirection`)))))
  (bind (_output_x _output_y) (break `/Game/Vector2` (`|GetArrayItem` _output_get (`KismetMathLibrary.RandomInteger` (`KismetArrayLibrary.Array_Length` _output_get)))))
  (bind _output_get_2 (set `local.spawnPosition` (`KismetMathLibrary.MakeVector` _output_x _output_y 20.0)))
  (return _output_get_2 (`local.spawnDirection`)))

(fn `fSetAllWarpPoint`
  (locals (NorthPoint :type "/Game/Play/Common/GroundObject/WarpPoint/WarpPointPosition Structure") (SouthPoint :type "/Game/Play/Common/GroundObject/WarpPoint/WarpPointPosition Structure") (EastPoint :type "/Game/Play/Common/GroundObject/WarpPoint/WarpPointPosition Structure") (WestPoint :type "/Game/Play/Common/GroundObject/WarpPoint/WarpPointPosition Structure") (vec2 :type "/Game/Vector2 Structure"))
  (bind _northpoint_position (break `/Game/Play/Common/GroundObject/WarpPoint/WarpPointPosition` (`local.NorthPoint`)))
  (bind _southpoint_position (break `/Game/Play/Common/GroundObject/WarpPoint/WarpPointPosition` (`local.SouthPoint`)))
  (bind _eastpoint_position (break `/Game/Play/Common/GroundObject/WarpPoint/WarpPointPosition` (`local.EastPoint`)))
  (bind _westpoint_position (break `/Game/Play/Common/GroundObject/WarpPoint/WarpPointPosition` (`local.WestPoint`)))
  (bind _northpoint_position_2 (break `/Game/Play/Common/GroundObject/WarpPoint/WarpPointPosition` (`local.NorthPoint`)))
  (bind _southpoint_position_2 (break `/Game/Play/Common/GroundObject/WarpPoint/WarpPointPosition` (`local.SouthPoint`)))
  (bind _eastpoint_position_2 (break `/Game/Play/Common/GroundObject/WarpPoint/WarpPointPosition` (`local.EastPoint`)))
  (bind _westpoint_position_2 (break `/Game/Play/Common/GroundObject/WarpPoint/WarpPointPosition` (`local.WestPoint`)))
  (bind _outactors (`GameplayStatics.GetAllActorsOfClass` "/Game/Play/Common/GroundObject/WarpPoint/BP_WarpPoint.BP_WarpPoint_C"))
  (bind _output_get (set `self.mWarpPoint` _outactors))
  (for _array_element _output_get
    (bind (_returnvalue_x _returnvalue_y) (`KismetMathLibrary.BreakVector` (`self.K2_GetActorLocation` _array_element)))
    ;[1 1 1] 変換
    (set `local.vec2` (make `/Game/Vector2` _returnvalue_x _returnvalue_y))
    (switch `/Game/Play/Common/GroundObject/Intersection/TraficLight/TraficLightDirection` (`/Game/Play/Common/GroundObject/WarpPoint/BP_WarpPoint.mDirection` _array_element)
      (:`NewEnumerator0`
        (`KismetArrayLibrary.Array_Add` _northpoint_position_2 (`local.vec2`)))
      (:`NewEnumerator1`
        (`KismetArrayLibrary.Array_Add` _southpoint_position (`local.vec2`)))
      (:`NewEnumerator2`
        (`KismetArrayLibrary.Array_Add` _eastpoint_position (`local.vec2`)))
      (:`NewEnumerator3`
        (`KismetArrayLibrary.Array_Add` _westpoint_position (`local.vec2`)))))
  (bind _enumvalue (foreach `/Game/Play/Common/GroundObject/Intersection/TraficLight/TraficLightDirection` false)
    (:`LoopBody`
      (switch `/Game/Play/Common/GroundObject/Intersection/TraficLight/TraficLightDirection` _enumvalue
        (:`NewEnumerator0`
          (`BlueprintMapLibrary.Map_Add` (`self.SpawnPointDirection`) _enumvalue (make `/Game/Play/Common/GroundObject/WarpPoint/WarpPointPosition` _northpoint_position)))
        (:`NewEnumerator1`
          (`BlueprintMapLibrary.Map_Add` (`self.SpawnPointDirection`) _enumvalue (make `/Game/Play/Common/GroundObject/WarpPoint/WarpPointPosition` _southpoint_position_2)))
        (:`NewEnumerator2`
          (`BlueprintMapLibrary.Map_Add` (`self.SpawnPointDirection`) _enumvalue (make `/Game/Play/Common/GroundObject/WarpPoint/WarpPointPosition` _eastpoint_position_2)))
        (:`NewEnumerator3`
          (`BlueprintMapLibrary.Map_Add` (`self.SpawnPointDirection`) _enumvalue (make `/Game/Play/Common/GroundObject/WarpPoint/WarpPointPosition` _westpoint_position_2)))))))

(fn `UserConstructionScript`)

(fn `WarpCar`
  (params (position :type "Vector Structure") (WarpCar :type "/Game/Play/Common/GroundObject/Car/BP_CarBase Object Reference") (spawnCarDirection :type "/Game/Play/Common/GroundObject/Intersection/TraficLight/TraficLightDirection Enum" :default "NewEnumerator0"))
  (locals (saveWarpCar :type "/Game/Play/Common/GroundObject/Car/BP_CarBase Object Reference") (`save CarDirection` :type "/Game/Play/Common/GroundObject/Intersection/TraficLight/TraficLightDirection Enum") (`spawnCar Angle` :type "/Game/Play/Common/GroundObject/Intersection/TraficLight/TraficLightDirection Enum"))
  (bind _spawnangle_angletorotation (break `/Game/Play/Common/GroundObject/WarpPoint/SpawnAngle` (`self.SpawnAngle`)))
  (bind _output_get (set `local.saveWarpCar` WarpCar))
  (set `local.save CarDirection` spawnCarDirection)
  (`self.K2_SetActorLocation` _output_get position false true)
  ;[1 1 1] 車を生成する位置から生成する方向に変換する
  (switch `/Game/Play/Common/GroundObject/Intersection/TraficLight/TraficLightDirection` (`local.save CarDirection`)
    (:`NewEnumerator0`
      (set `local.spawnCar Angle` "NewEnumerator0"))
    (:`NewEnumerator1`
      (set `local.spawnCar Angle` "NewEnumerator1"))
    (:`NewEnumerator2`
      (set `local.spawnCar Angle` "NewEnumerator2"))
    (:`NewEnumerator3`
      (set `local.spawnCar Angle` "NewEnumerator3")))
  (`/Game/Play/Common/GroundObject/Car/BP_CarBase.SetCarDirection` (`local.saveWarpCar`) (`local.spawnCar Angle`))
  ;[1 1 1] 出現する方角に応じて向きを変更する
  (`self.K2_SetActorRotation` (`local.saveWarpCar`) (`BlueprintMapLibrary.Map_Find` _spawnangle_angletorotation (`local.spawnCar Angle`)) false))