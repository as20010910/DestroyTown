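; Player controller for the DestructionCity game, routing input to per-scene controller actors for building, middle story, destruction and results.
; Create/delete functions spawn or destroy each one, with creation also setting cursor and click events.
; Building input checks GetPause, mayor input checks operability (movement also blocked while charging), and Space skips story or results.
; Pause toggles the pause widget and adjusts cursor and click settings by pause and game state.
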(event `InputAction|GameEnd`
  (params (Key :type "Key Structure"))
  ;[1 0 0] ゲーム終了処理
  (:`Pressed`
    (`KismetSystemLibrary.QuitGame` null "Quit")))

(event `InputAction|Pause`
  (params (Key :type "Key Structure"))
  (:`Pressed`
    (`self.fChangePause`) ; カーソル関連の処理
    (`/Game/Pause/WBP_Pause.fChangeDraw` (`/Game/Play/Common/GameMode/GM_DestructionCity.mWBP_Pause` (cast `/Game/Play/Common/GameMode/GM_DestructionCity` (`GameplayStatics.GetGameMode`) :!pure true))) ; 表示切替処理
  ))

(event `InputAction|ShiftSelectBuilding`
  (params (Key :type "Key Structure"))
  (bind _mbp_buildingcontroller (`self.mBP_BuildingController`))
  (:`Pressed`
    (if (`self.GetPause`)
      (if (`KismetSystemLibrary.IsValid` _mbp_buildingcontroller)
        (`/Game/Play/Building/Controller/BP_BuildingController.F Side Building Attributes` _mbp_buildingcontroller)))))

(event `InputAction|Building`
  (params (Key :type "Key Structure"))
  (bind _mbp_buildingcontroller (`self.mBP_BuildingController`))
  (:`Pressed`
    (if (`self.GetPause`)
      (if (`KismetSystemLibrary.IsValid` _mbp_buildingcontroller)
        (`/Game/Play/Building/Controller/BP_BuildingController.fBuilding` _mbp_buildingcontroller)))))

(event `InputAxis|CameraMoveForward`
  (params (AxisValue :type "Float (single-precision)"))
  (bind _mbp_buildingcontroller (`self.mBP_BuildingController`))
  (if (`self.GetPause`)
    (if (`KismetSystemLibrary.IsValid` _mbp_buildingcontroller)
      (`/Game/Play/Building/Controller/BP_BuildingController.fCameraMoveForward` _mbp_buildingcontroller AxisValue))))

(event `InputAxis|CameraMoveRight`
  (params (AxisValue :type "Float (single-precision)"))
  (bind _mbp_buildingcontroller (`self.mBP_BuildingController`))
  (if (`self.GetPause`)
    (if (`KismetSystemLibrary.IsValid` _mbp_buildingcontroller)
      (`/Game/Play/Building/Controller/BP_BuildingController.fCameraMoveRight` _mbp_buildingcontroller AxisValue))))

(event `InputAction|SwitchLeftBuildingAttributes`
  (params (Key :type "Key Structure"))
  (bind _mbp_buildingcontroller (`self.mBP_BuildingController`))
  (:`Pressed`
    (if (`self.GetPause`)
      (if (`KismetSystemLibrary.IsValid` _mbp_buildingcontroller)
        (`/Game/Play/Building/Controller/BP_BuildingController.F Change Building Attributes Up` _mbp_buildingcontroller)))))

(event `InputAction|SwitchRightBuildingAttributes`
  (params (Key :type "Key Structure"))
  (bind _mbp_buildingcontroller (`self.mBP_BuildingController`))
  (:`Pressed`
    (if (`self.GetPause`)
      (if (`KismetSystemLibrary.IsValid` _mbp_buildingcontroller)
        (`/Game/Play/Building/Controller/BP_BuildingController.F Change Building Attributes Down` _mbp_buildingcontroller)))))

(event `InputAction|MayorAttack`
  (params (Key :type "Key Structure"))
  (bind _mbp_destructioncontroller (`self.mBP_DestructionController`))
  ;[1 1 1] 市長の攻撃処理
  (:`Pressed`
    (`/Engine/EditorBlueprintResources/StandardMacros.IsValid` _mbp_destructioncontroller
      (:`Is Valid`
        (if (`/Game/Play/Destruction/BP_DestructionController.mIsOperable` _mbp_destructioncontroller)
          (set `self.mIsPressAttack` true) ; 攻撃ボタンを押しているフラグをtrueに
        ))))
  (:`Released`
    (`/Engine/EditorBlueprintResources/StandardMacros.IsValid` _mbp_destructioncontroller
      (:`Is Valid`
        (if (`/Game/Play/Destruction/BP_DestructionController.mIsOperable` _mbp_destructioncontroller)
          (`/Game/Play/Destruction/BP_DestructionController.fMayorAttack` _mbp_destructioncontroller) ; 市長の攻撃処理
          (set `self.mIsPressAttack` false) ; 攻撃ボタンを押しているフラグをfalseに
        )))))

(event `InputAxis|MayorMoveForward`
  (params (AxisValue :type "Float (single-precision)"))
  (bind _mbp_destructioncontroller (`self.mBP_DestructionController`))
  ;[1 1 1] 市長の前進処理
  (`/Engine/EditorBlueprintResources/StandardMacros.IsValid` _mbp_destructioncontroller
    (:`Is Valid`
      (if (`/Game/Play/Destruction/BP_DestructionController.mIsOperable` _mbp_destructioncontroller)
        (if (not (`/Game/Play/Destruction/BP_DestructionController.mIsCharge` (`self.mBP_DestructionController`)))
          (`/Game/Play/Destruction/BP_DestructionController.fMayorMoveForward` _mbp_destructioncontroller AxisValue))))))

(event `InputAxis|MayorTurn`
  (params (AxisValue :type "Float (single-precision)"))
  (bind _mbp_destructioncontroller (`self.mBP_DestructionController`))
  ;[1 1 1] 市長の縦方向の視点処理
  (`/Engine/EditorBlueprintResources/StandardMacros.IsValid` _mbp_destructioncontroller
    (:`Is Valid`
      (if (`/Game/Play/Destruction/BP_DestructionController.mIsOperable` _mbp_destructioncontroller)
        (`/Game/Play/Destruction/BP_DestructionController.fMayorTurn` _mbp_destructioncontroller AxisValue)))))

(event `InputAxis|MayorLookUp`
  (params (AxisValue :type "Float (single-precision)"))
  (bind _mbp_destructioncontroller (`self.mBP_DestructionController`))
  ;[1 1 1] 市長の横方向の視点処理
  (`/Engine/EditorBlueprintResources/StandardMacros.IsValid` _mbp_destructioncontroller
    (:`Is Valid`
      (if (`/Game/Play/Destruction/BP_DestructionController.mIsOperable` _mbp_destructioncontroller)
        (`/Game/Play/Destruction/BP_DestructionController.fMayorLookUp` _mbp_destructioncontroller AxisValue)))))

(event `InputAxis|MayorMoveRight`
  (params (AxisValue :type "Float (single-precision)"))
  (bind _mbp_destructioncontroller (`self.mBP_DestructionController`))
  ;[1 1 1] 市長の左右の移動処理
  (`/Engine/EditorBlueprintResources/StandardMacros.IsValid` _mbp_destructioncontroller
    (:`Is Valid`
      (if (`/Game/Play/Destruction/BP_DestructionController.mIsOperable` _mbp_destructioncontroller)
        (if (not (`/Game/Play/Destruction/BP_DestructionController.mIsCharge` (`self.mBP_DestructionController`)))
          (`/Game/Play/Destruction/BP_DestructionController.fMayorMoveRight` _mbp_destructioncontroller AxisValue))))))

(event `InputAction|SwitchLeftMayorAttack`
  (params (Key :type "Key Structure"))
  (bind _mbp_destructioncontroller (`self.mBP_DestructionController`))
  ;[1 1 1] 市長の攻撃アイコンを左に移動
  (:`Pressed`
    (`/Engine/EditorBlueprintResources/StandardMacros.IsValid` _mbp_destructioncontroller
      (:`Is Valid`
        (if (`/Game/Play/Destruction/BP_DestructionController.mIsOperable` _mbp_destructioncontroller)
          (`/Game/Play/Destruction/BP_DestructionController.fSwitchLeftMayorAttack` _mbp_destructioncontroller))))))

(event `InputAction|SwitchRightMayorAttack`
  (params (Key :type "Key Structure"))
  (bind _mbp_destructioncontroller (`self.mBP_DestructionController`))
  ;[1 1 1] 市長の攻撃アイコンを右に移動
  (:`Pressed`
    (`/Engine/EditorBlueprintResources/StandardMacros.IsValid` _mbp_destructioncontroller
      (:`Is Valid`
        (if (`/Game/Play/Destruction/BP_DestructionController.mIsOperable` _mbp_destructioncontroller)
          (`/Game/Play/Destruction/BP_DestructionController.fSwitchRightMayorAttack` _mbp_destructioncontroller))))))

(event `PlayFootSound`
  ;[1 1 1] 市長の足音を再生
  (`/Engine/EditorBlueprintResources/StandardMacros.DoOnce` false :!label _label
    (:`Completed`
      (`GameplayStatics.PlaySoundAtLocation` "/Game/Play/Destruction/Sounds/SoundWave/SoundEffect_FootSound.SoundEffect_FootSound" (0.0 0.0 0.0) (struct) 1.0 1.0 0.0 null null null)
      (`KismetSystemLibrary.Delay` 1.0)
      (goto _label :!via `Reset`))))

(event `Key|SpaceBar`
  (params (Key :type "Key Structure"))
  (bind _mbp_resultcontroller (`self.mBP_ResultController`))
  (bind _mbp_middlestorycontroller (`self.mBP_MiddleStoryController`))
  ;[1 1 1] ストーリーをスキップする
  (:`Pressed`
    (`/Engine/EditorBlueprintResources/StandardMacros.IsValid` _mbp_middlestorycontroller
      (:`Is Valid`
        (`/Game/Play/Story/BP_MiddleStoryController.SkipStory` _mbp_middlestorycontroller))
      (:`Is Not Valid`
        (`/Engine/EditorBlueprintResources/StandardMacros.IsValid` _mbp_resultcontroller
          (:`Is Valid`
            (`/Game/Result/BP_ResultController.SkipStory` _mbp_resultcontroller)))))))

(fn `fChangePause`
  (if (`|EnumEquality` (`/Game/Play/Common/GameInstance/GMI_DestructionCIty.mPause` (cast `/Game/Play/Common/GameInstance/GMI_DestructionCIty` (`GameplayStatics.GetGameInstance`) :!pure true)) "NewEnumerator0")
    (if (`|EnumEquality` (`/Game/Play/Common/GameMode/GM_DestructionCity.mGameState` (cast `/Game/Play/Common/GameMode/GM_DestructionCity` (`GameplayStatics.GetGameMode`) :!pure true)) "NewEnumerator1")
      (set `self.bShowMouseCursor` false) ; マウスカーソルを表示する
      (set `self.bEnableClickEvents` false) ; クリックイベントを有効にする
      (set `self.ClickEventKeys` (`self.mDestructionClickKeys`)) ; 使用するキーを設定
    )
    (else
      (set `self.bShowMouseCursor` true) ; マウスカーソルを表示する
      (set `self.bEnableClickEvents` true) ; クリックイベントを有効にする
      (set `self.ClickEventKeys` (`self.mBuildingClickKeys`)) ; 使用するキーを設定
    )))

(fn `fCreateBuildingController`
  ;[1 1 1] 各シーンのコントローラの作成
  (bind _returnvalue (`|SpawnActorFromClass` "/Game/Play/Building/Controller/BP_BuildingController.BP_BuildingController_C" (`KismetMathLibrary.MakeTransform` (0.0 0.0 0.0)) "Undefined" "OverrideRootScale" null null))
  (set `self.mBP_BuildingController` _returnvalue)
  (set `self.bShowMouseCursor` true) ; マウスカーソルを表示する
  (set `self.bEnableClickEvents` true) ; クリックイベントを有効にする
  (set `self.ClickEventKeys` (`self.mBuildingClickKeys`)) ; 使用するキーを設定
)

(fn `fCreateDestructionController`
  ;[1 1 1] 各シーンのコントローラの作成
  (bind _returnvalue (`|SpawnActorFromClass` "/Game/Play/Destruction/BP_DestructionController.BP_DestructionController_C" (`KismetMathLibrary.MakeTransform` (0.0 0.0 0.0)) "Undefined" "OverrideRootScale" null null))
  (set `self.mBP_DestructionController` _returnvalue)
  (set `self.bShowMouseCursor` false) ; マウスカーソルを表示する
  (set `self.bEnableClickEvents` false) ; クリックイベントを有効にする
  (set `self.ClickEventKeys` (`self.mDestructionClickKeys`)) ; 使用するキーを設定
)

(fn `fCreateMiddleStoryController`
  ;[1 1 1] 各シーンのコントローラの作成
  (bind _returnvalue (`|SpawnActorFromClass` "/Game/Play/Story/BP_MiddleStoryController.BP_MiddleStoryController_C" (`KismetMathLibrary.MakeTransform` (0.0 0.0 0.0)) "Undefined" "OverrideRootScale" null null))
  (set `self.mBP_MiddleStoryController` _returnvalue)
  (set `self.bShowMouseCursor` false) ; マウスカーソルを表示する
  (set `self.bEnableClickEvents` false) ; クリックイベントを有効にする
)

(fn `fCreateResultController`
  ;[1 1 1] 各シーンのコントローラの作成
  (bind _returnvalue (`|SpawnActorFromClass` "/Game/Result/BP_ResultController.BP_ResultController_C" (`KismetMathLibrary.MakeTransform` (0.0 0.0 0.0)) "Undefined" "OverrideRootScale" null null))
  (set `self.mBP_ResultController` _returnvalue)
  (set `self.bShowMouseCursor` false) ; マウスカーソルを表示する
  (set `self.bEnableClickEvents` false) ; クリックイベントを有効にする
)

(fn `fDeleteBuildingController`
  (bind _mbp_buildingcontroller (`self.mBP_BuildingController`))
  ;[1 1 1] 建物建築シーンのコントローラを削除
  (`/Engine/EditorBlueprintResources/StandardMacros.IsValid` _mbp_buildingcontroller
    (:`Is Valid`
      (`self.K2_DestroyActor` _mbp_buildingcontroller))))

(fn `fDeleteDestructionController`
  (bind _mbp_destructioncontroller (`self.mBP_DestructionController`))
  ;[1 1 1] 建物破壊シーンのコントローラを削除
  (`/Engine/EditorBlueprintResources/StandardMacros.IsValid` _mbp_destructioncontroller
    (:`Is Valid`
      (`self.K2_DestroyActor` _mbp_destructioncontroller))))

(fn `fDeleteMiddleStoryController`
  (bind _mbp_middlestorycontroller (`self.mBP_MiddleStoryController`))
  ;[1 1 1] 中盤ストーリーシーンのコントローラを削除
  (`/Engine/EditorBlueprintResources/StandardMacros.IsValid` _mbp_middlestorycontroller
    (:`Is Valid`
      (`self.K2_DestroyActor` _mbp_middlestorycontroller))))

(fn `fDeleteResultController`
  (bind _mbp_resultcontroller (`self.mBP_ResultController`))
  ;[1 1 1] 中盤ストーリーシーンのコントローラを削除
  (`/Engine/EditorBlueprintResources/StandardMacros.IsValid` _mbp_resultcontroller
    (:`Is Valid`
      (`self.K2_DestroyActor` _mbp_resultcontroller))))

(fn `UserConstructionScript`)