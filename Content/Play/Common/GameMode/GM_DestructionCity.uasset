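; GM_DestructionCity is the game mode for a city build-and-destroy game with Building, Middle Story and Destruction states.
; On BeginPlay it spawns a manager actor for each of the three states through FCreateManager.
; It then switches on MGameState to initialize the matching manager and has PC_DestructionCity create that state's controller.
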(event `self.ReceiveBeginPlay`
  (bind _aspc_destruction_city (cast `/Game/Play/Common/Controller/PC_DestructionCity` (`GameplayStatics.GetPlayerController` 0) :!pure true))
  ;[1 1 1] 初期化処理
  (`self.fCreateManager`) ; それぞれのゲームモードのマネージャーを生成
  (switch `/Game/Play/Common/GameMode/EN_GameSate` (`self.mGameState`)
    (:`NewEnumerator0`
      (`/Game/Play/Building/BP_BuildingManager.BuildingInitialize` (`self.mBP_BuildingManager`))
      (`/Game/Play/Common/Controller/PC_DestructionCity.fCreateBuildingController` _aspc_destruction_city))
    (:`NewEnumerator2`
      (`/Game/Story/BP_MiddleStoryManager.MiddleStoryInitialize` (`self.mBP_MiddleStoryManager`))
      (`/Game/Play/Common/Controller/PC_DestructionCity.fCreateMiddleStoryController` _aspc_destruction_city))
    (:`NewEnumerator1`
      (`/Game/Play/Destruction/BP_DestructionManager.DestructionInitialize` (`self.mBP_DestructionManager`))
      (`/Game/Play/Common/Controller/PC_DestructionCity.fCreateDestructionController` _aspc_destruction_city))))

(fn `fCreateManager`
  ;[1 1 1] それぞれのゲームモードの作成
  (bind _returnvalue (`|SpawnActorFromClass` "/Game/Play/Building/BP_BuildingManager.BP_BuildingManager_C" (`KismetMathLibrary.MakeTransform` (0.0 0.0 0.0)) "Undefined" "OverrideRootScale" null null))
  (set `self.mBP_BuildingManager` _returnvalue)
  (bind _returnvalue_2 (`|SpawnActorFromClass` "/Game/Play/Destruction/BP_DestructionManager.BP_DestructionManager_C" (`KismetMathLibrary.MakeTransform` (0.0 0.0 0.0)) "Undefined" "OverrideRootScale" null null))
  (set `self.mBP_DestructionManager` _returnvalue_2)
  (bind _returnvalue_3 (`|SpawnActorFromClass` "/Game/Story/BP_MiddleStoryManager.BP_MiddleStoryManager_C" (`KismetMathLibrary.MakeTransform` (0.0 0.0 0.0)) "Undefined" "OverrideRootScale" null null))
  (set `self.mBP_MiddleStoryManager` _returnvalue_3))

(fn `UserConstructionScript`)