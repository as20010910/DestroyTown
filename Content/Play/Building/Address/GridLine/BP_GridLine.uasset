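; BP_GridLine displays placement grid lines that match the building size currently selected in the city game.
; On BeginPlay or ChangeGridLine, it reads the selected size from the game mode's building manager cursor.
; It toggles child components under the square and two rectangle grid roots; large squares show none of these, and only small squares show the non-selectable model.
; HIddonGridLine hides all grids, the outer frame and that model.
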(event `self.ReceiveBeginPlay`
  (`self.ChangeGridLine`))

(event `ChangeGridLine`
  (bind _mbp_buildingmanager (`/Game/Play/Common/GameMode/GM_DestructionCity.mBP_BuildingManager` (cast `/Game/Play/Common/GameMode/GM_DestructionCity` (`GameplayStatics.GetGameMode`) :!pure true)))
  (bind _mbp_cursor (`/Game/Play/Building/BP_BuildingManager.mBP_Cursor` _mbp_buildingmanager))
  (`/Engine/EditorBlueprintResources/StandardMacros.IsValid` _mbp_buildingmanager
    (:`Is Valid`
      (`/Engine/EditorBlueprintResources/StandardMacros.IsValid` _mbp_cursor
        (:`Is Valid`
          (bind _value_size (`/Game/Play/Building/Cursor/BP_Cursor.fGetSelectBuildingSize` _mbp_cursor)) ; 現在選択中のサイズを取得
          (if (`|EnumEquality` _value_size "NewEnumerator0")
            (`self.NotSelectModelVisibiity` true)
            (else
              (`self.NotSelectModelVisibiity` false)))
          (switch `/Game/Play/Building/Data/EN_BuildingSize` _value_size
            (:`NewEnumerator0`
              (`self.ChangeGridVisibility` (`self.SSGrid`) true :!label _label)
              (`self.ChangeGridVisibility` (`self.MRGrid`))
              (`self.ChangeGridVisibility` (`self.LRGrid`)))
            (:`NewEnumerator1`
              (goto _label))
            (:`NewEnumerator2`
              (`self.ChangeGridVisibility` (`self.SSGrid`))
              (`self.ChangeGridVisibility` (`self.MRGrid`))
              (`self.ChangeGridVisibility` (`self.LRGrid`)))
            (:`NewEnumerator4`
              (`self.ChangeGridVisibility` (`self.SSGrid`))
              (`self.ChangeGridVisibility` (`self.MRGrid`) true)
              (`self.ChangeGridVisibility` (`self.LRGrid`)))
            (:`NewEnumerator5`
              (`self.ChangeGridVisibility` (`self.SSGrid`))
              (`self.ChangeGridVisibility` (`self.MRGrid`))
              (`self.ChangeGridVisibility` (`self.LRGrid`) true))))))))

(event `ChangeGridVisibility`
  (params (target :type "SceneComponent Object Reference") (DrawFlag :type Boolean))
  (bind _children (`SceneComponent.GetChildrenComponents` target false))
  ;[1 1 1] グリッド線の描画を一括変更
  (if DrawFlag
    (for _array_element _children
      (`SceneComponent.SetVisibility` _array_element true false))
    (else
      (for _array_element_2 _children
        (`SceneComponent.SetVisibility` _array_element_2 false false)))))

(event `NotSelectModelVisibiity`
  (params (`new Visibillity` :type Boolean))
  (bind _notselect (`self.NotSelect`))
  (if `new Visibillity`
    (`SceneComponent.SetVisibility` _notselect true false)
    (else
      (`SceneComponent.SetVisibility` _notselect false false))))

(event `HIddonGridLine`
  (`self.ChangeGridVisibility` (`self.OutFrame`))
  (`self.ChangeGridVisibility` (`self.SSGrid`))
  (`self.ChangeGridVisibility` (`self.MRGrid`))
  (`self.ChangeGridVisibility` (`self.LRGrid`))
  (`SceneComponent.SetVisibility` (`self.NotSelect`) false false))

(fn `UserConstructionScript`)