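; Flashing helper Blueprint under Building/Address that toggles a flash flag at a settable interval.
; On BeginPlay it spawns its own BP_Timer and starts a looping timer event at the DELTATIME step from GM_DestructionCity.
; While the move flag is set, each tick advances the BP_Timer and inverts the flash flag when it elapses.
; The file only maintains the flag and applies no visual change itself.
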(event `self.ReceiveBeginPlay`
  (bind _returnvalue (`|SpawnActorFromClass` "/Game/Play/Common/GroundObject/BP_Timer.BP_Timer_C" (`KismetMathLibrary.MakeTransform` (0.0 0.0 0.0)) "Undefined" "OverrideRootScale" null null)) ; タイマーの作成
  (set `self.mBP_Timer` _returnvalue)
  (`KismetSystemLibrary.K2_SetTimerDelegate` (delegate `CountUpdate`) (`/Game/Play/Common/GameMode/GM_DestructionCity.DELTA_TIME` (cast `/Game/Play/Common/GameMode/GM_DestructionCity` (`GameplayStatics.GetGameMode`) :!pure true)) true) ; 更新処理
)

(event `CountUpdate`
  (if (`self.mMoveFlag`)
    (bind _newparam (`/Game/Play/Common/GroundObject/BP_Timer.fCountUp` (`self.mBP_Timer`) (`/Game/Play/Common/GameMode/GM_DestructionCity.DELTA_TIME` (cast `/Game/Play/Common/GameMode/GM_DestructionCity` (`GameplayStatics.GetGameMode`) :!pure true))))
    (if _newparam
      (if (`self.mFlashFlag`)
        (set `self.mFlashFlag` false)
        (else
          (set `self.mFlashFlag` true))))))

(fn `fSetFlashInterval`
  (params (mMaxTime :type "Float (double-precision)"))
  (`/Game/Play/Common/GroundObject/BP_Timer.fSetMaxTime` (`self.mBP_Timer`) mMaxTime))

(fn `UserConstructionScript`)