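; BP_Section is a city building plot that hosts a placed building and lets houses develop into mansions.
; Cursor overlap previews the selected building as a translucent mesh on empty plots, or flashes upgradeable houses.
; Placement and development swap the BPBuildingBase child actor's class, then set its mesh and type.
; Mansion, service and production plots leave the address manager and lose collision, while FSelect toggles an unavailable-plot overlay.
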(event `SetBuilding`
  (bind _asbp_building_base (`self.fGetBuildingBase`))
  ;[1 1 1] 建物作成処理
  ;;[1 1 1] 現在選択している建物属性に応じて処理を設定
  (bind _buildinginfo (`/Game/Play/Building/Cursor/BP_Cursor.fGetSelectBuildingInfo` (`/Game/Play/Building/BP_BuildingManager.mBP_Cursor` (`/Game/Play/Common/GameMode/GM_DestructionCity.mBP_BuildingManager` (cast `/Game/Play/Common/GameMode/GM_DestructionCity` (`GameplayStatics.GetGameMode`) :!pure true)))))
  (switch `/Game/Play/Building/Data/EN_BuildingAttributes` (`.BuildingAttributes_21_00D082284D7C4698EF9227B7891E9CBD` (break `/Game/Play/Building/Data/ST_BuildingDataTable` _buildinginfo))
    (:`NewEnumerator0`
      ;;[1 1 1] 住居の時の処理
      (`ChildActorComponent.SetChildActorClass` (`self.BP_BuildingBase`) "/Game/Play/Building/BP_Building/BP_House.BP_House_C"))
    (:`NewEnumerator1`
      ;;[1 1 1] サービスの時の処理
      (`ChildActorComponent.SetChildActorClass` (`self.BP_BuildingBase`) "/Game/Play/Building/BP_Building/BP_ServiceBuilding.BP_ServiceBuilding_C")
      ;;[1 1 1] 住居以外は選択できないように
      (`self.DeleteSection` :!label _label))
    (:`NewEnumerator2`
      ;;[1 1 1] 生産の時の処理
      (`ChildActorComponent.SetChildActorClass` (`self.BP_BuildingBase`) "/Game/Play/Building/BP_Building/BP_ProductionBuilding.BP_ProductionBuilding_C")
      (goto _label)))
  ;;[1 1 1] モデルを設定
  (`/Game/Play/Building/BP_Building/BP_BuildingBase.fSetMesh` _asbp_building_base (break `/Game/Play/Building/Data/ST_BuildingDataTable` _buildinginfo))
  (`/Game/Play/Building/BP_Building/BP_BuildingBase.fClear` _asbp_building_base 1.0)
  (set `self.mState` "NewEnumerator1")
  (set `/Game/Play/Building/BP_Building/BP_BuildingBase.mBuilding` (break `/Game/Play/Building/Data/ST_BuildingDataTable` _buildinginfo) (`self.fGetBuildingBase`)) ; 建物の種類を保存
)

(event `SetDevelopment`
  (bind _asbp_building_base (`self.fGetBuildingBase`))
  ;[1 1 1] 建物発展処理
  (switch `/Game/Play/Building/Data/EN_Building` (`/Game/Play/Building/BP_Building/BP_BuildingBase.mBuilding` (`self.fGetBuildingBase`))
    (:`NewEnumerator0`
      ;;[1 1 1] マンションにする
      (`ChildActorComponent.SetChildActorClass` (`self.BP_BuildingBase`) "/Game/Play/Building/BP_Building/BP_Mansion.BP_Mansion_C")
      ;;[1 1 1] モデルを設定
      (`/Game/Play/Building/BP_Building/BP_BuildingBase.fSetMesh` (`self.fGetBuildingBase`) "NewEnumerator1")
      (set `/Game/Play/Building/BP_Building/BP_BuildingBase.mBuilding` "NewEnumerator1" _asbp_building_base) ; 建物の種類を保存
    )
    (:`NewEnumerator2`
      (`ChildActorComponent.SetChildActorClass` (`self.BP_BuildingBase`) "/Game/Play/Building/BP_Building/BP_Mansion.BP_Mansion_C")
      (`/Game/Play/Building/BP_Building/BP_BuildingBase.fSetMesh` (`self.fGetBuildingBase`) "NewEnumerator3")
      (set `/Game/Play/Building/BP_Building/BP_BuildingBase.mBuilding` "NewEnumerator3" _asbp_building_base) ; 建物の種類を保存
    )
    (:`NewEnumerator4`
      (`ChildActorComponent.SetChildActorClass` (`self.BP_BuildingBase`) "/Game/Play/Building/BP_Building/BP_Mansion.BP_Mansion_C")
      (`/Game/Play/Building/BP_Building/BP_BuildingBase.fSetMesh` (`self.fGetBuildingBase`) "NewEnumerator5")
      (set `/Game/Play/Building/BP_Building/BP_BuildingBase.mBuilding` "NewEnumerator5" _asbp_building_base) ; 建物の種類を保存
    ))
  (`/Game/Play/Building/BP_Building/BP_BuildingBase.fClear` _asbp_building_base 1.0) ; 透明度を戻す
  (`self.DeleteSection`))

(event `DeleteSection`
  ;[1 1 1] 選択できないように
  (`/Game/Play/Building/Address/BP_AddressManager.fDeleteAddressInSectionElement` (`/Game/Play/Building/BP_BuildingManager.mBP_AddressManager` (`/Game/Play/Common/GameMode/GM_DestructionCity.mBP_BuildingManager` (cast `/Game/Play/Common/GameMode/GM_DestructionCity` (`GameplayStatics.GetGameMode`) :!pure true))) (`self.K2_GetActorLocation`))
  (`PrimitiveComponent.SetCollisionEnabled` (`self.SectionCollider`) "NoCollision"))

(event `self.SectionCollider.OnComponentBeginOverlap`
  (params (OverlappedComponent :type "PrimitiveComponent Object Reference") (OtherActor :type "Actor Object Reference") (OtherComp :type "PrimitiveComponent Object Reference") (OtherBodyIndex :type Integer) (bFromSweep :type Boolean) (SweepResult :type "HitResult Structure (by ref)"))
  ;[1 1 1] 仮モデル設置処理
  ;;[1 1 1] 衝突したのがカーソルか確認
  (if (== (`/Game/Play/Building/Cursor/BP_Cursor.ClickCollider` (cast `/Game/Play/Building/Cursor/BP_Cursor` OtherActor :!pure true)) OtherComp)
    (`self.ChangeInstant`)))

(event `ChangeInstant`
  ;[1 1 1] 仮モデル設置処理
  (if (`|EnumEquality` (`self.mState`) "NewEnumerator0")
    (`self.SetInstantBuilding`) ; 仮建物作成処理
    (else
      (`self.SetDevelopmentBuilding`))))

(event `SetDevelopmentBuilding`
  ;[1 1 1] 仮モデル設置処理
  ;;[1 1 1] 発展できる建物のみ処理をする
  (switch `/Game/Play/Building/Data/EN_Building` (`/Game/Play/Building/BP_Building/BP_BuildingBase.mBuilding` (`self.fGetBuildingBase`))
    (:`NewEnumerator0`
      _)
    (:`NewEnumerator2`
      _)
    (:`NewEnumerator4`
      _))
  ;;[1 1 1] 家を点滅させる
  (bind _asbp_house (cast `/Game/Play/Building/BP_Building/BP_House` (`ChildActorComponent.ChildActor` (`self.BP_BuildingBase`))))
  (`/Engine/EditorBlueprintResources/StandardMacros.IsValid` _asbp_house
    (:`Is Valid`
      (set `/Game/Play/Building/BP_Building/BP_House.Flashiing Flag` true _asbp_house))))

(event `SetInstantBuilding`
  (bind _asbp_building_base (`self.fGetBuildingBase`))
  ;[1 1 1] 仮モデル設置処理
  (`/Game/Play/Building/BP_Building/BP_BuildingBase.fSetMesh` _asbp_building_base (`/Game/Play/Building/Cursor/BP_Cursor.mNowSelectBuilding` (`/Game/Play/Building/BP_BuildingManager.mBP_Cursor` (`/Game/Play/Common/GameMode/GM_DestructionCity.mBP_BuildingManager` (cast `/Game/Play/Common/GameMode/GM_DestructionCity` (`GameplayStatics.GetGameMode`) :!pure true))))) ; モデルを設定
  (`/Game/Play/Building/BP_Building/BP_BuildingBase.fClear` _asbp_building_base 0.3) ; 半透明モデルに
)

(event `self.SectionCollider.OnComponentEndOverlap`
  (params (OverlappedComponent :type "PrimitiveComponent Object Reference") (OtherActor :type "Actor Object Reference") (OtherComp :type "PrimitiveComponent Object Reference") (OtherBodyIndex :type Integer))
  (bind (_asbp_cursor _bsuccess) (cast `/Game/Play/Building/Cursor/BP_Cursor` OtherActor :!pure true))
  ;[1 1 1] 仮モデル削除処理
  ;;[1 1 1] 離れたのがカーソルか確認
  (if _bsuccess
    (if (== (`/Game/Play/Building/Cursor/BP_Cursor.ClickCollider` _asbp_cursor) OtherComp)
      (`self.DeleteInstant`))))

(event `DeleteInstant`
  ;[1 1 1] 仮モデル削除処理
  (if (`|EnumEquality` (`self.mState`) "NewEnumerator0")
    (`self.DeleteInstantModel`)
    (else
      (`self.DeleteDevelopmentBuilding`))))

(event `DeleteDevelopmentBuilding`
  (bind _asbp_building_base (`self.fGetBuildingBase`))
  ;[1 1 1] 仮モデル削除処理
  ;;[1 1 1] 発展できる建物のみ処理をする
  (switch `/Game/Play/Building/Data/EN_Building` (`/Game/Play/Building/BP_Building/BP_BuildingBase.mBuilding` (`self.fGetBuildingBase`))
    (:`NewEnumerator0`
      _)
    (:`NewEnumerator2`
      _)
    (:`NewEnumerator4`
      _))
  (`/Game/Play/Building/BP_Building/BP_BuildingBase.fClear` _asbp_building_base 1.0) ; 半透明モデルに
  ;;[1 1 1] 家を点滅を解除させる
  (bind _asbp_house (cast `/Game/Play/Building/BP_Building/BP_House` _asbp_building_base))
  (`/Engine/EditorBlueprintResources/StandardMacros.IsValid` _asbp_house
    (:`Is Valid`
      (set `/Game/Play/Building/BP_Building/BP_House.Flashiing Flag` false _asbp_house))))

(event `DeleteInstantModel`
  ;[1 1 1] 仮モデル削除処理
  (`/Game/Play/Building/BP_Building/BP_BuildingBase.fSetMesh` (`self.fGetBuildingBase`) "NewEnumerator13") ; モデルを設定
)

(fn `F Select`
  (params (IsSelect :type Boolean))
  (bind _notselectmodel (`self.NotSelectModel`))
  (if IsSelect
    (set `self.mNotSelectFlag` false) ; 使用可能に
    (`SceneComponent.SetVisibility` (`self.NotSelectModel`) false false) ; 消す
    (else
      (set `self.mNotSelectFlag` true) ; 一時的に使用できなくする
      (`SceneComponent.SetVisibility` _notselectmodel true false) ; 表示する
      (`PrimitiveComponent.SetMaterial` _notselectmodel 0 "/Game/Play/Building/BP_Building/Model/MT_NotSelect.MT_NotSelect"))))

(fn `fGetBuildingBase`
  (returns (`AsBP Building Base` :type "/Game/Play/Building/BP_Building/BP_BuildingBase Object Reference"))
  (return (cast `/Game/Play/Building/BP_Building/BP_BuildingBase` (`ChildActorComponent.ChildActor` (`self.BP_BuildingBase`)) :!pure true)))

(fn `fIsHouse`
  (returns (HouseFlag :type Boolean))
  (switch `/Game/Play/Building/Data/EN_Building` (`/Game/Play/Building/BP_Building/BP_BuildingBase.mBuilding` (`self.fGetBuildingBase`))
    (:`NewEnumerator13`
      _)
    (:`NewEnumerator0`
      (return true))
    (:`NewEnumerator1`
      _)
    (:`NewEnumerator2`
      (return true))
    (:`NewEnumerator3`
      _)
    (:`NewEnumerator4`
      (return true))
    (:`NewEnumerator5`
      _)
    (:`NewEnumerator6`
      _)
    (:`NewEnumerator7`
      _)
    (:`NewEnumerator8`
      _)
    (:`NewEnumerator9`
      _)
    (:`NewEnumerator10`
      _)
    (:`NewEnumerator11`
      _))
  (return false))

(fn `UserConstructionScript`)