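; BP_VariableSection is a building section actor whose footprint varies with its building size and which tracks a group of section actors.
; On BeginPlay it sets its X/Y scale from the size enum, covering square and rectangle footprints, and keeps its Z scale.
; A position function centers it on the grouped sections' average X/Y, taking Z from a member.
; A delete function forwards DeleteSection to every grouped section.
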(event `self.ReceiveBeginPlay`
  (`self.fCreateScale`))

(fn `fCraetePos`
  (locals (addPosition :type "Vector Structure"))
  (bind (_returnvalue_x _returnvalue_y) (`KismetMathLibrary.BreakVector` (/ (`local.addPosition`) (`KismetMathLibrary.Conv_IntToDouble` (`KismetArrayLibrary.Array_Length` (`self.mSectionVector`))))))
  (for _array_element (`self.mSectionVector`)
    ;[1 1 1] 平均を取る
    (set `local.addPosition` (+ (`self.K2_GetActorLocation` _array_element) (`local.addPosition`))))
  (bind (_returnvalue_x_2 _returnvalue_y_2 _returnvalue_z) (`KismetMathLibrary.BreakVector` (`self.K2_GetActorLocation` _array_element)))
  (`self.K2_SetActorLocation` (`KismetMathLibrary.MakeVector` _returnvalue_x _returnvalue_y _returnvalue_z) false true) ; 平均値を自身の座標に
)

(fn `fCreateScale`
  (locals (length :type Integer) (width :type Integer))
  (bind (_returnvalue_x _returnvalue_y _returnvalue_z) (`KismetMathLibrary.BreakVector` (`self.GetActorScale3D`)))
  (switch `/Game/Play/Building/Data/EN_BuildingSize` (`self.mBuildingSize`)
    (:`NewEnumerator0`
      ;[1 1 1] 奥行を定める
      (bind _output_get (set `local.length` 1))
      ;[1 1 1] 横幅を定める
      (set `local.width` _output_get :!label _label))
    (:`NewEnumerator1`
      (set `local.length` 2)
      (goto _label))
    (:`NewEnumerator2`
      (set `local.length` 3)
      (goto _label))
    (:`NewEnumerator4`
      (set `local.length` 2)
      (set `local.width` 1))
    (:`NewEnumerator5`
      (set `local.length` 2)
      (set `local.width` 3)))
  ;[1 1 1] 拡大率に反映させる
  (`self.SetActorScale3D` (`KismetMathLibrary.MakeVector` (`KismetMathLibrary.Conv_IntToDouble` (`local.length`)) (`KismetMathLibrary.Conv_IntToDouble` (`local.width`)) _returnvalue_z)))

(fn `fDeleteSection`
  (for _array_element (`self.mSectionVector`)
    (`self.DeleteSection` _array_element)))

(fn `UserConstructionScript`
  (`parent.UserConstructionScript`))