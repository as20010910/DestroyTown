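; BP_Address manages a block of child BP_Section building plots in the city game and spawns its grid lines.
; At BeginPlay it numbers the plots and caches their locations by building size and in a position-to-section map.
; Cursor placement queries that cache for the nearest selectable plot, while overlap checks disable and unmap conflicting plots.
; Tax collection pays out only for built plots recently rendered on screen, spawning coin UI.
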(event `self.ReceiveBeginPlay`
  ;[1 1 1] 初期化処理
  (`self.fSaveSectionPosition`) ; 各区画の座標を保存しておく
  (`self.SetSections`) ; 子BPを変数化
  (`self.CreateGrid`) ; グリッド線の作成
)

(event `CreateGrid`
  ;[1 1 1] グリッド線の作成
  (bind _returnvalue (`|SpawnActorFromClass` "/Game/Play/Building/Address/GridLine/BP_GridLine.BP_GridLine_C" (`self.GetTransform`) "Undefined" "OverrideRootScale" null null))
  (set `self.mGridLine` _returnvalue))

(event `ChangeGrid`
  ;[1 1 1] Grid変更処理
  (`/Game/Play/Building/Address/GridLine/BP_GridLine.ChangeGridLine` (`self.mGridLine`)))

(event `SetSections`
  ;[1 1 1] 区画管理処理
  (for (_array_element _array_index) (`self.GetAllChildActors` false)
    (bind _asbp_section (cast `/Game/Play/Building/Address/Section/BP_Section` _array_element :!pure true))
    (`KismetArrayLibrary.Array_Add` (`self.mSections`) _asbp_section)
    (set `/Game/Play/Building/Address/Section/BP_Section.mSectionNumber` _array_index _asbp_section)))

(event `SectionsTex`
  ;[1 1 1] 税金徴収処理
  (for _array_element (`self.mSections`)
    ;;[1 1 1] 家が建っていたら処理を行う
    (if (`|EnumInequality` (`/Game/Play/Building/Address/Section/BP_Section.mState` _array_element) "NewEnumerator0")
      (if (`self.WasRecentlyRendered` (`ChildActorComponent.ChildActor` (`/Game/Play/Building/Address/Section/BP_Section.BP_BuildingBase` _array_element)) (`/Game/Play/Common/GameMode/GM_DestructionCity.DELTA_TIME` (cast `/Game/Play/Common/GameMode/GM_DestructionCity` (`GameplayStatics.GetGameMode`) :!pure true)))
        (`/Game/Play/Building/Address/Section/BP_Section.CreateMoney` _array_element) ; コインUI生成処理
        (`/Game/Play/Building/BP_BuildingManager.fAddTex` (`/Game/Play/Common/GameMode/GM_DestructionCity.mBP_BuildingManager` (cast `/Game/Play/Common/GameMode/GM_DestructionCity` (`GameplayStatics.GetGameMode`) :!pure true)) (`/Game/Play/Building/BP_Building/BP_BuildingBase.mSaveTexNum` (`/Game/Play/Building/Address/Section/BP_Section.fGetBuildingBase` _array_element))) ; 税金追加処理
      ))))

(fn `fChackOverlapSecitons`
  (params (targetSection :type "/Game/Play/Building/Address/Section/BP_Section Object Reference") (DeleteFlag :type Boolean))
  (locals (array :type "Array of Integer") (section :type "/Game/Play/Building/Address/Section/BP_Section Object Reference") (sectionNum :type Integer :default -1) (NewLocalVar_0 :type Integer))
  (bind (_returnvalue_x _returnvalue_y) (`KismetMathLibrary.BreakVector` (`self.K2_GetActorLocation` (`local.section`))))
  (bind _output_get (set `local.section` targetSection))
  (set `local.array` (`/Game/Play/Building/Address/Section/BP_Section.fSectionPosition` _output_get)) ; とりあえず保存
  (if (not DeleteFlag)
    (`KismetArrayLibrary.Array_Add` (`self.mHousePosition`) (make `/Game/Vector2` _returnvalue_x _returnvalue_y)) ; 家用配列に追加
    (bind _output_get_2 (set `local.sectionNum` (`/Game/Play/Building/Address/Section/BP_Section.mSectionNumber` (`local.section`)))))
  (for _array_element (`self.mSections`)
    (bind _msectionnumber (`/Game/Play/Building/Address/Section/BP_Section.mSectionNumber` _array_element))
    (set `local.NewLocalVar_0` _msectionnumber)
    (if (!= _msectionnumber _output_get_2)
      (bind (_flag _section) (`/Game/Play/Building/Address/Section/BP_Section.F Is Get Section Position` _array_element (`local.array`)))
      (if _flag
        (set `/Game/Play/Building/Address/Section/BP_Section.mNotSelectFlag` true _section)
        (`self.fDeleteSectionElement` (`self.K2_GetActorLocation` _section)) ; Mapからも削除
      ))))

(fn `fDeleteSectionElement`
  (params (Position :type "Vector Structure"))
  (returns (DeleteFlag :type Boolean))
  (bind _mpositiontosection (`self.mPositionToSection`))
  (`BlueprintMapLibrary.Map_Remove` _mpositiontosection (make `/Game/Vector2` Position_X Position_Y))
  (return (== (`BlueprintMapLibrary.Map_Length` _mpositiontosection) 0)) ; 中身がなくなった時TRUE
)

(fn `fGetNearPosition`
  (params (targetPosition :type "Vector Structure"))
  (returns (nearPosition :type "Vector Structure") (nearSection :type "/Game/Play/Building/Address/Section/BP_Section Object Reference"))
  (locals (nowPosition :type "Vector Structure") (nearLength :type "Float (double-precision)") (nowLength :type "Float (double-precision)") (nearAddressIndex :type Integer) (`save TragetPosition` :type "Vector Structure") (saveSize :type "/Game/Play/Building/Data/EN_BuildingSize Enum") (saveIndex :type Integer))
  (bind (_save_tragetposition_x _save_tragetposition_y _save_tragetposition_z) (`KismetMathLibrary.BreakVector` (`local.save TragetPosition`)))
  (bind (_save_tragetposition_x_2 _save_tragetposition_y_2 _save_tragetposition_z_2) (`KismetMathLibrary.BreakVector` (`local.save TragetPosition`)))
  (bind (_save_tragetposition_x_3 _save_tragetposition_y_3 _save_tragetposition_z_3) (`KismetMathLibrary.BreakVector` (`local.save TragetPosition`)))
  (bind (_save_tragetposition_x_4 _save_tragetposition_y_4 _save_tragetposition_z_4) (`KismetMathLibrary.BreakVector` (`local.save TragetPosition`)))
  (bind (_output_x _output_y) (break `/Game/Vector2` (`|GetArrayItem` (`self.mHousePosition`) (`local.nearAddressIndex`))))
  (bind (_value _returnvalue) (`BlueprintMapLibrary.Map_Find` (`self.mPositionToSection`) (make `/Game/Vector2` _output_x _output_y)))
  (bind (_output_x_2 _output_y_2) (break `/Game/Vector2` (`|GetArrayItem` (break `/Game/Play/Building/Address/ST_Vector2Array` (`BlueprintMapLibrary.Map_Find` (`self.mSaveSectionPos`) (`local.saveSize`))) (`local.nearAddressIndex`))))
  (bind (_value_2 _returnvalue_2) (`BlueprintMapLibrary.Map_Find` (`self.mPositionToSection`) (make `/Game/Vector2` _output_x_2 _output_y_2)))
  (bind _mbp_cursor (`/Game/Play/Building/BP_BuildingManager.mBP_Cursor` (`/Game/Play/Common/GameMode/GM_DestructionCity.mBP_BuildingManager` (cast `/Game/Play/Common/GameMode/GM_DestructionCity` (`GameplayStatics.GetGameMode`) :!pure true))))
  (bind _mnowselectbuilding (`/Game/Play/Building/Cursor/BP_Cursor.mNowSelectBuilding` _mbp_cursor))
  (set `local.save TragetPosition` targetPosition) ; 多く使用するためあらかじめ保存しておく
  (bind _value_size (`/Game/Play/Building/Cursor/BP_Cursor.fGetSelectBuildingSize` _mbp_cursor)) ; 現在選択中の建物のサイズを取得する
  (bind _output_get (set `local.saveSize` _value_size))
  (for (_array_element _array_index) (break `/Game/Play/Building/Address/ST_Vector2Array` (`BlueprintMapLibrary.Map_Find` (`self.mSaveSectionPos`) _output_get))
    (bind _value_3 (`BlueprintMapLibrary.Map_Find` (`self.mPositionToSection`) (make `/Game/Vector2` (break `/Game/Vector2` _array_element) (`.Y_5_6EC1BF83480F7C51E3838D9E040D7D37` (break `/Game/Vector2` _array_element)))))
    (`/Engine/EditorBlueprintResources/StandardMacros.IsValid` _value_3
      (:`Is Valid`
        (if (`/Game/Play/Building/Address/Section/BP_Section.mNotSelectFlag` _value_3)
          _
          (elif (`|EnumInequality` (`/Game/Play/Building/Address/Section/BP_Section.mState` _value_3) "NewEnumerator3")
            (if (`|EnumEquality` (`/Game/Play/Building/Address/Section/BP_Section.mBuildingSize` _value_3) (`local.saveSize`))
              (bind _output_get_2 (set `local.nowPosition` (`KismetMathLibrary.MakeVector` (break `/Game/Vector2` _array_element) (`.Y_5_6EC1BF83480F7C51E3838D9E040D7D37` (break `/Game/Vector2` _array_element)) _save_tragetposition_z))) ; 要素を取得、同時に3次元に
              (set `local.nowLength` (`KismetMathLibrary.VSizeXY` (- _output_get_2 (`local.save TragetPosition`)))) ; 現在選択されている座標とカーソル座標の距離
              ;[1 1 1] 最初なら保存
              (if (`KismetMathLibrary.NearlyEqual_FloatFloat` (`local.nearLength`))
                (set `local.nearLength` (`local.nowLength`) :!label _label)
                (set `local.nearAddressIndex` _array_index) ; 配列番号を保存
                (elif (> (`local.nearLength`) (`local.nowLength`))
                  (goto _label)))))))))
  (if (or (`|EnumEquality` _mnowselectbuilding "NewEnumerator0") (`|EnumEquality` _mnowselectbuilding "NewEnumerator2") (`|EnumEquality` _mnowselectbuilding "NewEnumerator4"))
    (set `local.saveIndex` (`local.nearAddressIndex`)) ; 一時保存
    (for (_array_element_2 _array_index_2) (`self.mHousePosition`)
      (bind _value_4 (`BlueprintMapLibrary.Map_Find` (`self.mPositionToSection`) (make `/Game/Vector2` (break `/Game/Vector2` _array_element_2) (`.Y_5_6EC1BF83480F7C51E3838D9E040D7D37` (break `/Game/Vector2` _array_element_2)))))
      (`/Engine/EditorBlueprintResources/StandardMacros.IsValid` _value_4
        (:`Is Valid`
          (if (`/Game/Play/Building/Address/Section/BP_Section.mNotSelectFlag` _value_4)
            _
            (elif (`|EnumEquality` (`/Game/Play/Building/Address/Section/BP_Section.mBuildingSize` _value_4) (`local.saveSize`))
              (bind _output_get_3 (set `local.nowPosition` (`KismetMathLibrary.MakeVector` 0.0 0.0 _save_tragetposition_z_3))) ; 要素を取得、同時に3次元に
              (set `local.nowLength` (`KismetMathLibrary.VSizeXY` (- _output_get_3 (`local.save TragetPosition`)))) ; 現在選択されている座標とカーソル座標の距離
              (if (> (`local.nearLength`) (`local.nowLength`))
                (set `local.nearAddressIndex` (+ _array_index_2 (`local.nearAddressIndex`))) ; 配列番号を保存
              ))))))
    (if (< (`KismetArrayLibrary.Array_Length` (break `/Game/Play/Building/Address/ST_Vector2Array` (`BlueprintMapLibrary.Map_Find` (`self.mSaveSectionPos`) "NewEnumerator0"))) (`local.saveIndex`))
      ;[1 1 1] 一番近い座標の区画情報を取得、返す
      (if _returnvalue
        (return (`KismetMathLibrary.MakeVector` _output_x _output_y _save_tragetposition_z_4) _value)
        (else
          (return (0.0 0.0 0.0) null)))
      (else
        _)))
  ;[1 1 1] 一番近い座標の区画情報を取得、返す
  (if _returnvalue_2
    (return (`KismetMathLibrary.MakeVector` _output_x_2 _output_y_2 _save_tragetposition_z_2) _value_2)
    (else
      (return (0.0 0.0 0.0) null))))

(fn `fSaveSectionPosition`
  (locals (instantArray :type "Array of /Game/Vector2 Structure"))
  ;[1 1 1] マップ変数に格納
  (for (_array_element _array_index) (`self.GetAllChildActors` false)
    (if (`KismetSystemLibrary.IsValid` _array_element)
      (bind (_returnvalue_x _returnvalue_y) (`KismetMathLibrary.BreakVector` (`self.K2_GetActorLocation` _array_element)))
      (`KismetArrayLibrary.Array_Add` (`local.instantArray`) (make `/Game/Vector2` _returnvalue_x _returnvalue_y))
      (`BlueprintMapLibrary.Map_Add` (`self.mSaveSectionPos`) (`/Game/Play/Building/Address/Section/BP_Section.mBuildingSize` (cast `/Game/Play/Building/Address/Section/BP_Section` _array_element :!pure true)) (make `/Game/Play/Building/Address/ST_Vector2Array` (`local.instantArray`)))
      (`BlueprintMapLibrary.Map_Add` (`self.mPositionToSection`) (make `/Game/Vector2` _returnvalue_x _returnvalue_y) (cast `/Game/Play/Building/Address/Section/BP_Section` (`|GetArrayItem` (`self.GetAllChildActors` false) _array_index) :!pure true)))))

(fn `UserConstructionScript`)