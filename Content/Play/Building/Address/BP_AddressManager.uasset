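; BP_AddressManager manages the city's BP_Address blocks and their building sections in the DestructionCity game.
; On BeginPlay it gathers every address, maps their sections by building size, and starts a looping timer that updates each address's grid lines.
; Helpers remove sections from that map and find the address or selectable section nearest a position in XY.
; FAddressTex runs each address's FSectionsTex and plays a coin sound if any reports success.
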(event `self.ReceiveBeginPlay`
  (`self.fAllAddressSet`)
  (`self.fSaveSectionPosition`)
  (`KismetSystemLibrary.K2_SetTimerDelegate` (delegate `ChangeGrid`) (`/Game/Play/Common/GameMode/GM_DestructionCity.DELTA_TIME` (cast `/Game/Play/Common/GameMode/GM_DestructionCity` (`GameplayStatics.GetGameMode`) :!pure true)) true))

(event `ChangeGrid`
  (for _array_element (`self.mAddress`)
    (`/Game/Play/Building/Address/BP_Address.ChangeGrid` _array_element)))

(fn `fAddressTex`
  (locals (createFlag :type Boolean))
  (for _array_element (`self.mAddress`)
    (bind _flag (`/Game/Play/Building/Address/BP_Address.F Sections Tex` _array_element))
    (if _flag
      (set `local.createFlag` true) ; 一つでも生成されたらフラグを建てる
    ))
  (if (`local.createFlag`)
    (`GameplayStatics.SpawnSound2D` "/Game/Play/Building/Sound/SE/SoundEffect_Coin.SoundEffect_Coin" 1.0 1.0 0.0 null) ; SEを鳴らす
    (set `/Game/Play/Building/Sound/BP_BuildingSoundManager.mSE_Coin` null (`/Game/Play/Building/BP_BuildingManager.mBP_BuildingSoundManager` (`/Game/Play/Common/GameMode/GM_DestructionCity.mBP_BuildingManager` (cast `/Game/Play/Common/GameMode/GM_DestructionCity` (`GameplayStatics.GetGameMode`) :!pure true))))))

(fn `fAllAddressSet`
  (bind _outactors (`GameplayStatics.GetAllActorsOfClass` "/Game/Play/Building/Address/BP_Address.BP_Address_C"))
  (set `self.mAddress` _outactors))

(fn `fDeleteSectionElementToArray`
  (params (SectionPosition :type "Array of /Game/Play/Building/Address/Section/BP_Section Object Reference"))
  (locals (insArray :type "Array of /Game/Play/Building/Address/Section/BP_Section Object Reference"))
  (bind _mmap (`self.mMap`))
  (for _array_element SectionPosition
    (bind _mbuildingsize (`/Game/Play/Building/Address/Section/BP_Section.mBuildingSize` _array_element))
    (bind _value (`BlueprintMapLibrary.Map_Find` _mmap _mbuildingsize))
    (bind _output_get (set `local.insArray` (break `/Game/Play/Building/Address/ST_SectionArray` _value)))
    (`KismetArrayLibrary.Array_RemoveItem` _output_get _array_element)
    (`KismetArrayLibrary.Array_Clear` (break `/Game/Play/Building/Address/ST_SectionArray` _value))
    (`BlueprintMapLibrary.Map_Add` _mmap _mbuildingsize (make `/Game/Play/Building/Address/ST_SectionArray` (`local.insArray`)))))

(fn `fDeleteSectionElementToPosition`
  (params (SectionPosition :type "Vector Structure"))
  (bind _enumvalue (foreach `/Game/Play/Building/Data/EN_BuildingSize` false)
    (:`LoopBody`
      (bind _value (`BlueprintMapLibrary.Map_Find` (`self.mMap`) _enumvalue))
      (for _array_element (break `/Game/Play/Building/Address/ST_SectionArray` _value)
        (if (== (`self.K2_GetActorLocation` _array_element) SectionPosition)
          (`KismetArrayLibrary.Array_RemoveItem` (break `/Game/Play/Building/Address/ST_SectionArray` _value) _array_element))))))

(fn `fGetNearPositionAddress`
  (params (targetPosition :type "Vector Structure"))
  (returns (NearAddress :type "/Game/Play/Building/Address/BP_Address Object Reference"))
  (locals (nowPosition :type "Vector Structure") (nearLength :type "Float (double-precision)") (nowLength :type "Float (double-precision)") (nearAddressIndex :type Integer) (`save TragetPosition` :type "Vector Structure") (saveSize :type "/Game/Play/Building/Data/EN_BuildingSize Enum") (saveIndex :type Integer))
  (bind (_save_tragetposition_x _save_tragetposition_y _save_tragetposition_z) (`KismetMathLibrary.BreakVector` (`local.save TragetPosition`)))
  (set `local.save TragetPosition` targetPosition) ; 多く使用するためあらかじめ保存しておく
  (for (_array_element _array_index) (`self.mAddress`)
    (bind (_returnvalue_x _returnvalue_y) (`KismetMathLibrary.BreakVector` (`self.K2_GetActorLocation` _array_element)))
    (bind _output_get (set `local.nowPosition` (`KismetMathLibrary.MakeVector` _returnvalue_x _returnvalue_y _save_tragetposition_z))) ; 要素を取得、同時に3次元に
    (set `local.nowLength` (`KismetMathLibrary.VSizeXY` (- _output_get (`local.save TragetPosition`)))) ; 現在選択されている座標とカーソル座標の距離
    ;[1 1 1] 最初なら保存
    (if (`KismetMathLibrary.NearlyEqual_FloatFloat` (`local.nearLength`))
      (set `local.nearLength` (`local.nowLength`) :!label _label)
      (set `local.nearAddressIndex` _array_index) ; 配列番号を保存
      (elif (> (`local.nearLength`) (`local.nowLength`))
        (goto _label))))
  (return (`|GetArrayItem` (`self.mAddress`) (`local.nearAddressIndex`))))

(fn `fGetNearPositionSection`
  (params (targetPosition :type "Vector Structure") (sections :type "Array of /Game/Play/Building/Address/Section/BP_Section Object Reference"))
  (returns (NearSection :type "/Game/Play/Building/Address/Section/BP_Section Object Reference"))
  (locals (nowPosition :type "Vector Structure") (nearLength :type "Float (double-precision)") (nowLength :type "Float (double-precision)") (nearAddressIndex :type Integer) (`save TragetPosition` :type "Vector Structure") (saveSize :type "/Game/Play/Building/Data/EN_BuildingSize Enum") (saveIndex :type Integer) (count :type Integer))
  (bind (_save_tragetposition_x _save_tragetposition_y _save_tragetposition_z) (`KismetMathLibrary.BreakVector` (`local.save TragetPosition`)))
  (set `local.save TragetPosition` targetPosition) ; 多く使用するためあらかじめ保存しておく
  (for (_array_element _array_index) sections
    (`/Engine/EditorBlueprintResources/StandardMacros.IsValid` _array_element
      (:`Is Valid`
        (if (`/Game/Play/Building/Address/Section/BP_Section.mNotSelectFlag` _array_element)
          _
          (elif (`|EnumInequality` (`/Game/Play/Building/Address/Section/BP_Section.mState` _array_element) "NewEnumerator3")
            (bind (_returnvalue_x _returnvalue_y) (`KismetMathLibrary.BreakVector` (`self.K2_GetActorLocation` _array_element)))
            (bind _output_get (set `local.nowPosition` (`KismetMathLibrary.MakeVector` _returnvalue_x _returnvalue_y _save_tragetposition_z))) ; 要素を取得、同時に3次元に
            (set `local.nowLength` (`KismetMathLibrary.VSizeXY` (- _output_get (`local.save TragetPosition`)))) ; 現在選択されている座標とカーソル座標の距離
            ;[1 1 1] 最初なら保存
            (if (`KismetMathLibrary.NearlyEqual_FloatFloat` (`local.nearLength`))
              (set `local.nearLength` (`local.nowLength`) :!label _label)
              (set `local.nearAddressIndex` _array_index) ; 配列番号を保存
              (elif (> (`local.nearLength`) (`local.nowLength`))
                (goto _label))))))))
  (return (`|GetArrayItem` sections (`local.nearAddressIndex`))))

(fn `fSaveSectionPosition`
  (locals (array :type "Array of /Game/Play/Building/Address/Section/BP_Section Object Reference"))
  (bind _array (`local.array`))
  (bind _enumvalue (foreach `/Game/Play/Building/Data/EN_BuildingSize` false)
    (:`LoopBody`
      (for _array_element (`self.mAddress`)
        (for _array_element_2 (`/Game/Play/Building/Address/BP_Address.mSections` _array_element)
          (`/Engine/EditorBlueprintResources/StandardMacros.IsValid` _array_element_2
            (:`Is Valid`
              (if (`|EnumEquality` (`/Game/Play/Building/Address/Section/BP_Section.mBuildingSize` _array_element_2) _enumvalue)
                (`KismetArrayLibrary.Array_Add` (`local.array`) _array_element_2))))))
      (`BlueprintMapLibrary.Map_Add` (`self.mMap`) _enumvalue (make `/Game/Play/Building/Address/ST_SectionArray` _array))
      (`KismetArrayLibrary.Array_Clear` _array))))

(fn `UserConstructionScript`)