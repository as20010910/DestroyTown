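; Building-phase preprocessing actor that runs the start countdown before building begins.
; BeginPlay creates the countdown widget, blacks out the screen and starts the GameMode's fade, then polls on a looping timer until it ends.
; It then plays the countdown sound, hands it to the building sound manager, and ticks the number down every second.
; Below zero, it removes the widget and sets MFinish.
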(event `self.ReceiveBeginPlay`
  (bind _asgm_destruction_city (cast `/Game/Play/Common/GameMode/GM_DestructionCity` (`GameplayStatics.GetGameMode`) :!pure true))
  (bind _mwbp_fade (`/Game/Play/Common/GameMode/GM_DestructionCity.mWBP_Fade` _asgm_destruction_city))
  ;[1 1 1] 開始カウントダウン
  (bind _returnvalue (`|CreateWidget` "/Game/Play/Building/UI/CountDown/WBP_BuildingCountDown.WBP_BuildingCountDown_C")) ; 開始カウントダウン
  (bind _output_get (set `self.mWBP_CountDown` _returnvalue))
  (`UserWidget.AddToViewport` _output_get 0)
  (`/Game/Play/Building/UI/CountDown/WBP_BuildingCountDown.fSetDrawString` _output_get "NewEnumerator0")
  (`/Game/Play/Common/Fade/WBP_Fade.BlackOut` _mwbp_fade) ; 画面黒塗り
  (`/Game/Play/Common/Fade/WBP_Fade.FadeInitialize` _mwbp_fade "NewEnumerator1" 0.02)
  (bind _returnvalue_2 (`KismetSystemLibrary.K2_SetTimerDelegate` (delegate `FadeStandBy`) (`/Game/Play/Common/GameMode/GM_DestructionCity.DELTA_TIME` _asgm_destruction_city) true)))

(event `FadeStandBy`
  (if (`/Game/Play/Common/Fade/WBP_Fade.mEnd` (`/Game/Play/Common/GameMode/GM_DestructionCity.mWBP_Fade` (cast `/Game/Play/Common/GameMode/GM_DestructionCity` (`GameplayStatics.GetGameMode`) :!pure true)))
    (`KismetSystemLibrary.K2_SetTimerDelegate` (delegate `CountDown`) 1.0 true)
    (bind _returnvalue (`GameplayStatics.SpawnSound2D` "/Game/Play/Building/Sound/SE/SoundEffect_Countdown.SoundEffect_Countdown" 1.0 1.0 0.0 null)) ; カウントダウンSEを流す
    (set `/Game/Play/Building/Sound/BP_BuildingSoundManager.mSE_Countdown` _returnvalue (`/Game/Play/Building/BP_BuildingManager.mBP_BuildingSoundManager` (`/Game/Play/Common/GameMode/GM_DestructionCity.mBP_BuildingManager` (cast `/Game/Play/Common/GameMode/GM_DestructionCity` (`GameplayStatics.GetGameMode`) :!pure true))))
    (`KismetSystemLibrary.K2_ClearAndInvalidateTimerHandle` (stale `self.ReceiveBeginPlay` _returnvalue_2)) ; 事前処理が終わったら処理をする
    (set `/Game/Play/Building/UI/CountDown/WBP_BuildingCountDown.mCountDownNum` (`self.mCountDownNum`) (`self.mWBP_CountDown`)) ; カウントダウン初期値設定
  ))

(event `CountDown`
  (bind _result (`/Engine/EditorBlueprintResources/StandardMacros.DecrementInt` (`self.mCountDownNum`))
    (:`  `
      (bind _output_get (set `/Game/Play/Building/UI/CountDown/WBP_BuildingCountDown.mCountDownNum` _result (`self.mWBP_CountDown`))) ; UI表示を更新
      (if (< _output_get 0)
        (`Widget.RemoveFromParent` (`self.mWBP_CountDown`)) ; UIを消す
        (set `self.mFinish` true)))))

(fn `fPreprocessingUpdate`
  (if true
    _))

(fn `UserConstructionScript`)