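; BP_Camera is a camera actor for the game's building controller, with input-driven zoom on a spring arm.
; Zoom in and out actions step the arm length by a zoom speed, clamped between minimum and maximum lengths.
; Forward and right axis events are empty, as their local-offset movement nodes are left disconnected and never run.
; Tick prints the actor's location as debug output.
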(event `InputAxis|CameraMoveForward`
  (params (AxisValue :type "Float (single-precision)"))
  ;[1 1 1] カメラの移動
)

(event `InputAxis|CameraMoveRight`
  (params (AxisValue :type "Float (single-precision)"))
  ;[1 1 1] カメラの移動
)

(event `InputAction|CameraZoomIn`
  (params (Key :type "Key Structure"))
  ;[1 1 1] カメラのズーム
  (:`Pressed`
    (set `SpringArmComponent.TargetArmLength` (`KismetMathLibrary.FClamp` (- (`SpringArmComponent.TargetArmLength` (`self.SpringArm`)) (`self.mCameraZoomSpeed`)) (`self.mMinTargetLength`) (`self.mMaxTargetLength`)) (`self.SpringArm`)) ; スプリングアームの長さを短くしズームインする
  ))

(event `InputAction|CameraZoomOut`
  (params (Key :type "Key Structure"))
  ;[1 1 1] カメラのズーム
  (:`Pressed`
    (set `SpringArmComponent.TargetArmLength` (`KismetMathLibrary.FClamp` (+ (`SpringArmComponent.TargetArmLength` (`self.SpringArm`)) (`self.mCameraZoomSpeed`)) (`self.mMinTargetLength`) (`self.mMaxTargetLength`)) (`self.SpringArm`)) ; スプリングアームの長さを長くしズームアウトする
  ))

(event `self.ReceiveTick`
  (params (DeltaSeconds :type "Float (single-precision)"))
  (`KismetSystemLibrary.PrintString` (`KismetStringLibrary.Conv_VectorToString` (`self.K2_GetActorLocation`))))

(fn `UserConstructionScript`)