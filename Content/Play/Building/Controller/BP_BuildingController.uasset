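; Building-mode controller that spawns and possesses the camera, registers a cursor with the building manager, and handles build and selection actions.
; Move functions accumulate a velocity that a looping timer eases into the camera position and decays.
; FBuilding builds or develops the cursor's selected section, then runs an overlap check on its address.
; Zoom and switch functions step the building selection and refresh the info gauge; the original spring-arm zoom code is unreachable.
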(event `self.ReceiveBeginPlay`
  (bind _returnvalue (`|SpawnActorFromClass` "/Game/Play/Building/Controller/BP_Camera.BP_Camera_C" (`KismetMathLibrary.MakeTransform` (0.0 0.0 0.0)) "Undefined" "OverrideRootScale" null null)) ; カメラ生成
  (bind _output_get (set `self.mBP_Camera` _returnvalue))
  (`Controller.Possess` (`GameplayStatics.GetPlayerController` 0) _output_get) ; カメラ接続
  (`KismetSystemLibrary.K2_SetTimerDelegate` (delegate `CameraUpdate`) (`/Game/Play/Common/GameMode/GM_DestructionCity.DELTA_TIME` (cast `/Game/Play/Common/GameMode/GM_DestructionCity` (`GameplayStatics.GetGameMode`) :!pure true)) true) ; カメラ更新処理
  (bind _returnvalue_2 (`|SpawnActorFromClass` "/Game/Play/Building/Cursor/BP_Cursor.BP_Cursor_C" (`KismetMathLibrary.MakeTransform` (0.0 0.0 0.0)) "Undefined" "OverrideRootScale" null null)) ; カーソル作成
  (set `/Game/Play/Building/BP_BuildingManager.mBP_Cursor` _returnvalue_2 (`/Game/Play/Common/GameMode/GM_DestructionCity.mBP_BuildingManager` (cast `/Game/Play/Common/GameMode/GM_DestructionCity` (`GameplayStatics.GetGameMode`) :!pure true))))

(event `CameraUpdate`
  (if (`KismetSystemLibrary.IsValid` (`self.mBP_Camera`))
    (`self.fCameraUpdate`)))

(fn `fBuilding`
  (locals (section :type "/Game/Play/Building/Address/Section/BP_Section Object Reference"))
  (bind _section (`local.section`))
  (bind _section_2 (`local.section`))
  (bind _mbp_cursor (`/Game/Play/Building/BP_BuildingManager.mBP_Cursor` (`/Game/Play/Common/GameMode/GM_DestructionCity.mBP_BuildingManager` (cast `/Game/Play/Common/GameMode/GM_DestructionCity` (`GameplayStatics.GetGameMode`) :!pure true))))
  (bind _mselectsection (`/Game/Play/Building/Cursor/BP_Cursor.mSelectSection` _mbp_cursor))
  (bind _mselectaddress (`/Game/Play/Building/Cursor/BP_Cursor.mSelectAddress` _mbp_cursor))
  (`/Engine/EditorBlueprintResources/StandardMacros.IsValid` _mselectsection
    (:`Is Valid`
      (bind _output_get (set `local.section` _mselectsection))
      ;[1 1 1] 建っているものが家かどうか
      (bind _houseflag (`/Game/Play/Building/Address/Section/BP_Section.fIsHouse` _output_get))
      (if _houseflag
        (`/Game/Play/Building/Address/Section/BP_Section.SetDevelopment` (`local.section`))
        (`/Game/Play/Building/Address/BP_Address.fChackOverlapSecitons` _mselectaddress _section_2 true :!label _label) ; 家以外ならこっち
        (else
          (`/Game/Play/Building/Address/Section/BP_Section.SetBuilding` _section) ; それ以外なら家を建てる処理
          (if (`|EnumEquality` (`/Game/Play/Building/Address/Section/BP_Section.mState` _section) "NewEnumerator1")
            (goto _label)
            (else
              (`/Game/Play/Building/Address/BP_Address.fChackOverlapSecitons` _mselectaddress _section_2 false) ; 家ならこっち
            )))))))

(fn `fCameraMoveForward`
  (params (`Axis Value` :type "Float (double-precision)"))
  (bind _returnvalue (`KismetMathLibrary.MakeVector` (* `Axis Value` (`/Game/Play/Building/Controller/BP_Camera.mCameraMoveSpeed` (`self.mBP_Camera`)))))
  ;[1 1 1] カメラの移動
  ;;[1 1 1] 値が入っているときのみ処理
  (if (`KismetMathLibrary.NotEqualExactly_VectorVector` _returnvalue)
    (set `self.mSaveCameraMoveVel` (+ _returnvalue (`self.mSaveCameraMoveVel`)))
    (set `self.mTargetCameraVel` (+ _returnvalue (`self.K2_GetActorLocation` (`self.mBP_Camera`))))))

(fn `fCameraMoveRight`
  (params (`Axis Value` :type "Float (double-precision)"))
  (bind _returnvalue (`KismetMathLibrary.MakeVector` 0.0 (* `Axis Value` (`/Game/Play/Building/Controller/BP_Camera.mCameraMoveSpeed` (`self.mBP_Camera`)))))
  ;[1 1 1] カメラの移動
  ;;[1 1 1] 値が入っているときのみ処理
  (if (`KismetMathLibrary.NotEqualExactly_VectorVector` _returnvalue)
    (set `self.mSaveCameraMoveVel` (+ _returnvalue (`self.mSaveCameraMoveVel`)))
    (set `self.mTargetCameraVel` (+ _returnvalue (`self.K2_GetActorLocation` (`self.mBP_Camera`))))))

(fn `fCameraUpdate`
  (locals (SPRING_ARM :type "Float (double-precision)" :default 0.08))
  (bind _msavecameramovevel (`self.mSaveCameraMoveVel`))
  (bind _returnvalue (`self.K2_GetActorLocation` (`self.mBP_Camera`)))
  (if (`KismetMathLibrary.NotEqualExactly_VectorVector` (`self.mSaveCameraMoveVel`))
    (`self.K2_SetActorLocation` (`self.mBP_Camera`) (`KismetMathLibrary.VLerp` _returnvalue (+ _returnvalue (`self.mSaveCameraMoveVel`)) (`local.SPRING_ARM`)) false true)
    (set `self.mSaveCameraMoveVel` (- _msavecameramovevel (* _msavecameramovevel (`local.SPRING_ARM`))))))

(fn `fCameraZoomIn`
  (bind _mbp_buildingmanager (`/Game/Play/Common/GameMode/GM_DestructionCity.mBP_BuildingManager` (cast `/Game/Play/Common/GameMode/GM_DestructionCity` (`GameplayStatics.GetGameMode`) :!pure true)))
  (bind _mbp_selectbuildingmanager (`/Game/Play/Building/BP_BuildingManager.mBP_SelectBuildingManager` _mbp_buildingmanager))
  ;[1 1 1] 一番上じゃなければ処理をする
  (if (`|EnumInequality` (`/Game/Play/Building/UI/SelectBuilding/BP_SelectBuildingManager.mBuildingAttributesState` _mbp_selectbuildingmanager) "NewEnumerator0")
    (`/Game/Play/Building/UI/SelectBuilding/BP_SelectBuildingManager.fSelectLeft` _mbp_selectbuildingmanager)
    (`/Game/Play/Building/UI/BuildingInfo/WBP_BuildingInfo.fChangeGauge` (`/Game/Play/Building/BP_BuildingManager.mWBP_BuildingInfo` _mbp_buildingmanager))))

(fn `fCameraZoomOut`
  (bind _mbp_buildingmanager (`/Game/Play/Common/GameMode/GM_DestructionCity.mBP_BuildingManager` (cast `/Game/Play/Common/GameMode/GM_DestructionCity` (`GameplayStatics.GetGameMode`) :!pure true)))
  (bind _mbp_selectbuildingmanager (`/Game/Play/Building/BP_BuildingManager.mBP_SelectBuildingManager` _mbp_buildingmanager))
  ;[1 1 1] 一番下じゃなければ処理をする
  (if (`|EnumInequality` (`/Game/Play/Building/UI/SelectBuilding/BP_SelectBuildingManager.mBuildingAttributesState` _mbp_selectbuildingmanager) "NewEnumerator2")
    (`/Game/Play/Building/UI/SelectBuilding/BP_SelectBuildingManager.fSelectRight` _mbp_selectbuildingmanager)
    (`/Game/Play/Building/UI/BuildingInfo/WBP_BuildingInfo.fChangeGauge` (`/Game/Play/Building/BP_BuildingManager.mWBP_BuildingInfo` _mbp_buildingmanager))))

(fn `fSwitchLeftBuildingAttributes`
  (bind _mbp_buildingmanager (`/Game/Play/Common/GameMode/GM_DestructionCity.mBP_BuildingManager` (cast `/Game/Play/Common/GameMode/GM_DestructionCity` (`GameplayStatics.GetGameMode`) :!pure true)))
  (bind _mbp_selectbuildingmanager (`/Game/Play/Building/BP_BuildingManager.mBP_SelectBuildingManager` _mbp_buildingmanager))
  ;[1 1 1] 一番左じゃなければ処理をする
  (if (`|EnumInequality` (`/Game/Play/Building/UI/SelectBuilding/BP_SelectBuildingManager.mSelectBuildingState` _mbp_selectbuildingmanager) "NewEnumerator0")
    (`/Game/Play/Building/UI/SelectBuilding/BP_SelectBuildingManager.F Wheel Up` _mbp_selectbuildingmanager)
    (`/Game/Play/Building/UI/BuildingInfo/WBP_BuildingInfo.fChangeGauge` (`/Game/Play/Building/BP_BuildingManager.mWBP_BuildingInfo` _mbp_buildingmanager))))

(fn `fSwitchRightBuildingAttributes`
  (bind _mbp_buildingmanager (`/Game/Play/Common/GameMode/GM_DestructionCity.mBP_BuildingManager` (cast `/Game/Play/Common/GameMode/GM_DestructionCity` (`GameplayStatics.GetGameMode`) :!pure true)))
  (bind _mbp_selectbuildingmanager (`/Game/Play/Building/BP_BuildingManager.mBP_SelectBuildingManager` _mbp_buildingmanager))
  ;[1 1 1] 一番右じゃなければ処理をする
  (if (`|EnumInequality` (`/Game/Play/Building/UI/SelectBuilding/BP_SelectBuildingManager.mSelectBuildingState` _mbp_selectbuildingmanager) "NewEnumerator2")
    (`/Game/Play/Building/UI/SelectBuilding/BP_SelectBuildingManager.F Wheel Down` _mbp_selectbuildingmanager)
    (`/Game/Play/Building/UI/BuildingInfo/WBP_BuildingInfo.fChangeGauge` (`/Game/Play/Building/BP_BuildingManager.mWBP_BuildingInfo` _mbp_buildingmanager))))

(fn `UserConstructionScript`)