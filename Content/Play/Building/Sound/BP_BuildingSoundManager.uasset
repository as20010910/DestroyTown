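; Sound manager for the building part of the game, owning its BGM, a daily-life ambience and positional effects for building, car and facility sounds.
; BeginPlay starts the two 2D sounds; FUpVolumeDailyLife raises the ambience in capped steps.
; FCreateSound pools audio components per sound type, replaying an idle one or spawning another, and returns its index.
; That index lets callers move or fetch a sound; FDestroySound destroys all pooled components.
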(event `self.ReceiveBeginPlay`
  (bind _returnvalue (`GameplayStatics.SpawnSound2D` "/Game/Play/Building/Sound/BGM/BGM_Building.BGM_Building" 1.0 1.0 0.0 null)) ; BGM作成
  (set `self.mBGM_Building` _returnvalue)
  (bind _returnvalue_2 (`GameplayStatics.SpawnSound2D` "/Game/Play/Building/Sound/SE/SoundEffect_DailyLife.SoundEffect_DailyLife" 0.01 1.0 0.0 null)) ; 生活音作成(疑似無音)
  (set `self.mSE_DailyLife` _returnvalue_2))

(fn `fCreateSound`
  (params (SoundType :type "/Game/Play/Building/Sound/EN_BuildingSoundArray Enum" :default "NewEnumerator0") (Location :type "Vector Structure"))
  (returns (index :type Integer))
  (locals (instantArray :type "Array of AudioComponent Object Reference") (sound :type "SoundBase Object Reference") (instant :type "AudioComponent Object Reference") (saveIndex :type Integer))
  (bind _instantarray (`local.instantArray`))
  ;[1 1 1] 列挙型に合った音を設定する
  (switch `/Game/Play/Building/Sound/EN_BuildingSoundArray` SoundType
    (:`NewEnumerator4`
      (set `local.sound` "/Game/Play/Building/Sound/SE/SoundEffect_Building.SoundEffect_Building")
      (set `local.instantArray` (`self.mSE_Building`)))
    (:`NewEnumerator0`
      (set `local.sound` "/Game/Play/Building/Sound/SE/SoundEffect_BuildingCompleted.SoundEffect_BuildingCompleted")
      (bind _output_get (set `local.instantArray` (`self.mSE_BuildingCompleted`))))
    (:`NewEnumerator5`
      (set `local.sound` "/Game/Play/Building/Sound/SE/SoundEffect_Car.SoundEffect_Car")
      (set `local.instantArray` (`self.mSE_Car`)))
    (:`NewEnumerator6`
      (set `local.sound` "/Game/Play/Building/Sound/SE/SoundEffect_Laboratory.SoundEffect_Laboratory")
      (set `local.instantArray` (`self.mSE_Laboratory`)))
    (:`NewEnumerator7`
      (set `local.sound` "/Game/Play/Building/Sound/SE/SoundEffect_Sawmill.SoundEffect_Sawmill")
      (set `local.instantArray` (`self.mSE_Sawmill`)))
    (:`NewEnumerator8`
      (set `local.sound` "/Game/Play/Building/Sound/SE/SoundEffect_School.SoundEffect_School")
      (set `local.instantArray` (`self.mSE_School`))))
  (for (_array_element _array_index) _output_get
    (if (not (`AudioComponent.IsPlaying` _array_element))
      (`SceneComponent.K2_SetWorldLocation` _array_element Location false true)
      (`AudioComponent.Play` _array_element 0.0)
      (set `local.saveIndex` _array_index)
      ;[1 1 1] 再設定する
      (switch `/Game/Play/Building/Sound/EN_BuildingSoundArray` SoundType :!label _label
        (:`NewEnumerator4`
          (set `self.mSE_Building` _instantarray))
        (:`NewEnumerator0`
          (set `self.mSE_BuildingCompleted` _instantarray))
        (:`NewEnumerator5`
          (set `self.mSE_Car` _instantarray))
        (:`NewEnumerator6`
          (set `self.mSE_Laboratory` _instantarray))
        (:`NewEnumerator7`
          (set `self.mSE_Sawmill` _instantarray))
        (:`NewEnumerator8`
          (set `self.mSE_School` _instantarray)))
      (return (`local.saveIndex`))))
  (bind _returnvalue (`GameplayStatics.SpawnSoundAtLocation` (`local.sound`) Location (struct) 1.0 1.0 0.0 "/Game/Play/Building/Sound/test.test" null false))
  (bind _returnvalue_2 (`KismetArrayLibrary.Array_Add` (`local.instantArray`) _returnvalue)) ; 配列を追加
  (set `local.saveIndex` _returnvalue_2)
  (goto _label))

(fn `fDestroySound`
  (`|ExecutionSequence`
    (:`then_0`
      (for _array_element (`self.mSE_Building`)
        (`ActorComponent.K2_DestroyComponent` _array_element)))
    (:`then_1`
      (for _array_element_2 (`self.mSE_BuildingCompleted`)
        (`ActorComponent.K2_DestroyComponent` _array_element_2)))
    (:`then_2`
      (for _array_element_3 (`self.mSE_Car`)
        (`ActorComponent.K2_DestroyComponent` _array_element_3)))
    (:`then_3`
      (for _array_element_4 (`self.mSE_Laboratory`)
        (`ActorComponent.K2_DestroyComponent` _array_element_4)))
    (:`then_4`
      (for _array_element_5 (`self.mSE_Sawmill`)
        (`ActorComponent.K2_DestroyComponent` _array_element_5)))
    (:`then_5`
      (for _array_element_6 (`self.mSE_School`)
        (`ActorComponent.K2_DestroyComponent` _array_element_6)))))

(fn `fGetSoundArray`
  (params (Sound :type "/Game/Play/Building/Sound/EN_BuildingSoundArray Enum" :default "NewEnumerator4") (index :type Integer))
  (returns (SoundValue :type "AudioComponent Object Reference"))
  (locals (i :type Integer))
  (set `local.i` index)
  (switch `/Game/Play/Building/Sound/EN_BuildingSoundArray` Sound
    (:`NewEnumerator4`
      (return (`|GetArrayItem` (`self.mSE_Building`) (`local.i`))))
    (:`NewEnumerator0`
      (return (`|GetArrayItem` (`self.mSE_BuildingCompleted`) (`local.i`))))
    (:`NewEnumerator5`
      (return (`|GetArrayItem` (`self.mSE_Car`) (`local.i`))))
    (:`NewEnumerator6`
      (return (`|GetArrayItem` (`self.mSE_Laboratory`) (`local.i`))))
    (:`NewEnumerator7`
      (return (`|GetArrayItem` (`self.mSE_Sawmill`) (`local.i`))))
    (:`NewEnumerator8`
      (return (`|GetArrayItem` (`self.mSE_School`) (`local.i`))))))

(fn `fMoveSound`
  (params (Sound :type "/Game/Play/Building/Sound/EN_BuildingSoundArray Enum" :default "NewEnumerator0") (index :type Integer) (NewLocation :type "Vector Structure"))
  (locals (location :type "Vector Structure") (i :type Integer))
  (set `local.location` NewLocation)
  (set `local.i` index)
  (switch `/Game/Play/Building/Sound/EN_BuildingSoundArray` Sound
    (:`NewEnumerator4`
      (`SceneComponent.K2_SetWorldLocation` (`|GetArrayItem` (`self.mSE_Building`) (`local.i`)) (`local.location`) false true))
    (:`NewEnumerator0`
      (`SceneComponent.K2_SetWorldLocation` (`|GetArrayItem` (`self.mSE_BuildingCompleted`) (`local.i`)) (`local.location`) false true))
    (:`NewEnumerator5`
      (`SceneComponent.K2_SetWorldLocation` (`|GetArrayItem` (`self.mSE_Car`) (`local.i`)) (`local.location`) false true))
    (:`NewEnumerator6`
      (`SceneComponent.K2_SetWorldLocation` (`|GetArrayItem` (`self.mSE_Laboratory`) (`local.i`)) (`local.location`) false true))
    (:`NewEnumerator7`
      (`SceneComponent.K2_SetWorldLocation` (`|GetArrayItem` (`self.mSE_Sawmill`) (`local.i`)) (`local.location`) false true))
    (:`NewEnumerator8`
      (`SceneComponent.K2_SetWorldLocation` (`|GetArrayItem` (`self.mSE_School`) (`local.i`)) (`local.location`) false true))))

(fn `fUpVolumeDailyLife`
  (locals (UP_NUM :type "Float (double-precision)" :default 0.005) (MAX_NUM :type "Float (double-precision)" :default 0.065))
  (bind _mse_dailylife (`self.mSE_DailyLife`))
  (if (< (`AudioComponent.VolumeMultiplier` (`self.mSE_DailyLife`)) (`local.MAX_NUM`))
    (bind _output_get (set `self.mNowDailyLifeVolume` (+ (`self.mNowDailyLifeVolume`) (`local.UP_NUM`)))) ; 音量を上げる
    (if (> _output_get (`local.MAX_NUM`))
      (set `self.mNowDailyLifeVolume` (`local.MAX_NUM`)) ; 音量を上げる
    )
    (`AudioComponent.SetVolumeMultiplier` _mse_dailylife (`self.mNowDailyLifeVolume`))
    (`KismetSystemLibrary.PrintString` (`KismetStringLibrary.Conv_DoubleToString` (`AudioComponent.VolumeMultiplier` _mse_dailylife)))))

(fn `UserConstructionScript`)