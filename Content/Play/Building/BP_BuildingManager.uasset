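; Manager for the city-building phase, running it from preprocessing through a timed countdown to fade-out and cleanup.
; Polls BP_BuildingPreprocessing until finished, then spawns sub-managers (data, address, car, selection, events) and the HUD.
; Looping timers drive population-based car spawning, pause-gated tax collection and the countdown with sound.
; At time-up it clears UI, grid lines, icons and effects, saving money and population to the GameInstance for mayor stat upgrades.
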(event `BuildingInitialize`
  ;[1 1 1] 音管理マネージャの作成
  (bind _returnvalue (`|SpawnActorFromClass` "/Game/Play/Building/Sound/BP_BuildingSoundManager.BP_BuildingSoundManager_C" (`KismetMathLibrary.MakeTransform` (0.0 0.0 0.0)) "Undefined" "OverrideRootScale" null null))
  (bind _output_get (set `self.mBP_BuildingSoundManager` _returnvalue))
  (`/Game/Play/Building/Sound/BP_BuildingSoundManager.VolumeUpdateSE` _output_get)
  (`self.fDeleteBlackBox`)
  (bind _returnvalue_2 (`|SpawnActorFromClass` "/Game/Play/Building/BP_BuildingPreprocessing.BP_BuildingPreprocessing_C" (`KismetMathLibrary.MakeTransform` (0.0 0.0 0.0)) "Undefined" "OverrideRootScale" null null))
  (set `self.mBP_BuildingPreprocessing` _returnvalue_2)
  (bind _returnvalue_3 (`KismetSystemLibrary.K2_SetTimerDelegate` (delegate `BuildingPreprocessing`) (`/Game/Play/Common/GameMode/GM_DestructionCity.DELTA_TIME` (cast `/Game/Play/Common/GameMode/GM_DestructionCity` (`GameplayStatics.GetGameMode`) :!pure true)) true)) ; 事前処理
)

(event `BuildingPreprocessing`
  (bind _mbp_buildingpreprocessing (`self.mBP_BuildingPreprocessing`))
  (`/Game/Play/Building/BP_BuildingPreprocessing.fPreprocessingUpdate` _mbp_buildingpreprocessing)
  (if (`/Game/Play/Building/BP_BuildingPreprocessing.mFinish` _mbp_buildingpreprocessing)
    (`KismetSystemLibrary.K2_ClearAndInvalidateTimerHandle` (stale `BuildingInitialize` _returnvalue_3)) ; 事前処理が終わったら処理をする
    (`/Game/Play/Building/Controller/BP_BuildingController.BuildingControllerInitialize` (`/Game/Play/Common/Controller/PC_DestructionCity.mBP_BuildingController` (cast `/Game/Play/Common/Controller/PC_DestructionCity` (`GameplayStatics.GetPlayerController` 0) :!pure true))) ; 操作関連の初期化処理
    (`self.fCreateManager`) ; 管理マネージャの作成
    (`self.fCreateUI`) ; UI作成処理
    (`/Game/Play/Building/Sound/BP_BuildingSoundManager.VolumeUpdateBGM` (`self.mBP_BuildingSoundManager`))
    ;[1 1 1] 車生成処理
    (`KismetSystemLibrary.K2_SetTimerDelegate` (delegate `CarCreateUpdate`) (`/Game/Play/Common/GameMode/GM_DestructionCity.DELTA_TIME` (cast `/Game/Play/Common/GameMode/GM_DestructionCity` (`GameplayStatics.GetGameMode`) :!pure true)) true)
    ;[1 1 1] 税金処理
    (bind _returnvalue (`|SpawnActorFromClass` "/Game/Play/Common/GroundObject/BP_Timer.BP_Timer_C" (`KismetMathLibrary.MakeTransform` (0.0 0.0 0.0)) "Undefined" "OverrideRootScale" null null))
    (bind _output_get (set `self.mTexTimer` _returnvalue))
    (`/Game/Play/Common/GroundObject/BP_Timer.fSetMaxTime` _output_get (`self.TEX_TIME`))
    (bind _returnvalue_2 (`KismetSystemLibrary.K2_SetTimerDelegate` (delegate `TexUpdate`) (`/Game/Play/Common/GameMode/GM_DestructionCity.DELTA_TIME` (cast `/Game/Play/Common/GameMode/GM_DestructionCity` (`GameplayStatics.GetGameMode`) :!pure true)) true))
    (bind _returnvalue_3 (`KismetSystemLibrary.K2_SetTimerDelegate` (delegate `TimeCount`) 1.0 true))))

(event `CarCreateUpdate`
  ;[1 1 1] 車生成処理
  (if (>= (`self.mCarPeopleCountNum`) (`self.CAR_CREATE_PEOPLE_NUM`))
    (`self.fCarCreateCount`)))

(event `TexUpdate`
  ;[1 1 1] 税金処理
  (if (`self.ChackPause`)
    (bind _newparam (`/Game/Play/Common/GroundObject/BP_Timer.fCountUp` (`self.mTexTimer`) (`/Game/Play/Common/GameMode/GM_DestructionCity.DELTA_TIME` (cast `/Game/Play/Common/GameMode/GM_DestructionCity` (`GameplayStatics.GetGameMode`) :!pure true))))
    (if _newparam
      (`/Game/Play/Building/Address/BP_AddressManager.fAddressTex` (`self.mBP_AddressManager`)) ; 税金回収Effect作成処理
    )))

(event `TimeCount`
  ;[1 1 1] カウントダウン処理
  (if (`self.ChackPause`)
    (if (> (`self.mTimeLimit`) 0)
      (bind _result (`/Engine/EditorBlueprintResources/StandardMacros.DecrementInt` (`self.mTimeLimit`))
        (:`  `
          (bind _output_get (set `self.mTimeLimit` _result))
          (`self.fSetCountDownSound`)
          (set `/Game/Play/Building/UI/CountDown/WBP_BuildingCountDown.mCountDownNum` _output_get (`self.mWBP_BuildingCountdown`)) ; UI表示を更新
        ))
      (else
        ;;[1 1 1] 終了時処理
        (set `self.mFadeStartFlag` true)
        (`KismetSystemLibrary.K2_ClearAndInvalidateTimerHandle` (stale `BuildingPreprocessing` _returnvalue_3))
        (`KismetSystemLibrary.K2_ClearAndInvalidateTimerHandle` (stale `BuildingPreprocessing` _returnvalue_2))
        ;[1 1 1] 建築シーン最終フェード処理
        (`KismetSystemLibrary.K2_SetTimerDelegate` (delegate `FinishFade`) (`/Game/Play/Common/GameMode/GM_DestructionCity.DELTA_TIME` (cast `/Game/Play/Common/GameMode/GM_DestructionCity` (`GameplayStatics.GetGameMode`) :!pure true)) true)))
    (else
      (bind (_returnvalue _mse_countdown) (`self.ChackCountDownSE`)
        (:`Is Valid`
          (if _returnvalue
            (`AudioComponent.Stop` _mse_countdown)))))))

(event `FinishFade`
  (bind _mwbp_fade (`/Game/Play/Common/GameMode/GM_DestructionCity.mWBP_Fade` (cast `/Game/Play/Common/GameMode/GM_DestructionCity` (`GameplayStatics.GetGameMode`) :!pure true)))
  ;[1 1 1] 建築シーン最終フェード処理
  (if (`self.mFadeStartFlag`)
    (`/Game/Play/Common/Fade/WBP_Fade.FadeInitialize` _mwbp_fade "NewEnumerator0" 0.01)
    (set `self.mFadeStartFlag` false)
    (elif (`/Game/Play/Common/Fade/WBP_Fade.mEnd` _mwbp_fade)
      (set `self.mFinish` true)
      (`self.Finalize`) ; 破棄前の最終処理
    )))

(event `Finalize`
  (`self.fSetStatusUpValue`) ; 市長のステータスアップに必要な情報をセット
  (`self.AllGridDelete`) ; 全てのグリッド線を消す
  (`/Game/Play/Building/Sound/BP_BuildingSoundManager.fAllSoundFadeOut` (`self.mBP_BuildingSoundManager`)) ; 音量を下げる処理
  (`self.fDeleteUI`) ; UIをすべて消す
  (`self.fDeleteCursor`) ; カーソル削除処理
  (`self.DeleteIcon`) ; 発展アイコン削除処理
  (`self.DeleteAllEffect`) ; エフェクトの削除処理
)

(event `AllGridDelete`
  (bind _outactors (`GameplayStatics.GetAllActorsOfClass` "/Game/Play/Building/Address/GridLine/BP_GridLine.BP_GridLine_C"))
  (for _array_element _outactors
    (`/Game/Play/Building/Address/GridLine/BP_GridLine.HIddonGridLine` _array_element)))

(event `AllBuildingCreate`
  (bind _outactors (`GameplayStatics.GetAllActorsOfClass` "/Game/Play/Building/Address/Section/BP_Section.BP_Section_C"))
  (for _array_element _outactors
    (bind _asbp_prefab (cast `/Game/Play/Building/BP_Building/BP_Prefab` (`/Game/Play/Building/Address/Section/BP_Section.fGetBuildingBase` _array_element))) ; 建設中の建物のみ処理をする
    (`/Game/Play/Building/BP_Building/BP_Prefab.Finish` _asbp_prefab) ; 完成処理
  ))

(event `DeleteIcon`
  (bind _outactors (`GameplayStatics.GetAllActorsOfClass` "/Game/Play/Building/BP_Building/BuildingIcon/BP_BuildingIcon.BP_BuildingIcon_C"))
  (for _array_element _outactors
    (`self.K2_DestroyActor` _array_element)))

(event `DeleteAllEffect`
  (bind _outactors (`GameplayStatics.GetAllActorsOfClass` "/Game/Play/Building/BP_Building/BP_House.BP_House_C"))
  (for _array_element _outactors
    (`/Game/Play/Building/BP_Building/BP_House.DeleteEffect` _array_element)))

(fn `fAddTex`
  (params (`tex num` :type Integer))
  (set `self.mTexNum` (+ `tex num` (`self.mTexNum`))))

(fn `fCarCreateCount`
  (locals (finishFlag :type Boolean :default true))
  (bind _mbp_carcreatemanager (`self.mBP_CarCreateManager`))
  (while (`local.finishFlag`)
    (bind _result (`/Engine/EditorBlueprintResources/StandardMacros.IncrementInt` (`/Game/Play/Common/GroundObject/Car/BP_CarCreateManager.mCarCreateNum` _mbp_carcreatemanager))
      (:`  `
        (set `/Game/Play/Common/GroundObject/Car/BP_CarCreateManager.mCarCreateNum` _result _mbp_carcreatemanager)
        (set `self.mCarPeopleCountNum` (- (`self.mCarPeopleCountNum`) (`self.CAR_CREATE_PEOPLE_NUM`))) ; 増加人口減少
        (set `local.finishFlag` (< (/ (`self.mCarPeopleCountNum`) (`self.CAR_CREATE_PEOPLE_NUM`)) 0)))))
  (set `/Game/Play/Common/GroundObject/Car/BP_CarCreateManager.CarCreateFlag` true _mbp_carcreatemanager) ; 生成フラグを建てる
)

(fn `fCreateManager`
  ;[1 1 1] データ管理クラスの作成
  (bind _returnvalue (`|SpawnActorFromClass` "/Game/Play/Building/Data/BP_BuildingDataTableManager.BP_BuildingDataTableManager_C" (`KismetMathLibrary.MakeTransform` (0.0 0.0 0.0)) "Undefined" "OverrideRootScale" null null))
  (set `self.mBP_BuildingDataTableManager` _returnvalue)
  ;[1 1 1] 区画管理クラスの作成
  (bind _returnvalue_2 (`|SpawnActorFromClass` "/Game/Play/Building/Address/BP_AddressManager.BP_AddressManager_C" (`KismetMathLibrary.MakeTransform` (0.0 0.0 0.0)) "Undefined" "OverrideRootScale" null null))
  (set `self.mBP_AddressManager` _returnvalue_2)
  ;[1 1 1] 車関連の生成処理
  ;;[1 1 1] 車転移管理クラスの生成処理
  (bind _returnvalue_3 (`|SpawnActorFromClass` "/Game/Play/Common/GroundObject/WarpPoint/BP_WarpManager.BP_WarpManager_C" (`KismetMathLibrary.MakeTransform` (0.0 0.0 0.0)) "Undefined" "OverrideRootScale" null null))
  (bind _output_get (set `self.mBP_WarpManager` _returnvalue_3))
  ;;[1 1 1] 車生成管理クラスの生成処理
  (bind _returnvalue_4 (`|SpawnActorFromClass` "/Game/Play/Common/GroundObject/Car/BP_CarCreateManager.BP_CarCreateManager_C" (`KismetMathLibrary.MakeTransform` (0.0 0.0 0.0)) "Undefined" "OverrideRootScale" null null))
  (bind _output_get_2 (set `self.mBP_CarCreateManager` _returnvalue_4))
  (`/Game/Play/Common/GroundObject/Car/BP_CarCreateManager.fSetCarMoveVel` _output_get_2 (`self.PLAY_CAR_MOVE_VEL`))
  (`/Game/Play/Common/GroundObject/Car/BP_CarCreateManager.SetWarpManager` _output_get_2 _output_get)
  ;[1 1 1] 現在選択している建物を表すＵＩ管理クラスを作成
  (bind _returnvalue_5 (`|SpawnActorFromClass` "/Game/Play/Building/UI/SelectBuilding/BP_SelectBuildingManager.BP_SelectBuildingManager_C" (`KismetMathLibrary.MakeTransform` (0.0 0.0 0.0)) "Undefined" "OverrideRootScale" null null))
  (bind _output_get_3 (set `self.mBP_SelectBuildingManager` _returnvalue_5))
  (`/Game/Play/Building/UI/SelectBuilding/BP_SelectBuildingManager.SelectBuildingInitialize` _output_get_3)
  ;[1 1 1] 不定期開催イベント管理マネージャ
  (bind _returnvalue_6 (`|SpawnActorFromClass` "/Game/Play/Building/UnscheduledEvent/BP_UnscheduledEventManager.BP_UnscheduledEventManager_C" (`KismetMathLibrary.MakeTransform` (0.0 0.0 0.0)) "Undefined" "OverrideRootScale" null null))
  (set `self.mBP_UnscheduledEventManager` _returnvalue_6))

(fn `fCreateUI`
  (`|ExecutionSequence`
    (:`then_0`
      ;[1 1 1] 建物情報ＵＩ
      (bind _returnvalue (`|CreateWidget` "/Game/Play/Building/UI/BuildingInfo/WBP_BuildingInfo.WBP_BuildingInfo_C"))
      (set `self.mWBP_BuildingInfo` _returnvalue)
      ;[1 1 1] 街の人数ＵＩ
      (bind _returnvalue_2 (`|CreateWidget` "/Game/Play/Building/UI/CitizenNum/WBP_PeopleTest.WBP_PeopleTest_C"))
      (set `self.mWBP_CitizenNum` _returnvalue_2)
      ;[1 1 1] 不定期イベントUI
      (bind _returnvalue_3 (`|CreateWidget` "/Game/Play/Building/UI/Event/WBP_Event.WBP_Event_C"))
      (set `self.mWBP_Event` _returnvalue_3)
      ;[1 1 1] お金UI
      (bind _returnvalue_4 (`|CreateWidget` "/Game/Play/Building/UI/Money/WBP_MoneyUI.WBP_MoneyUI_C"))
      (set `self.mWBP_Money` _returnvalue_4)
      ;[1 1 1] 時間制限UI
      (bind _returnvalue_5 (`|CreateWidget` "/Game/Play/Building/UI/TimeLimit/WBP_TimeLimit.WBP_TimeLimit_C"))
      (set `self.mWBP_TimeLimit` _returnvalue_5)
      ;[1 1 1] カウントダウンUIの作成
      (bind _returnvalue_6 (`|CreateWidget` "/Game/Play/Building/UI/CountDown/WBP_BuildingCountDown.WBP_BuildingCountDown_C"))
      (bind _output_get (set `self.mWBP_BuildingCountdown` _returnvalue_6))
      (`/Game/Play/Building/UI/CountDown/WBP_BuildingCountDown.fSetDrawString` _output_get "NewEnumerator1"))
    (:`then_1`
      (`UserWidget.AddToViewport` (`self.mWBP_BuildingInfo`) 10)
      (`UserWidget.AddToViewport` (`self.mWBP_Event`) 10)
      (`UserWidget.AddToViewport` (`self.mWBP_Money`) 10)
      (`UserWidget.AddToViewport` (`self.mWBP_BuildingCountdown`) 10)
      (`UserWidget.AddToViewport` (`self.mWBP_CitizenNum`) 10)
      ;[1 1 1] フラグが立っている場合、描画する
      (if (`self.mTimerDrawFlag`)
        (`UserWidget.AddToViewport` (`self.mWBP_TimeLimit`) 10)))))

(fn `fDeleteBlackBox`
  (bind _outactors (`GameplayStatics.GetAllActorsOfClass` "/Game/Play/Common/GroundObject/BlackBox/BP_BlackBox.BP_BlackBox_C"))
  (for _array_element _outactors
    (`self.K2_DestroyActor` _array_element)))

(fn `fDeleteCursor`
  (locals (NewLocalVar_0 :type "/Game/Play/Building/Address/Section/BP_Section Object Reference"))
  (bind _mbp_cursor (`self.mBP_Cursor`))
  (`/Engine/EditorBlueprintResources/StandardMacros.IsValid` _mbp_cursor
    (:`Is Valid`
      (set `/Game/Play/Building/Cursor/BP_Cursor.mEnd` true _mbp_cursor)
      (`/Game/Play/Building/Address/Section/BP_Section.DeleteInstant` (`/Game/Play/Building/Cursor/BP_Cursor.mSelectSection` _mbp_cursor)) ; 選択していた区画の削除
      (set `/Game/Play/Building/Cursor/BP_Cursor.mSelectSection` (`local.NewLocalVar_0`) _mbp_cursor)
      (`self.K2_DestroyActor` _mbp_cursor))))

(fn `fDeleteUI`
  (`Widget.RemoveFromParent` (`self.mWBP_BuildingInfo`))
  (`Widget.RemoveFromParent` (`self.mWBP_Event`))
  (`Widget.RemoveFromParent` (`self.mWBP_Money`))
  (`Widget.RemoveFromParent` (`self.mWBP_TimeLimit`))
  (`Widget.RemoveFromParent` (`self.mWBP_BuildingCountdown`))
  (`Widget.RemoveFromParent` (`self.mWBP_CitizenNum`))
  (`/Game/Play/Building/UI/SelectBuilding/BP_SelectBuildingManager.fDeleteUI` (`self.mBP_SelectBuildingManager`)))

(fn `fPeopleNumDown`
  (params (mVariavleNum :type Integer))
  (set `self.mCarPeopleCountNum` (- mVariavleNum (`self.mCarPeopleCountNum`))) ; 減少人口を保存
)

(fn `fPeopleNumUp`
  (params (mVariavleNum :type Integer))
  (set `self.mCarPeopleCountNum` (+ mVariavleNum (`self.mCarPeopleCountNum`))) ; 増加人口を保存
  (set `self.mPeopleCountNum` (+ mVariavleNum (`self.mPeopleCountNum`))))

(fn `fSetCountDownSound`
  (bind (_returnvalue _mse_countdown) (`self.ChackCountDownSE`)
    (:`Is Valid`
      (if _returnvalue
        (`AudioComponent.Stop` _mse_countdown)
        (switch `int` (`self.mTimeLimit`) :!label _label
          (:`0`
            (bind _returnvalue_2 (`GameplayStatics.SpawnSound2D` "/Game/Play/Building/Sound/SE/SoundEffect_Countdown.SoundEffect_Countdown" 1.0 1.0 3.0 null))
            (set `/Game/Play/Building/Sound/BP_BuildingSoundManager.mSE_Countdown` _returnvalue_2 (`self.mBP_BuildingSoundManager`)))
          (:`1`
            (bind _returnvalue_3 (`GameplayStatics.SpawnSound2D` "/Game/Play/Building/Sound/SE/SoundEffect_Countdown.SoundEffect_Countdown" 1.0 1.0 0.0 null :!label _label_2))
            (set `/Game/Play/Building/Sound/BP_BuildingSoundManager.mSE_Countdown` _returnvalue_3 (`self.mBP_BuildingSoundManager`)))
          (:`2`
            (goto _label_2))
          (:`3`
            (goto _label_2)))))
    (:`Is Not Valid`
      (goto _label))))

(fn `fSetStatusUpValue`
  ;[1 1 1] 市長のステータスアップに必要な情報をセット
  (bind _asgmi_destruction_city (cast `/Game/Play/Common/GameInstance/GMI_DestructionCIty` (`GameplayStatics.GetGameInstance`)))
  (set `/Game/Play/Common/GameInstance/GMI_DestructionCIty.mRemainingTotalMoney` (`self.mTexNum`) _asgmi_destruction_city)
  (set `/Game/Play/Common/GameInstance/GMI_DestructionCIty.mTotalPeopleNum` (`self.mPeopleCountNum`) _asgmi_destruction_city))

(fn `fSubFund`
  (params (Building :type "/Game/Play/Building/Data/EN_Building Enum" :default "NewEnumerator13"))
  (bind _value (`/Game/Play/Building/Data/BP_BuildingDataTableManager.fMap` (`self.mBP_BuildingDataTableManager`) Building))
  (set `self.mTexNum` (- (`self.mTexNum`) (`.BuildingFund_15_3682A8A942F60B1D8FC3AB9A10138CAC` (break `/Game/Play/Building/Data/ST_BuildingDataTable` _value)))))

(fn `UserConstructionScript`)