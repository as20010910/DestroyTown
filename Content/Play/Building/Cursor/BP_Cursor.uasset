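; Building placement cursor that snaps to the map section nearest the mouse and shows a flashing preview of the selected building.
; A looping timer line-traces the mouse, finds the nearest section for the building's size and address, then moves the instant preview when the section changes.
; A faster timer follows a spawned BP_Flashing to alternate the preview's FClear value.
; FGetBuildingInfoItem returns the selected building for empty sections, or the matching mansion for existing houses.
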(event `self.ReceiveBeginPlay`
  (bind _returnvalue (`|SpawnActorFromClass` "/Game/Play/Building/Address/BP_Flashing.BP_Flashing_C" (`KismetMathLibrary.MakeTransform` (0.0 0.0 0.0)) "Undefined" "OverrideRootScale" null null)) ; 点滅処理の生成
  (bind _output_get (set `self.mFlash` _returnvalue))
  (`/Game/Play/Building/Address/BP_Flashing.fSetFlashInterval` _output_get (`self.FLASH_INTERVAL`)) ; 点滅感覚の設定
  (set `/Game/Play/Building/Address/BP_Flashing.mMoveFlag` true _output_get) ; 点滅処理開始
  (`KismetSystemLibrary.K2_SetTimerDelegate` (delegate `SectionFlashUpdate`) (`/Game/Play/Common/GameMode/GM_DestructionCity.DELTA_TIME` (cast `/Game/Play/Common/GameMode/GM_DestructionCity` (`GameplayStatics.GetGameMode`) :!pure true)) true) ; 区画点滅処理
  ;[1 1 1] カーソルの更新処理
  (`KismetSystemLibrary.K2_SetTimerDelegate` (delegate `CursorMoveUpdate`) (* 5 (`/Game/Play/Common/GameMode/GM_DestructionCity.DELTA_TIME` (cast `/Game/Play/Common/GameMode/GM_DestructionCity` (`GameplayStatics.GetGameMode`) :!pure true))) true))

(event `CursorMoveUpdate`
  ;[1 1 1] カーソルの更新処理
  (`self.fMouseRayCast`) ; マウスレイキャスト
  (`self.F Send Address Sample Building`) ; カーソルから一番近い区画を選択する処理
  (bind _nearaddress (`/Game/Play/Building/Address/BP_AddressManager.fGetNearPositionAddress` (`/Game/Play/Building/BP_BuildingManager.mBP_AddressManager` (`/Game/Play/Common/GameMode/GM_DestructionCity.mBP_BuildingManager` (cast `/Game/Play/Common/GameMode/GM_DestructionCity` (`GameplayStatics.GetGameMode`) :!pure true))) (`self.mMouseRealPos`))) ; 一番近い番地を取得する
  (set `self.mSelectAddress` _nearaddress)
  (`self.UpdateSection`) ; 自身の区画変数の更新処理
)

(event `SectionFlashUpdate`
  (bind _asbp_building_base (`/Game/Play/Building/Address/Section/BP_Section.fGetBuildingBase` (`self.mBeforeSection`)))
  (`/Engine/EditorBlueprintResources/StandardMacros.IsValid` (`self.mSelectSection`) ; 存在しているとき処理を行う
    (:`Is Valid`
      (if (`/Game/Play/Building/Address/BP_Flashing.mFlashFlag` (`self.mFlash`))
        (`/Game/Play/Building/BP_Building/BP_BuildingBase.fClear` _asbp_building_base 0.5)
        (else
          (`/Game/Play/Building/BP_Building/BP_BuildingBase.fClear` _asbp_building_base 0.2))))))

(event `UpdateSection`
  ;[1 1 1] 選択区画変更更新処理
  (`/Engine/EditorBlueprintResources/StandardMacros.IsValid` (`self.mSelectSection`)
    (:`Is Valid`
      (`/Engine/EditorBlueprintResources/StandardMacros.IsValid` (`self.mBeforeSection`)
        (:`Is Valid`
          (if (!= (`self.mSelectSection`) (`self.mBeforeSection`))
            (`/Game/Play/Building/Address/Section/BP_Section.DeleteInstant` (`self.mBeforeSection`)) ; 選択していた区画の削除
            (`/Game/Play/Building/Address/Section/BP_Section.ChangeInstant` (`self.mSelectSection`)) ; 建物を建てる
            (set `self.mBeforeSection` (`self.mSelectSection`)) ; 新しいものに更新
          ))
        (:`Is Not Valid`
          (set `self.mBeforeSection` (`self.mSelectSection`)) ; 空の場合は保存する
        )))))

(fn `F Send Address Sample Building`
  (locals (addressManager :type "/Game/Play/Building/Address/BP_AddressManager Object Reference") (nowPosition :type "Vector Structure") (nearLength :type "Float (double-precision)") (nearAddressIndex :type Integer) (nowLength :type "Float (double-precision)") (nowAddress :type "/Game/Play/Building/Address/BP_Address Object Reference") (MINDISTANCE :type "Float (double-precision)" :default 10000.0) (NOWSECTION :type "/Game/Play/Building/Address/Section/BP_Section Object Reference") (instantactor :type "Actor Object Reference") (mNowSize :type "/Game/Play/Building/Data/EN_BuildingSize Enum") (NewLocalVar_0 :type "/Game/Play/Building/Address/Section/BP_Section Object Reference"))
  (bind _mbp_buildingmanager (`/Game/Play/Common/GameMode/GM_DestructionCity.mBP_BuildingManager` (cast `/Game/Play/Common/GameMode/GM_DestructionCity` (`GameplayStatics.GetGameMode`) :!pure true)))
  (bind _value_size (`self.fGetSelectBuildingSize` (`/Game/Play/Building/BP_BuildingManager.mBP_Cursor` _mbp_buildingmanager))) ; 現在選択中の建物のサイズを取得する
  ;[1 1 1] 簡略化
  (bind _output_get (set `local.addressManager` (`/Game/Play/Building/BP_BuildingManager.mBP_AddressManager` _mbp_buildingmanager)))
  (bind _nearsection (`/Game/Play/Building/Address/BP_AddressManager.fGetNearPositionSection` (`local.addressManager`) (`self.mMouseRealPos`) (break `/Game/Play/Building/Address/ST_SectionArray` (`BlueprintMapLibrary.Map_Find` (`/Game/Play/Building/Address/BP_AddressManager.mMap` _output_get) _value_size)))) ; 一番近い区画を取得する
  ;[1 1 1] 保存する
  (`self.K2_SetActorLocation` (`self.K2_GetActorLocation` _nearsection) false true)
  (set `self.mSelectSection` _nearsection))

(fn `fDeleteSection`
  (locals (BP_Section :type "/Game/Play/Building/Address/Section/BP_Section Object Reference"))
  (set `self.mSelectSection` (`local.BP_Section`)))

(fn `fGetBuildingInfoItem`
  (returns (mNowSelectBuilding :type "/Game/Play/Building/Data/EN_Building Enum"))
  (bind _mselectsection (`self.mSelectSection`))
  (`/Engine/EditorBlueprintResources/StandardMacros.IsValid` _mselectsection
    (:`Is Valid`
      (switch `/Game/Play/Building/Address/Section/EN_SectionState` (`/Game/Play/Building/Address/Section/BP_Section.mState` _mselectsection)
        (:`NewEnumerator0`
          (return (`self.mNowSelectBuilding`)))
        (:`NewEnumerator2`
          (switch `/Game/Play/Building/Data/EN_Building` (`/Game/Play/Building/BP_Building/BP_BuildingBase.mBuilding` (`/Game/Play/Building/Address/Section/BP_Section.fGetBuildingBase` _mselectsection))
            (:`NewEnumerator0`
              (return "NewEnumerator1"))
            (:`NewEnumerator2`
              (return "NewEnumerator3"))
            (:`NewEnumerator4`
              (return "NewEnumerator5"))))))))

(fn `fGetSelectBuildingInfo`
  (returns (BuildingInfo :type "/Game/Play/Building/Data/ST_BuildingDataTable Structure"))
  (bind _value (`/Game/Play/Building/Data/BP_BuildingDataTableManager.fMap` (`/Game/Play/Building/BP_BuildingManager.mBP_BuildingDataTableManager` (`/Game/Play/Common/GameMode/GM_DestructionCity.mBP_BuildingManager` (cast `/Game/Play/Common/GameMode/GM_DestructionCity` (`GameplayStatics.GetGameMode`) :!pure true))) (`self.mNowSelectBuilding`)))
  (return _value))

(fn `fGetSelectBuildingSize`
  (returns (`Value Size` :type "/Game/Play/Building/Data/EN_BuildingSize Enum"))
  (bind _mbp_buildingmanager (`/Game/Play/Common/GameMode/GM_DestructionCity.mBP_BuildingManager` (cast `/Game/Play/Common/GameMode/GM_DestructionCity` (`GameplayStatics.GetGameMode`) :!pure true)))
  (bind _value (`/Game/Play/Building/Data/BP_BuildingDataTableManager.fMap` (`/Game/Play/Building/BP_BuildingManager.mBP_BuildingDataTableManager` _mbp_buildingmanager) (`/Game/Play/Building/Cursor/BP_Cursor.mNowSelectBuilding` (`/Game/Play/Building/BP_BuildingManager.mBP_Cursor` _mbp_buildingmanager))))
  (return (`.Size_36_88201531459E6DE419D45D8963D69E1B` (break `/Game/Play/Building/Data/ST_BuildingDataTable` _value))))

(fn `fMouseRayCast`
  (locals (adjustMousePosition :type "/Game/Vector2 Structure"))
  (bind _returnvalue (`GameplayStatics.GetPlayerController` 0))
  (bind (_locationx _locationy) (`PlayerController.GetMousePosition` _returnvalue))
  (bind (_worldlocation _worlddirection) (`PlayerController.DeprojectScreenPositionToWorld` _returnvalue _locationx _locationy))
  (bind (_outhit _returnvalue_2) (`KismetSystemLibrary.LineTraceSingleForObjects` _worldlocation (+ _worldlocation (* _worlddirection 10000)) (`|MakeArray` "ObjectTypeQuery1" :!type "EObjectTypeQuery Enum")))
  (if _returnvalue_2
    (set `self.mMouseRealPos` (`.Location` (`GameplayStatics.BreakHitResult` _outhit)))))

(fn `UserConstructionScript`)