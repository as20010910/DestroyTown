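; Base actor for a city building with a destructible mesh, configured per building type from data tables reached through GM_DestructionCity.
; An outline mesh highlights it while the Mayor overlaps its damage collision.
; On first fracture it lets the Mayor pass, adds damage cost and score (mansions doubled), then fades by timer-driven opacity until destroyed.
; It also handles applied damage, one-time fire spread for wooden types, red tinting and upgrade-type lookup.
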(event `self.ReceiveBeginPlay`
  ;[1 1 1] 初期化処理
)

(event `ColorRedUpdate`
  (if (`self.mRedFlag`)
    (set `self.mRedFlag` false)
    (`self.fResetMaterials`)))

(event `SetOutlineMesh`
  (bind _outlinemesh (`self.OutlineMesh`))
  ;[1 1 1] アウトラインメッシュをセットする
  (bind _destructionbuildingdata (`self.fGetDestructionBuildingData`))
  (`StaticMeshComponent.SetStaticMesh` (`self.OutlineMesh`) (`.OutlineMesh_16_412A5C5C44D570BA8280B4B5564D46A6` (break `/Game/Play/Destruction/Building/Data/ST_DestructionBuildingData` _destructionbuildingdata)))
  (for _index (range (+ (`PrimitiveComponent.GetNumMaterials` _outlinemesh) 1))
    (`PrimitiveComponent.SetMaterial` _outlinemesh _index "/Game/Play/Building/BP_Building/Outline/MTI_Outline.MTI_Outline")))

(event `BuildingApplyDamage`
  (params (AttackDamage :type "Float (double-precision)") (ImpluseDir :type "Vector Structure") (ImpulseStrength :type "Float (double-precision)"))
  ;[1 1 1] 建物にダメージを与える処理
  (`DestructibleComponent.ApplyDamage` (`self.Building`) AttackDamage (+ (`self.K2_GetActorLocation`) (`self.mDamageShiftPos`)) ImpluseDir ImpulseStrength))

(event `WoodenBuildingSpreadOfFire`
  (params (MayorAttackState :type "/Game/Play/Destruction/Mayor/Data/EN_MayorAttackState Enum" :default "NewEnumerator0"))
  ;[1 1 1] 建物の延焼処理
  (bind _iswooden (`self.fCheckWoodenBuilding`))
  (if (and _iswooden (`|EnumEquality` MayorAttackState "NewEnumerator1"))
    (`/Engine/EditorBlueprintResources/StandardMacros.DoOnce` false
      (:`Completed`
        (set `self.mIsSpreadOfFire` true)
        (`|SpawnActorFromClass` "/Game/Play/Destruction/Building/SpecialEffects/BP_SpreadOfFire.BP_SpreadOfFire_C" (`self.GetTransform`) "Undefined" "OverrideRootScale" null null)))))

(event `self.Building.OnComponentFracture`
  (params (HitPoint :type "Vector Structure (by ref)") (HitDirection :type "Vector Structure (by ref)"))
  ;[1 1 1] 建物が壊された時の処理
  (`/Engine/EditorBlueprintResources/StandardMacros.DoOnce` false
    (:`Completed`
      (set `self.mIsDestroyed` true) ; 建物が破壊された確認フラグをtrueに
      (`PrimitiveComponent.SetCollisionEnabled` (`self.Building`) "PhysicsOnly") ; 建物のコリジョンを変更し市長が建物上を移動できるように
      (`self.InvisibleOutlineMesh`) ; アウトラインを消す
      (bind _newparam (`self.fGetBuildingData` true)) ; 建物データを取得
      (`/Game/Play/Destruction/BP_DestructionManager.fAddAmoutDamage` (`/Game/Play/Common/GameMode/GM_DestructionCity.mBP_DestructionManager` (cast `/Game/Play/Common/GameMode/GM_DestructionCity` (`GameplayStatics.GetGameMode`) :!pure true)) (`.AmountDamage_19_113FD47A439AFCC53D09B596F01BB7F5` (break `/Game/Play/Building/Data/ST_BuildingDataTable` _newparam))) ; 被害総額追加処理
      (`self.fAdd DestroyScore` (break `/Game/Play/Building/Data/ST_BuildingDataTable` _newparam))
      (set `self.mNowMatAlpha` (`self.DEFAULT_DESTRUCTION_ALPHA`))
      (`KismetSystemLibrary.K2_SetTimerDelegate` (delegate `TransparentBuilding`) (`/Game/Play/Common/GameMode/GM_DestructionCity.DELTA_TIME` (cast `/Game/Play/Common/GameMode/GM_DestructionCity` (`GameplayStatics.GetGameMode`) :!pure true)) true))))

(event `TransparentBuilding`
  (bind _returnvalue (- (`self.mNowMatAlpha`) (`self.CLEAR_SPEED`)))
  ;[1 1 1] 透過処理
  (set `self.mNowMatAlpha` _returnvalue) ; α値を減少させる
  (if (<= _returnvalue 0.0)
    (`self.K2_DestroyActor`) ; 削除
    (else
      (`self.fClear` _returnvalue) ; 透過処理
    )))

(event `VisibleOutlineMesh`
  ;[1 1 1] アウトラインの表示処理
  (if (not (`self.mIsDestroyed`))
    (`SceneComponent.SetVisibility` (`self.OutlineMesh`) true false)))

(event `self.DamageCollision.OnComponentBeginOverlap`
  (params (OverlappedComponent :type "PrimitiveComponent Object Reference") (OtherActor :type "Actor Object Reference") (OtherComp :type "PrimitiveComponent Object Reference") (OtherBodyIndex :type Integer) (bFromSweep :type Boolean) (SweepResult :type "HitResult Structure (by ref)"))
  ;[1 0.8516 0] テスト
  (cast `/Game/Play/Destruction/Mayor/BP_Mayor` OtherActor)
  (`self.VisibleOutlineMesh`))

(event `self.DamageCollision.OnComponentEndOverlap`
  (params (OverlappedComponent :type "PrimitiveComponent Object Reference") (OtherActor :type "Actor Object Reference") (OtherComp :type "PrimitiveComponent Object Reference") (OtherBodyIndex :type Integer))
  ;[1 0.8516 0] テスト
  (cast `/Game/Play/Destruction/Mayor/BP_Mayor` OtherActor)
  (`self.InvisibleOutlineMesh`))

(event `InvisibleOutlineMesh`
  ;[1 1 1] アウトラインの表示処理
  (`SceneComponent.SetVisibility` (`self.OutlineMesh`) false false))

(event `SetDestructionBuildingData`
  ;[1 1 1] 破壊用の建物データをセット
  (bind _destructionbuildingdata (`self.fGetDestructionBuildingData`)) ; 破壊用の建物データの取得
  (set `self.mDamageShiftPos` (`.DamageShiftPos_5_25186031467A2CA9766835B4FCC13612` (break `/Game/Play/Destruction/Building/Data/ST_DestructionBuildingData` _destructionbuildingdata))) ; ダメージを与える座標をセット
  (`SceneComponent.SetWorldScale3D` (`self.DamageCollision`) (`.DamageCollisionScale_8_AD39EC51423E4E6FC04D27BDF691B395` (break `/Game/Play/Destruction/Building/Data/ST_DestructionBuildingData` _destructionbuildingdata))) ; ダメージコリジョンのサイズをセット
)

(fn `F Color Red Mesh`
  (bind _building (`self.Building`))
  (for (_ _array_index) (`MeshComponent.GetMaterials` _building)
    (`PrimitiveComponent.SetMaterial` _building _array_index "/Game/Play/Building/BP_Building/Model/MT_ClearRed.MT_ClearRed"))
  (set `self.mRedFlag` true))

(fn `fAdd DestroyScore`
  (params (Building :type "/Game/Play/Building/Data/EN_Building Enum" :default "NewEnumerator13"))
  (locals (ST_SCOREBASE :type "/Game/Play/Common/ST_ScoreBase Structure"))
  (bind _asgm_destruction_city (cast `/Game/Play/Common/GameMode/GM_DestructionCity` (`GameplayStatics.GetGameMode`) :!pure true))
  (bind _value (`self.fCastMansionScore` Building))
  (set `/Game/Play/Common/GameMode/GM_DestructionCity.mDestroyScore` (+ _value (`/Game/Play/Common/GameMode/GM_DestructionCity.mDestroyScore` _asgm_destruction_city)) _asgm_destruction_city))

(fn `fCastMansionScore`
  (params (Building :type "/Game/Play/Building/Data/EN_Building Enum" :default "NewEnumerator13"))
  (returns (Value :type "Float (double-precision)"))
  (locals (ST_SCORE_BASE :type "/Game/Play/Common/ST_ScoreBase Structure"))
  (bind _st_score_base_scorebase (break `/Game/Play/Common/ST_ScoreBase` (`local.ST_SCORE_BASE`)))
  (bind _st_score_base_scorebase_2 (break `/Game/Play/Common/ST_ScoreBase` (`local.ST_SCORE_BASE`)))
  (if (or (`|EnumEquality` Building "NewEnumerator1") (`|EnumEquality` Building "NewEnumerator3") (`|EnumEquality` Building "NewEnumerator5"))
    (return (* 2 (`BlueprintMapLibrary.Map_Find` _st_score_base_scorebase Building)))
    (else
      (return (`BlueprintMapLibrary.Map_Find` _st_score_base_scorebase_2 Building)))))

(fn `fCheckWoodenBuilding`
  (returns (IsWooden :type Boolean))
  (bind _mbuilding (`self.mBuilding`))
  ;[1 1 1] 建物が木材か調べる
  (return (or (`|EnumEquality` _mbuilding "NewEnumerator0") (`|EnumEquality` _mbuilding "NewEnumerator1"))))

(fn `fClear`
  (params (ParameterValue :type "Float (double-precision)"))
  ;[1 1 1] 透明度の指定
  (`MeshComponent.SetScalarParameterValueOnMaterials` (`self.Building`) "Opacity" ParameterValue))

(fn `fGetBuildingData`
  (params (IsDestructionPart :type Boolean))
  (returns (NewParam :type "/Game/Play/Building/Data/ST_BuildingDataTable Structure"))
  ;[1 1 1] 建物データを取得する
  (bind _asgm_destruction_city (cast `/Game/Play/Common/GameMode/GM_DestructionCity` (`GameplayStatics.GetGameMode`)))
  (if IsDestructionPart
    (bind _value (`/Game/Play/Building/Data/BP_BuildingDataTableManager.fMap` (`/Game/Play/Destruction/BP_DestructionManager.mBP_BuildingDataTableManager` (`/Game/Play/Common/GameMode/GM_DestructionCity.mBP_DestructionManager` _asgm_destruction_city)) (`self.mBuilding`))) ; 建物に対応するデータテーブルを取得
    (return _value)
    (else
      (bind _value_2 (`/Game/Play/Building/Data/BP_BuildingDataTableManager.fMap` (`/Game/Play/Building/BP_BuildingManager.mBP_BuildingDataTableManager` (`/Game/Play/Common/GameMode/GM_DestructionCity.mBP_BuildingManager` _asgm_destruction_city)) (`self.mBuilding`))) ; 建物に対応するデータテーブルを取得
      (return _value_2))))

(fn `fGetDestructionBuildingData`
  (returns (DestructionBuildingData :type "/Game/Play/Destruction/Building/Data/ST_DestructionBuildingData Structure"))
  ;[1 1 1] 破壊用の建物データの取得
  (bind _asgm_destruction_city (cast `/Game/Play/Common/GameMode/GM_DestructionCity` (`GameplayStatics.GetGameMode`)))
  (bind _mbp_destructionbuildingdatatablemanager (`/Game/Play/Destruction/BP_DestructionManager.mBP_DestructionBuildingDataTableManager` (`/Game/Play/Common/GameMode/GM_DestructionCity.mBP_DestructionManager` _asgm_destruction_city)))
  (`/Engine/EditorBlueprintResources/StandardMacros.IsValid` _mbp_destructionbuildingdatatablemanager
    (:`Is Valid`
      (bind _buildingdatatable (`/Game/Play/Destruction/Building/Data/BP_DestructionBuildingDataTableManager.fMap` _mbp_destructionbuildingdatatablemanager (`self.mBuilding`)))
      (return _buildingdatatable))))

(fn `fResetMaterials`
  (bind _building (`self.Building`))
  (for (_ _array_index) (`MeshComponent.GetMaterials` _building)
    (`PrimitiveComponent.SetMaterial` _building _array_index null)))

(fn `fReturnDevelopBuilding`
  (params (BeforeCreate :type "/Game/Play/Building/Data/EN_Building Enum" :default "NewEnumerator13"))
  (returns (`Develop Building` :type "/Game/Play/Building/Data/EN_Building Enum"))
  (if (`|EnumEquality` BeforeCreate "NewEnumerator0")
    (return "NewEnumerator1")
    (elif (`|EnumEquality` BeforeCreate "NewEnumerator2")
      (return "NewEnumerator3")
      (elif (`|EnumEquality` BeforeCreate "NewEnumerator4")
        (return "NewEnumerator5")
        (else
          (return "NewEnumerator13"))))))

(fn `fSetMesh`
  (params (NewParam :type "/Game/Play/Building/Data/EN_Building Enum" :default "NewEnumerator13"))
  (if (`|EnumEquality` NewParam "NewEnumerator13")
    (`DestructibleComponent.SetDestructibleMesh` (`self.Building`) null)
    (else
      (bind _value (`/Game/Play/Building/Data/BP_BuildingDataTableManager.fMap` (`/Game/Play/Building/BP_BuildingManager.mBP_BuildingDataTableManager` (`/Game/Play/Common/GameMode/GM_DestructionCity.mBP_BuildingManager` (cast `/Game/Play/Common/GameMode/GM_DestructionCity` (`GameplayStatics.GetGameMode`) :!pure true))) NewParam))
      (`DestructibleComponent.SetDestructibleMesh` (`self.Building`) (`.DestructibleMesh_28_C4AEC3F449FA69CAC7814881C59E681D` (break `/Game/Play/Building/Data/ST_BuildingDataTable` _value)))
      (`self.fResetMaterials`) ; マテリアル情報をリセットする
    )))

(fn `UserConstructionScript`)