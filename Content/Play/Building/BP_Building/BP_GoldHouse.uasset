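; BP_GoldHouse is a gold variant of a game building that picks its type at random and starts out hidden.
; On BeginPlay it offsets MGoldBuilding by a random index within MGoldBuildingTypes, assigns the result to MBuilding, then runs the parent's setup.
; It then hides the Building component through SetGoldHouseVisibility, an event that can also show it.
; Construction, overlap and tick defer to the parent.
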(event `self.ReceiveBeginPlay`
  ;[1 1 1] 初期化処理
  (`self.fSetGoldBuildingType`) ; 金の建物の種類をランダムでセットする
  (set `self.mBuilding` (`self.mGoldBuilding`))
  (`parent.ReceiveBeginPlay`)
  (`self.SetGoldHouseVisibility` false) ; 可視性をオフに
)

(event `self.ReceiveActorBeginOverlap`
  (params (OtherActor :type "Actor Object Reference"))
  (`parent.ReceiveActorBeginOverlap` OtherActor))

(event `self.ReceiveTick`
  (params (DeltaSeconds :type "Float (single-precision)"))
  (`parent.ReceiveTick` DeltaSeconds))

(event `SetGoldHouseVisibility`
  (params (IsVisibility :type Boolean))
  ;[1 1 1] 建物の可視性をセット
  (`SceneComponent.SetVisibility` (`self.Building`) IsVisibility false))

(fn `fSetGoldBuildingType`
  ;[1 1 1] 金の建物の種類をランダムでセットする
  (set `self.mGoldBuilding` (cast `/Game/Play/Building/Data/EN_Building` (+ (`self.mGoldBuilding`) (`KismetMathLibrary.Conv_IntToByte` (`KismetMathLibrary.RandomIntegerInRange` 0 (`KismetArrayLibrary.Array_LastIndex` (`self.mGoldBuildingTypes`))))))))

(fn `UserConstructionScript`
  (`parent.UserConstructionScript`))