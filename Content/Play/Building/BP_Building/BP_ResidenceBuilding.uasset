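; BP_ResidenceBuilding is a residential building Blueprint that adds citizens to the city's population.
; Its initialization function reads the building's data row from the building data table manager, reached through the GM_DestructionCity game mode's building manager.
; It then passes that row's CitizenGain to the manager to raise the people count.
; The event graph holds only disabled default events, and the construction script just calls its parent.
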(fn `fResidenceInitialize`
  (bind _mbp_buildingmanager (`/Game/Play/Common/GameMode/GM_DestructionCity.mBP_BuildingManager` (cast `/Game/Play/Common/GameMode/GM_DestructionCity` (`GameplayStatics.GetGameMode`) :!pure true)))
  (bind _value (`/Game/Play/Building/Data/BP_BuildingDataTableManager.fMap` (`/Game/Play/Building/BP_BuildingManager.mBP_BuildingDataTableManager` _mbp_buildingmanager) (`self.mBuilding`)))
  (`/Game/Play/Building/BP_BuildingManager.fPeopleNumUp` _mbp_buildingmanager (`.CitizenGain_17_96480A2B483BACD462A4BABB9CDDD37C` (break `/Game/Play/Building/Data/ST_BuildingDataTable` _value))) ; 家建て時の人数を増加させる
)

(fn `UserConstructionScript`
  (`parent.UserConstructionScript`))