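; BP_Prefab is the construction-site placeholder for a building, shown with a prefab destructible mesh and scalable to footprint presets.
; On BeginPlay it starts a construction sound and creates a screen-space time gauge widget.
; Looping timers keep the gauge projected over the actor and advance it every second.
; When the gauge fills, it tells its parent section to complete the building, swaps the sound and removes the gauge.
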(event `self.ReceiveBeginPlay`
  (`parent.ReceiveBeginPlay`)
  (`self.fSetPrefabMesh`) ; メッシュ設定
  (bind _index (`/Game/Play/Building/Sound/BP_BuildingSoundManager.fCreateSound` (`/Game/Play/Building/BP_BuildingManager.mBP_BuildingSoundManager` (`/Game/Play/Common/GameMode/GM_DestructionCity.mBP_BuildingManager` (cast `/Game/Play/Common/GameMode/GM_DestructionCity` (`GameplayStatics.GetGameMode`) :!pure true))) "NewEnumerator4" (`self.K2_GetActorLocation`))) ; 建築中の音を鳴らす
  (set `self.mSoundIndex` _index) ; 配列番号管理
  (`self.fCreateGauge`) ; 時間可視化ゲージの作成
  (`KismetSystemLibrary.K2_SetTimerDelegate` (delegate `GaugePositionUpdate`) (`/Game/Play/Common/GameMode/GM_DestructionCity.DELTA_TIME` (cast `/Game/Play/Common/GameMode/GM_DestructionCity` (`GameplayStatics.GetGameMode`) :!pure true)) true) ; ゲージ位置更新処理
  (`KismetSystemLibrary.K2_SetTimerDelegate` (delegate `GaugeNumUpdate`) 1.0 true) ; ゲージ位置更新処理
)

(event `GaugePositionUpdate`
  (`self.fMoveGauge`))

(event `GaugeNumUpdate`
  (bind _mwbp_creategauge (`self.mWBP_CreateGauge`))
  (`/Game/Play/Building/UI/CreateTimeGauge/WBP_CreateTimeGauge.fUpGauge` _mwbp_creategauge)
  (bind _return (`/Game/Play/Building/UI/CreateTimeGauge/WBP_CreateTimeGauge.fChackFinish` _mwbp_creategauge))
  (if _return
    (`self.Finish`) ; プレハブ終了処理
  ))

(event `DEBUG`
  ;[1 0.9875 0] 5秒後に生成
  (`self.Finish`) ; プレハブ終了処理
)

(event `Finish`
  (bind _mbp_buildingsoundmanager (`/Game/Play/Building/BP_BuildingManager.mBP_BuildingSoundManager` (`/Game/Play/Common/GameMode/GM_DestructionCity.mBP_BuildingManager` (cast `/Game/Play/Common/GameMode/GM_DestructionCity` (`GameplayStatics.GetGameMode`) :!pure true))))
  (`/Game/Play/Building/Address/Section/BP_Section.F Complete Building` (`self.mParentSection`)) ; 建物を建てる処理
  (bind _soundvalue (`/Game/Play/Building/Sound/BP_BuildingSoundManager.fGetSoundArray` _mbp_buildingsoundmanager "NewEnumerator4" (`self.mSoundIndex`))) ; 建築中の音を止める
  (`AudioComponent.Stop` _soundvalue)
  (`/Game/Play/Building/Sound/BP_BuildingSoundManager.fCreateSound` _mbp_buildingsoundmanager "NewEnumerator0" (`self.K2_GetActorLocation`))
  (`Widget.RemoveFromParent` (`self.mWBP_CreateGauge`)) ; ゲージを非表示に
)

(fn `fCreateGauge`
  (bind _returnvalue (`|CreateWidget` "/Game/Play/Building/UI/CreateTimeGauge/WBP_CreateTimeGauge.WBP_CreateTimeGauge_C"))
  (bind _output_get (set `self.mWBP_CreateGauge` _returnvalue))
  (`/Game/Play/Building/UI/CreateTimeGauge/WBP_CreateTimeGauge.fSetPosition` _output_get (/ (`PlayerController.ProjectWorldLocationToScreen` (`GameplayStatics.GetPlayerController` 0) (+ (`self.K2_GetActorLocation`) (0.0 -50.0 100.0)) false) (`WidgetLayoutLibrary.GetViewportScale`))) ; レイキャスト
  (`UserWidget.AddToViewport` _output_get 0))

(fn `fMoveGauge`
  (`/Game/Play/Building/UI/CreateTimeGauge/WBP_CreateTimeGauge.fSetPosition` (`self.mWBP_CreateGauge`) (/ (`PlayerController.ProjectWorldLocationToScreen` (`GameplayStatics.GetPlayerController` 0) (+ (`self.K2_GetActorLocation`) (0.0 -50.0 100.0)) false) (`WidgetLayoutLibrary.GetViewportScale`))) ; レイキャスト
)

(fn `fSetParentSection`
  (params (section :type "/Game/Play/Building/Address/Section/BP_Section Object Reference"))
  (set `self.mParentSection` section))

(fn `fSetPrefabMesh`
  (`DestructibleComponent.SetDestructibleMesh` (`self.Building`) "/Game/Play/Building/BP_Building/Model/Prefab/APEXM_Prefab.APEXM_Prefab")
  (`self.fResetMaterials`) ; マテリアル情報をリセットする
)

(fn `fSetPrefabSize`
  (params (mPrefabSize :type "/Game/Play/Building/Data/EN_BuildingSize Enum" :default "NewEnumerator0"))
  (locals (x :type "Float (double-precision)") (y :type "Float (double-precision)"))
  (switch `/Game/Play/Building/Data/EN_BuildingSize` mPrefabSize
    (:`NewEnumerator0`
      (set `local.x` 1.0)
      (set `local.y` 1.0))
    (:`NewEnumerator1`
      (set `local.x` 2.0)
      (set `local.y` 2.0))
    (:`NewEnumerator2`
      (set `local.x` 3.0)
      (set `local.y` 3.0))
    (:`NewEnumerator4`
      (set `local.x` 1.0)
      (set `local.y` 2.0))
    (:`NewEnumerator5`
      (set `local.x` 2.0)
      (set `local.y` 3.0)))
  ;[1 1 1] 拡大率設定
  (`self.SetActorScale3D` (`KismetMathLibrary.MakeVector` (`local.x`) (`local.y`) 1.0)))

(fn `UserConstructionScript`
  (`parent.UserConstructionScript`))