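; Building data manager Blueprint that caches DT_Building rows for lookup.
; On BeginPlay, it loops over an enum's entry count, looks up rows named by each index, and appends those found to an array.
; FMap converts its parameter to an integer, decrements it and returns the array element at that position, so lookups depend on the order rows were added.
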(event `self.ReceiveBeginPlay`
  (`self.fSetTableData`))

(fn `fMap`
  (params (NewParam :type "/Game/Play/Building/Data/EN_Building Enum" :default "NewEnumerator0"))
  (returns (value :type "/Game/Play/Building/Data/ST_BuildingDataTable Structure"))
  (locals (NewLocalVar_0 :type "/Game/Play/Building/Data/ST_BuildingDataTable Structure"))
  (bind _result (`/Engine/EditorBlueprintResources/StandardMacros.DecrementInt` (`KismetMathLibrary.Conv_ByteToInt` NewParam))
    (:`  `
      (bind _output (`|GetArrayItem` (`self.mST_BuildingDataTable`) _result))
      (set `local.NewLocalVar_0` _output)
      (return _output))))

(fn `fSetTableData`
  (for _index (range (+ (enumcount `/Game/Play/Building/Data/EN_Building`) 1))
    (bind _returnvalue (`|GetDataTableRow` "/Game/Play/Building/Data/DT_Building.DT_Building" (`KismetStringLibrary.Conv_StringToName` (`KismetStringLibrary.Conv_IntToString` _index)))
      (:`then`
        (`KismetArrayLibrary.Array_Add` (`self.mST_BuildingDataTable`) _returnvalue)))))

(fn `UserConstructionScript`)