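; BP_UnscheduledEventManager triggers random disaster events in the city-building game, active only outside casual mode.
; A looping timer rolls a percentage chance to start an event, gated by a creation flag tied to the absence of a hospital.
; A per-second update runs the event until a spawned BP_Timer expires.
; Only infectious disease is implemented, draining population through the building manager; fog, gas, famine and pollution are empty stubs.
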(event `EventManagerInitialize`)

(event `self.ReceiveBeginPlay`
  (bind _returnvalue (`|SpawnActorFromClass` "/Game/Play/Common/GroundObject/BP_Timer.BP_Timer_C" (`KismetMathLibrary.MakeTransform` (0.0 0.0 0.0)) "Undefined" "OverrideRootScale" null null))
  (bind _output_get (set `self.mEventTimer` _returnvalue))
  (`/Game/Play/Common/GroundObject/BP_Timer.fSetMaxTime` _output_get 5.0)
  (if (not (`/Game/Play/Building/BP_BuildingManager.mCasual` (`/Game/Play/Common/GameMode/GM_DestructionCity.mBP_BuildingManager` (cast `/Game/Play/Common/GameMode/GM_DestructionCity` (`GameplayStatics.GetGameMode`) :!pure true))))
    (`KismetSystemLibrary.K2_SetTimerDelegate` (delegate `EventProcessing`) (`self.mInterEvent`) true 10.0 2.0)
    (`KismetSystemLibrary.K2_SetTimerDelegate` (delegate `EventUpdate`) 1.0 true) ; イベントの更新処理
  ))

(event `EventProcessing`
  (if (`self.mEventCreateFlag`)
    (if (`self.mEventFlag`)
      _
      (elif (>= (`self.mPercentageEvent`) (`KismetMathLibrary.RandomFloatInRange` 0.0 100.0))
        (set `self.mEventFlag` true)
        (set `self.mEvent` "NewEnumerator0") ; 乱数でイベントを指定
      ))))

(event `EventUpdate`
  (if (and (`self.mEventFlag`) (`self.mEventCreateFlag`))
    (bind _newparam (`/Game/Play/Common/GroundObject/BP_Timer.fCountUp` (`self.mEventTimer`) 1.0))
    (if _newparam
      ;[1 1 1] イベント一時停止処理
      (`/Game/Play/Common/GroundObject/BP_Timer.fReset` (`self.mEventTimer`))
      (set `self.mEventFlag` false)
      (else
        (switch `/Game/Play/Building/UnscheduledEvent/EN_UnscheduledEvent` (`self.mEvent`)
          (:`NewEnumerator0`
            (`self.InfectiousDisease`)))))))

(event `ThickFog`)

(event `PoisonousGas`)

(event `Famine`)

(event `Pollution`)

(fn `fGetBuildingManager`
  (returns (mBP_BuildingManager :type "/Game/Play/Building/BP_BuildingManager Object Reference"))
  (return (`/Game/Play/Common/GameMode/GM_DestructionCity.mBP_BuildingManager` (cast `/Game/Play/Common/GameMode/GM_DestructionCity` (`GameplayStatics.GetGameMode`) :!pure true))))

(fn `InfectiousDisease`
  (locals (DECREASE_NUM :type "/Game/Play/Building/UnscheduledEvent/EN_UnscheduledEvent Enum"))
  (`/Game/Play/Building/BP_BuildingManager.fPeopleNumDown` (`self.fGetBuildingManager`) 1) ; 人口減少
)

(fn `UserConstructionScript`)